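; Coin pickup that flies toward the player and adds to their coin component when collected.
; On BeginPlay a timeline lerps the coin from its current location toward player pawn 0 each update, while a short delay arms collection.
; Tick polls the sphere for overlap with the player's capsule; once armed, it calls AddCoins on BPCCoins and destroys the actor.
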(event EventBeginPlay
  (Utilities|FlowControl|Sequence
    (:then_0
      (Utilities|FlowControl|Delay 0.65)
      (Variables|Default|SetCanGain true))
    (:then_1
      (bind _positionalpha (Timeline|Timeline_0 PlayFromStart)
        (:Update
          (bind _asbp_player_character (Utilities|Casting|CastToBP_PlayerCharacter (Game|Player|GetPlayerPawn 0)))
          (Transformation|SetActorLocation (Math|Vector|Lerp(Vector) (Transformation|GetActorLocation) (Transformation|GetActorLocation _asbp_player_character) _positionalpha) false false))))))

(event EventTick
  (params (DeltaSeconds :type Float%20%28single-precision%29))
  (if (Class|PrimitiveComponent|IsOverlappingComponent (Variables|Default|GetSphere) (Variables|/Script/Engine.Character|GetCapsuleComponent (Variables|Default|GetBP_PlayerCharacter)))
    (if (Variables|Default|GetCanGain)
      (Default|AddCoins (Variables|/Game/Player/Blueprints/BP_PlayerCharacter.BP_PlayerCharacter_C|GetBPC_Coins (Variables|Default|GetBP_PlayerCharacter)))
      (Actor|DestroyActor))))

(fn ConstructionScript)