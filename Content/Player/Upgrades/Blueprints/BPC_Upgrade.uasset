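; Player upgrade component that offers random, non-duplicate upgrade choices in a widget after a time-dilation ramp, then pauses the game.
; Major-threshold levels offer one-time special upgrades instead of tiered stat boosts.
; Picks either raise stats on the player's combat, dash and health components or bind effects to their dispatchers.
; Tiers and specials are stored in BP_SaveGame, cast from the GameInstance, and reapplied on BeginPlay by replaying each upgrade.
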(event Custom|ResetUpgrades
  (bind _returnvalue (Game|GetCurrentLevelName true))
  (if (Utilities|Enum|Equal(Enum) _returnvalue "WhiteBox_Test")
    _))

(event Custom|UpgradeChosen
  (params (UpgradeChosen :type E_Upgrades%20Enum :default "NewEnumerator0"))
  (bind _bp_playercharacter (Variables|Objects|GetBP_PlayerCharacter))
  (bind _bpc_playerrangedbasic (Variables|/Game/Player/Blueprints/BP_PlayerCharacter.BP_PlayerCharacter_C|GetBPC_PlayerRangedBasic _bp_playercharacter))
  (bind _bpc_playermeleebasic (Variables|/Game/Player/Blueprints/BP_PlayerCharacter.BP_PlayerCharacter_C|GetBPC_PlayerMeleeBasic _bp_playercharacter))
  ;[0.03529 0.03529 0.03529] Called When upgrade has been choosen (OnClick) and upgrades depending on upgrade chosen
  (Game|SetGamePaused false)
  (Rendering|SetVisibility (Variables|/Game/Player/Blueprints/BP_PlayerCharacter.BP_PlayerCharacter_C|GetHealthBar%20%28Widget%29 (Variables|Objects|GetBP_PlayerCharacter)) true false)
  (Default|TimeDilationDelay (Variables|Objects|GetBP_ThirdPersonGameMode) "/Game/UI/TimeDilation/UpgradeCurve.UpgradeCurve" true)
  (Utilities|ToggleUpgradeWidget false)
  (Default|ResetAllAttacks (Variables|/Game/Player/Blueprints/BP_PlayerCharacter.BP_PlayerCharacter_C|GetBPC_PlayerCombatHandler (Variables|Objects|GetBP_PlayerCharacter)))
  (switch Utilities|FlowControl|Switch|SwitchonE_Upgrades UpgradeChosen
    (:NewEnumerator1
      (BasicUpgrades|UpgradeHP "NewEnumerator1")
      (bind _asbp_save_game (Utilities|Casting|CastToBP_SaveGame (Game|GetGameInstance) :!label _label))
      (Variables|/Game/SaveSystem/BP_SaveGame.BP_SaveGame_C|SetUpgrade%20Tier _asbp_save_game (Variables|BasicUpgrades|GetS_Upgrades)))
    (:NewEnumerator3
      (BasicUpgrades|UpgradeDash "NewEnumerator3")
      (goto _label))
    (:NewEnumerator2
      (BasicUpgrades|UpgradeMeleeDamage "NewEnumerator2")
      (goto _label))
    (:NewEnumerator4
      (BasicUpgrades|UpgradeRangedDamage "NewEnumerator4")
      (goto _label))
    (:NewEnumerator9
      (BasicUpgrades|UpgradeSlam "NewEnumerator9")
      (goto _label))
    (:NewEnumerator8
      (BasicUpgrades|UpgradeHookDamage "NewEnumerator8")
      (goto _label))
    (:NewEnumerator6
      (BasicUpgrades|UpgradeMeleeAttackSpeed "NewEnumerator6")
      (goto _label))
    (:NewEnumerator7
      (BasicUpgrades|UpgradeRangedAttackSpeed "NewEnumerator7")
      (goto _label))
    (:NewEnumerator10
      (EventDispatchers|BindEventtoOnTriggerWeaponTrace _bpc_playermeleebasic (EventDispatchers|CreateEvent :!event UpgradeLifeSteal))
      (Utilities|Array|AddUnique (Variables|Default|GetE_TakenSpecialUpgrades) UpgradeChosen :!label _label_2)
      (bind _asbp_save_game_2 (Utilities|Casting|CastToBP_SaveGame (Game|GetGameInstance)))
      (Variables|/Game/SaveSystem/BP_SaveGame.BP_SaveGame_C|SetSpecial%20Upgrades _asbp_save_game_2 (Variables|Default|GetE_TakenSpecialUpgrades)))
    (:NewEnumerator12
      (EventDispatchers|BindEventtoOnTriggerSpawnProjectile _bpc_playerrangedbasic (EventDispatchers|CreateEvent :!event UpgradePiercingArrows))
      (goto _label_2))
    (:NewEnumerator13
      (EventDispatchers|BindEventtoOnDash (Variables|/Game/Player/Blueprints/BP_PlayerCharacter.BP_PlayerCharacter_C|GetBPC_PlayerDash _bp_playercharacter) (EventDispatchers|CreateEvent :!event UpgradeDashShield))
      (goto _label_2))
    (:NewEnumerator14
      (EventDispatchers|BindEventtoOnKnockbackUpgrade _bpc_playermeleebasic (EventDispatchers|CreateEvent :!event UpgradeMeleeKnockback))
      (goto _label_2))
    (:NewEnumerator15
      ;;[1 1 1] Unused
      (EventDispatchers|BindEventtoOnSplitUpgrade _bpc_playerrangedbasic (EventDispatchers|CreateEvent :!event UpgradeArrowSplit(Unused)))
      (goto _label_2))
    (:NewEnumerator16
      (Variables|/Game/Player/Blueprints/BP_PlayerCharacter.BP_PlayerCharacter_C|SetAttackSpeedKillstreak _bp_playercharacter true)
      (EventDispatchers|BindEventtoOnEnemyKillDispatcher _bp_playercharacter (EventDispatchers|CreateEvent :!event UpgradeAttackSpeedPerKill))
      (goto _label_2))
    (:NewEnumerator17
      (Variables|/Game/Player/Blueprints/BP_PlayerCharacter.BP_PlayerCharacter_C|SetAttackDamageKillstreak _bp_playercharacter true)
      (EventDispatchers|BindEventtoOnEnemyKillDispatcher _bp_playercharacter (EventDispatchers|CreateEvent :!event UpgradeAttackDamagePerKill))
      (goto _label_2))))

(event Custom|DelayFinished
  ;[0.03529 0.03529 0.03529] Shows upgrade widget
  (Utilities|ToggleUpgradeWidget true)
  (CallFunction|GenerateRandomUpgrades self)
  (Default|CallShowUpgradeWidget (Variables|Objects|GetWB_UpgradeWidget) (Variables|Default|GetE_UpgradePerChoice))
  (Game|SetGamePaused true))

(event Custom|ShowUpgrades
  ;[0.03529 0.03529 0.03529] Shows upgrade widget
  (Default|TimeDilationDelay (Variables|Objects|GetBP_ThirdPersonGameMode) "/Game/UI/TimeDilation/UpgradeCurve.UpgradeCurve" false)
  (Utilities|FlowControl|Delay 0.3)
  (Rendering|SetVisibility (Variables|/Game/Player/Blueprints/BP_PlayerCharacter.BP_PlayerCharacter_C|GetHealthBar%20%28Widget%29 (Variables|Objects|GetBP_PlayerCharacter)) false false))

(event EventBeginPlay
  ;[0.03529 0.03529 0.03529] Setup
  (|GetObjects)
  (|BindEvents)
  (bind _returnvalue (UserInterface|CreateWidget "/Game/Player/Upgrades/Blueprints/WB_UpgradePopUp.WB_UpgradePopUp_C" (Game|GetPlayerController 0) (Variables|Objects|GetBP_PlayerCharacter) (Variables|Default|GetE_UpgradePerChoice)))
  (bind _output_get (Variables|Objects|SetWB_UpgradeWidget _returnvalue))
  (UserInterface|SetWidget (Variables|/Game/Player/Blueprints/BP_PlayerCharacter.BP_PlayerCharacter_C|GetUpgrade%20%28Widget%29 (Variables|Objects|GetBP_PlayerCharacter)) _output_get)
  (Utilities|ToggleUpgradeWidget false)
  (bind _asbp_save_game (Utilities|Casting|CastToBP_SaveGame (Game|GetGameInstance)))
  (for _array_element (Variables|BasicUpgrades|GetE_Upgrades)
    (CallFunction|LoadUpgrades _array_element (.UpgradeTier (Utilities|Struct|BreakS_Upgrades (.Value (Utilities|Map|Find (Variables|/Game/SaveSystem/BP_SaveGame.BP_SaveGame_C|GetUpgrade%20Tier _asbp_save_game) _array_element)))) (.UpgradeTier (Utilities|Struct|BreakS_Upgrades (.Value (Utilities|Map|Find (Variables|/Game/SaveSystem/BP_SaveGame.BP_SaveGame_C|GetUpgrade%20Tier _asbp_save_game) _array_element)))) (.UpgradeTier (Utilities|Struct|BreakS_Upgrades (.Value (Utilities|Map|Find (Variables|/Game/SaveSystem/BP_SaveGame.BP_SaveGame_C|GetUpgrade%20Tier _asbp_save_game) _array_element)))) (.UpgradeTier (Utilities|Struct|BreakS_Upgrades (.Value (Utilities|Map|Find (Variables|/Game/SaveSystem/BP_SaveGame.BP_SaveGame_C|GetUpgrade%20Tier _asbp_save_game) _array_element)))) (.UpgradeTier (Utilities|Struct|BreakS_Upgrades (.Value (Utilities|Map|Find (Variables|/Game/SaveSystem/BP_SaveGame.BP_SaveGame_C|GetUpgrade%20Tier _asbp_save_game) _array_element)))) (.UpgradeTier (Utilities|Struct|BreakS_Upgrades (.Value (Utilities|Map|Find (Variables|/Game/SaveSystem/BP_SaveGame.BP_SaveGame_C|GetUpgrade%20Tier _asbp_save_game) _array_element)))) (.UpgradeTier (Utilities|Struct|BreakS_Upgrades (.Value (Utilities|Map|Find (Variables|/Game/SaveSystem/BP_SaveGame.BP_SaveGame_C|GetUpgrade%20Tier _asbp_save_game) _array_element)))) (.UpgradeTier (Utilities|Struct|BreakS_Upgrades (.Value (Utilities|Map|Find (Variables|/Game/SaveSystem/BP_SaveGame.BP_SaveGame_C|GetUpgrade%20Tier _asbp_save_game) _array_element)))))
    (bind _returnvalue_2 (Game|GetCurrentLevelName true))
    (if (Utilities|Enum|Equal(Enum) _returnvalue_2 "WhiteBox_Test")
      _))
  (for _array_element_2 (Variables|/Game/SaveSystem/BP_SaveGame.BP_SaveGame_C|GetSpecial%20Upgrades _asbp_save_game)
    (CallFunction|LoadSpecialUpgrades _array_element_2)))

(fn GenerateRandomUpgrades
  (bind _bp_playercharacter (Variables|Objects|GetBP_PlayerCharacter))
  (bind _bpc_levelup (Variables|/Game/Player/Blueprints/BP_PlayerCharacter.BP_PlayerCharacter_C|GetBPC_LevelUp _bp_playercharacter))
  ;[0.03529 0.03529 0.03529] Sets TEMPUpgrades so i can remove upgrade indexes from array and prevent duplicates
  (LocalVariables|SetTEMPUpgrades (Variables|BasicUpgrades|GetE_Upgrades))
  ;[0.03529 0.03529 0.03529] Remove special upgrades that can only be taken once. Empty per default
  (for _array_element (Variables|Default|GetE_TakenSpecialUpgrades)
    (Utilities|Array|RemoveItem (Variables|SpecialUpgrades|GetE_SpecialUpgrades) _array_element))
  (bind _keys (Utilities|Map|Keys (Variables|Default|GetE_UpgradeChoices)))
  ;[0.03529 0.03529 0.03529] Major  Upgrade Check
  (Math|Integer|CompareInt (Math|Integer|%(Integer) (Variables|/Game/Player/Blueprints/BPC_LevelUp.BPC_LevelUp_C|GetCurrentPlayerLevel _bpc_levelup) (Variables|/Game/Player/Blueprints/BPC_LevelUp.BPC_LevelUp_C|GetMajorUpgradeThreshold _bpc_levelup))
    (:>
      _)
    (:==
      ;[0.03529 0.03529 0.03529] Make only unique upgrades available
      (Utilities|Array|Clear (LocalVariables|GetTEMPUpgrades))
      (for _array_element_2 (Variables|SpecialUpgrades|GetE_SpecialUpgrades)
        (Utilities|Array|AddUnique (LocalVariables|GetTEMPUpgrades) _array_element_2))))
  ;[0.03529 0.03529 0.03529 1 19] Find & set TEMPRandomUpgrade -> add into map with choice x as key -> remove TEMPRandomUpgrade index from TEMPUpgrades -> repeat
  (for _array_element_3 _keys
    (bind _output_get (LocalVariables|SetTEMPRandomUpgrade (.OutItem (Utilities|Array|Random (LocalVariables|GetTEMPUpgrades)))))
    (Utilities|Map|Add (Variables|Default|GetE_UpgradePerChoice) _array_element_3 _output_get)
    (Utilities|Array|RemoveItem (LocalVariables|GetTEMPUpgrades) _output_get)))

(fn UpgradeHP
  (params (E_Upgrade :type E_Upgrades%20Enum :default "NewEnumerator5"))
  (bind _bp_playercharacter (Variables|Objects|GetBP_PlayerCharacter))
  (bind _s_upgrades (Variables|BasicUpgrades|GetS_Upgrades))
  (bind _value (Utilities|Map|Find _s_upgrades E_Upgrade))
  (bind _bpc_damagesystem (Variables|/Game/Player/Blueprints/BP_PlayerCharacter.BP_PlayerCharacter_C|GetBPC_DamageSystem _bp_playercharacter))
  (bind (_upgradetier _upgradevalue) (Utilities|Struct|BreakS_Upgrades _value))
  (bind _result (Math|Integer|IncrementInt _upgradetier)
    (:%20%20
      (Utilities|StoreTempEUpgrade _s_upgrades _value E_Upgrade _result _upgradevalue)
      (bind _output_get (LocalVariables|SetNewMaxHealth (* (+ (/ _upgradevalue 1e+02) 1.0) (Variables|/Game/DamageSystem/BPC_DamageSystem.BPC_DamageSystem_C|GetmaxHealth (Variables|/Game/Player/Blueprints/BP_PlayerCharacter.BP_PlayerCharacter_C|GetBPC_DamageSystem (Variables|Objects|GetBP_PlayerCharacter))))))
      ;[0.08854 0.08854 0.08854] Set current Health to (NewMaxHealth - MaxHealth) + Health
      ; This will add the hp gained from the upgrade to current health
      (Variables|/Game/DamageSystem/BPC_DamageSystem.BPC_DamageSystem_C|Sethealth _bpc_damagesystem (+ (- _output_get (Variables|/Game/DamageSystem/BPC_DamageSystem.BPC_DamageSystem_C|GetmaxHealth _bpc_damagesystem)) (Variables|/Game/DamageSystem/BPC_DamageSystem.BPC_DamageSystem_C|Gethealth _bpc_damagesystem)))
      (bind _output_get_2 (Variables|/Game/DamageSystem/BPC_DamageSystem.BPC_DamageSystem_C|SetmaxHealth _bpc_damagesystem _output_get))
      (Development|PrintString (Utilities|String|ToString(Float) _output_get_2)))))

(fn UpgradeDash
  (params (E_Upgrade :type E_Upgrades%20Enum :default "NewEnumerator5"))
  (bind _bp_playercharacter (Variables|Objects|GetBP_PlayerCharacter))
  (bind _s_upgrades (Variables|BasicUpgrades|GetS_Upgrades))
  (bind _value (Utilities|Map|Find _s_upgrades E_Upgrade))
  (bind _bpc_playerdash (Variables|/Game/Player/Blueprints/BP_PlayerCharacter.BP_PlayerCharacter_C|GetBPC_PlayerDash _bp_playercharacter))
  (bind (_upgradetier _upgradevalue) (Utilities|Struct|BreakS_Upgrades _value))
  (bind _result (Math|Integer|IncrementInt _upgradetier)
    (:%20%20
      (Utilities|StoreTempEUpgrade _s_upgrades _value E_Upgrade _result _upgradevalue)
      (Variables|/Game/Player/Blueprints/BPC_PlayerDash.BPC_PlayerDash_C|SetDash%20CDDuration _bpc_playerdash (+ (Variables|/Game/Player/Blueprints/BPC_PlayerDash.BPC_PlayerDash_C|GetDash%20CDDuration _bpc_playerdash) _upgradevalue)))))

(fn UpgradeMeleeDamage
  (params (E_Upgrade :type E_Upgrades%20Enum :default "NewEnumerator5"))
  (bind _s_upgrades (Variables|BasicUpgrades|GetS_Upgrades))
  (bind _bp_playercharacter (Variables|Objects|GetBP_PlayerCharacter))
  (bind _value (Utilities|Map|Find _s_upgrades E_Upgrade))
  (bind _bpc_playermeleebasic (Variables|/Game/Player/Blueprints/BP_PlayerCharacter.BP_PlayerCharacter_C|GetBPC_PlayerMeleeBasic _bp_playercharacter))
  (bind (_upgradetier _upgradevalue) (Utilities|Struct|BreakS_Upgrades _value))
  (bind _result (Math|Integer|IncrementInt _upgradetier)
    (:%20%20
      (Utilities|StoreTempEUpgrade _s_upgrades _value E_Upgrade _result _upgradevalue)
      (Variables|/Game/Player/Blueprints/BPC_PlayerCombatHandler.BPC_PlayerCombatHandler_C|SetMinDamage _bpc_playermeleebasic (+ _upgradevalue (Variables|/Game/Player/Blueprints/BPC_PlayerCombatHandler.BPC_PlayerCombatHandler_C|GetMinDamage _bpc_playermeleebasic)))
      (Variables|/Game/Player/Blueprints/BPC_PlayerCombatHandler.BPC_PlayerCombatHandler_C|SetMaxDamage _bpc_playermeleebasic (+ _upgradevalue (Variables|/Game/Player/Blueprints/BPC_PlayerCombatHandler.BPC_PlayerCombatHandler_C|GetMaxDamage _bpc_playermeleebasic)))
      (Development|PrintString (Utilities|String|ToString(Float) (Variables|/Game/Player/Blueprints/BPC_PlayerCombatHandler.BPC_PlayerCombatHandler_C|GetMaxDamage _bpc_playermeleebasic))))))

(fn UpgradeRangedDamage
  (params (E_Upgrade :type E_Upgrades%20Enum :default "NewEnumerator5"))
  (bind _bp_playercharacter (Variables|Objects|GetBP_PlayerCharacter))
  (bind _s_upgrades (Variables|BasicUpgrades|GetS_Upgrades))
  (bind _value (Utilities|Map|Find _s_upgrades E_Upgrade))
  (bind _bpc_playerrangedbasic (Variables|/Game/Player/Blueprints/BP_PlayerCharacter.BP_PlayerCharacter_C|GetBPC_PlayerRangedBasic _bp_playercharacter))
  (bind (_upgradetier _upgradevalue) (Utilities|Struct|BreakS_Upgrades _value))
  (bind _result (Math|Integer|IncrementInt _upgradetier)
    (:%20%20
      (Utilities|StoreTempEUpgrade _s_upgrades _value E_Upgrade _result _upgradevalue)
      (Variables|/Game/Player/Blueprints/BPC_PlayerCombatHandler.BPC_PlayerCombatHandler_C|SetMinDamage _bpc_playerrangedbasic (+ _upgradevalue (Variables|/Game/Player/Blueprints/BPC_PlayerCombatHandler.BPC_PlayerCombatHandler_C|GetMinDamage _bpc_playerrangedbasic)))
      (Variables|/Game/Player/Blueprints/BPC_PlayerCombatHandler.BPC_PlayerCombatHandler_C|SetMaxDamage _bpc_playerrangedbasic (+ _upgradevalue (Variables|/Game/Player/Blueprints/BPC_PlayerCombatHandler.BPC_PlayerCombatHandler_C|GetMaxDamage _bpc_playerrangedbasic))))))

(fn UpgradeSlam
  (params (E_Upgrade :type E_Upgrades%20Enum :default "NewEnumerator5"))
  (bind _bp_playercharacter (Variables|Objects|GetBP_PlayerCharacter))
  (bind _s_upgrades (Variables|BasicUpgrades|GetS_Upgrades))
  (bind _value (Utilities|Map|Find _s_upgrades E_Upgrade))
  (bind _bpc_playermeleeheavy (Variables|/Game/Player/Blueprints/BP_PlayerCharacter.BP_PlayerCharacter_C|GetBPC_PlayerMeleeHeavy _bp_playercharacter))
  (bind (_upgradetier _upgradevalue) (Utilities|Struct|BreakS_Upgrades _value))
  (bind _result (Math|Integer|IncrementInt _upgradetier)
    (:%20%20
      (Utilities|StoreTempEUpgrade _s_upgrades _value E_Upgrade _result _upgradevalue)
      (Variables|/Game/Player/Blueprints/BPC_PlayerCombatHandler.BPC_PlayerCombatHandler_C|SetMinDamage _bpc_playermeleeheavy (+ _upgradevalue (Variables|/Game/Player/Blueprints/BPC_PlayerCombatHandler.BPC_PlayerCombatHandler_C|GetMinDamage _bpc_playermeleeheavy)))
      (Variables|/Game/Player/Blueprints/BPC_PlayerCombatHandler.BPC_PlayerCombatHandler_C|SetMaxDamage _bpc_playermeleeheavy (+ _upgradevalue (Variables|/Game/Player/Blueprints/BPC_PlayerCombatHandler.BPC_PlayerCombatHandler_C|GetMaxDamage _bpc_playermeleeheavy))))))

(fn UpgradeHookDamage
  (params (E_Upgrade :type E_Upgrades%20Enum :default "NewEnumerator5"))
  (bind _bp_playercharacter (Variables|Objects|GetBP_PlayerCharacter))
  (bind _s_upgrades (Variables|BasicUpgrades|GetS_Upgrades))
  (bind _value (Utilities|Map|Find _s_upgrades E_Upgrade))
  (bind _bpc_playerhook (Variables|/Game/Player/Blueprints/BP_PlayerCharacter.BP_PlayerCharacter_C|GetBPC_PlayerHook _bp_playercharacter))
  (bind (_upgradetier _upgradevalue) (Utilities|Struct|BreakS_Upgrades _value))
  (bind _result (Math|Integer|IncrementInt _upgradetier)
    (:%20%20
      (Utilities|StoreTempEUpgrade _s_upgrades _value E_Upgrade _result _upgradevalue)
      (Variables|/Game/Player/Blueprints/BPC_PlayerCombatHandler.BPC_PlayerCombatHandler_C|SetMinDamage _bpc_playerhook (+ _upgradevalue (Variables|/Game/Player/Blueprints/BPC_PlayerCombatHandler.BPC_PlayerCombatHandler_C|GetMinDamage _bpc_playerhook)))
      (Variables|/Game/Player/Blueprints/BPC_PlayerCombatHandler.BPC_PlayerCombatHandler_C|SetMaxDamage _bpc_playerhook (+ _upgradevalue (Variables|/Game/Player/Blueprints/BPC_PlayerCombatHandler.BPC_PlayerCombatHandler_C|GetMaxDamage _bpc_playerhook))))))

(fn UpgradeMeleeAttackSpeed
  (params (E_Upgrade :type E_Upgrades%20Enum :default "NewEnumerator5"))
  (bind _bp_playercharacter (Variables|Objects|GetBP_PlayerCharacter))
  (bind _s_upgrades (Variables|BasicUpgrades|GetS_Upgrades))
  (bind _value (Utilities|Map|Find _s_upgrades E_Upgrade))
  (bind _bpc_playermeleebasic (Variables|/Game/Player/Blueprints/BP_PlayerCharacter.BP_PlayerCharacter_C|GetBPC_PlayerMeleeBasic _bp_playercharacter))
  (bind (_upgradetier _upgradevalue) (Utilities|Struct|BreakS_Upgrades _value))
  (bind _result (Math|Integer|IncrementInt _upgradetier)
    (:%20%20
      (Utilities|StoreTempEUpgrade _s_upgrades _value E_Upgrade _result _upgradevalue)
      (Variables|/Game/Player/Blueprints/BPC_PlayerCombatHandler.BPC_PlayerCombatHandler_C|SetAnimationPlayRate _bpc_playermeleebasic (+ _upgradevalue (Variables|/Game/Player/Blueprints/BPC_PlayerCombatHandler.BPC_PlayerCombatHandler_C|GetAnimationPlayRate _bpc_playermeleebasic))))))

(fn UpgradeRangedAttackSpeed
  (params (E_Upgrade :type E_Upgrades%20Enum :default "NewEnumerator5"))
  (bind _s_upgrades (Variables|BasicUpgrades|GetS_Upgrades))
  (bind _bp_playercharacter (Variables|Objects|GetBP_PlayerCharacter))
  (bind _value (Utilities|Map|Find _s_upgrades E_Upgrade))
  (bind _bpc_playerrangedbasic (Variables|/Game/Player/Blueprints/BP_PlayerCharacter.BP_PlayerCharacter_C|GetBPC_PlayerRangedBasic _bp_playercharacter))
  (bind (_upgradetier _upgradevalue) (Utilities|Struct|BreakS_Upgrades _value))
  (bind _result (Math|Integer|IncrementInt _upgradetier)
    (:%20%20
      (Utilities|StoreTempEUpgrade _s_upgrades _value E_Upgrade _result _upgradevalue)
      (Variables|/Game/Player/Blueprints/BPC_PlayerCombatHandler.BPC_PlayerCombatHandler_C|SetAnimationPlayRate _bpc_playerrangedbasic (+ _upgradevalue (Variables|/Game/Player/Blueprints/BPC_PlayerCombatHandler.BPC_PlayerCombatHandler_C|GetAnimationPlayRate _bpc_playerrangedbasic))))))

(fn UpgradeLifeSteal
  (bind _bp_playercharacter (Variables|Objects|GetBP_PlayerCharacter))
  (bind _bpc_damagesystem (Variables|/Game/Player/Blueprints/BP_PlayerCharacter.BP_PlayerCharacter_C|GetBPC_DamageSystem _bp_playercharacter))
  (bind _maxhealth (Variables|/Game/DamageSystem/BPC_DamageSystem.BPC_DamageSystem_C|GetmaxHealth _bpc_damagesystem))
  (for _array_element (Variables|/Game/Player/Blueprints/BPC_PlayerMeleeBasic.BPC_PlayerMeleeBasic_C|GetactorHitByTrace (Variables|/Game/Player/Blueprints/BP_PlayerCharacter.BP_PlayerCharacter_C|GetBPC_PlayerMeleeBasic _bp_playercharacter))
    (Math|Float|CompareFloat (+ (Variables|/Game/DamageSystem/BPC_DamageSystem.BPC_DamageSystem_C|Gethealth _bpc_damagesystem) (/ _maxhealth 1e+03)) _maxhealth
      (:>
        (Variables|/Game/DamageSystem/BPC_DamageSystem.BPC_DamageSystem_C|Sethealth _bpc_damagesystem _maxhealth :!label _label))
      (:==
        (goto _label))
      (:<
        (Variables|/Game/DamageSystem/BPC_DamageSystem.BPC_DamageSystem_C|Sethealth _bpc_damagesystem (+ (Variables|/Game/DamageSystem/BPC_DamageSystem.BPC_DamageSystem_C|Gethealth _bpc_damagesystem) (/ _maxhealth 1e+03)))))))

(fn UpgradePiercingArrows
  (Variables|/Game/Projectile/Blueprints/BP_ProjectileArrow.BP_ProjectileArrow_C|SetIsPiercing (Variables|/Game/Player/Blueprints/BPC_PlayerRangedBasic.BPC_PlayerRangedBasic_C|GetSpawnedArrow (Variables|/Game/Player/Blueprints/BP_PlayerCharacter.BP_PlayerCharacter_C|GetBPC_PlayerRangedBasic (Variables|Objects|GetBP_PlayerCharacter))) true))

(fn UpgradeDashShield
  (Variables|/Game/DamageSystem/BPC_DamageSystem.BPC_DamageSystem_C|SetisInvincible (Variables|/Game/Player/Blueprints/BP_PlayerCharacter.BP_PlayerCharacter_C|GetBPC_DamageSystem (Variables|Objects|GetBP_PlayerCharacter)) (Variables|Default|GetIs%20Invincible))
  (if (Variables|Default|GetIs%20Invincible)
    (Components|Activation|Activate (Variables|/Game/Player/Blueprints/BP_PlayerCharacter.BP_PlayerCharacter_C|GetDash_shield (Variables|Objects|GetBP_PlayerCharacter)) false)))

(fn LoadUpgrades
  (params (Selection :type E_Upgrades%20Enum :default "NewEnumerator5") (LastIndex :type Integer) (LastIndex2 :type Integer) (LastIndex3 :type Integer) (LastIndex4 :type Integer) (LastIndex5 :type Integer) (LastIndex6 :type Integer) (LastIndex7 :type Integer) (LastIndex8 :type Integer))
  (switch Utilities|FlowControl|Switch|SwitchonE_Upgrades Selection
    (:NewEnumerator1
      (for _index (range 1 LastIndex3)
        (BasicUpgrades|UpgradeHP "NewEnumerator1")))
    (:NewEnumerator3
      (for _index_2 (range 1 LastIndex)
        (BasicUpgrades|UpgradeDash "NewEnumerator3")))
    (:NewEnumerator2
      (for _index_3 (range 1 LastIndex2)
        (BasicUpgrades|UpgradeMeleeDamage "NewEnumerator2")))
    (:NewEnumerator4
      (for _index_4 (range 1 LastIndex6)
        (BasicUpgrades|UpgradeRangedDamage "NewEnumerator4")))
    (:NewEnumerator9
      (for _index_5 (range 1 LastIndex5)
        (BasicUpgrades|UpgradeSlam "NewEnumerator9")))
    (:NewEnumerator8
      (for _index_6 (range 1 LastIndex4)
        (BasicUpgrades|UpgradeHookDamage "NewEnumerator8")))
    (:NewEnumerator6
      (for _index_7 (range 1 LastIndex8)
        (BasicUpgrades|UpgradeMeleeAttackSpeed "NewEnumerator6")))
    (:NewEnumerator7
      (for _index_8 (range 1 LastIndex7)
        (BasicUpgrades|UpgradeRangedAttackSpeed "NewEnumerator7")))))

(fn UpgradeMeleeKnockback
  (for _array_element (Variables|/Game/Player/Blueprints/BPC_PlayerMeleeBasic.BPC_PlayerMeleeBasic_C|GetactorHitByTrace (Variables|/Game/Player/Blueprints/BP_PlayerCharacter.BP_PlayerCharacter_C|GetBPC_PlayerMeleeBasic (Variables|Objects|GetBP_PlayerCharacter)))
    (bind _asbp_enemy_base (Utilities|Casting|CastToBP_EnemyBase _array_element))
    (Default|Knockback _asbp_enemy_base 1.5e+03)))

(fn UpgradeArrowSplit(Unused)
  (bind _returnvalue (Math|Random|RandomFloatinRange 1.0 5.0))
  (bind _bp_playercharacter (Variables|Objects|GetBP_PlayerCharacter))
  (bind _bpc_playerrangedbasic (Variables|/Game/Player/Blueprints/BP_PlayerCharacter.BP_PlayerCharacter_C|GetBPC_PlayerRangedBasic _bp_playercharacter))
  (bind _spawnedarrow (Variables|/Game/Player/Blueprints/BPC_PlayerRangedBasic.BPC_PlayerRangedBasic_C|GetSpawnedArrow _bpc_playerrangedbasic))
  (bind _projectilemovement (Variables|/Game/Projectile/Blueprints/BP_ProjectileBase.BP_ProjectileBase_C|GetProjectileMovement _spawnedarrow))
  (for _index (range 0 2)
    (Variables|/Game/Player/Blueprints/BPC_PlayerRangedBasic.BPC_PlayerRangedBasic_C|SetSpawn%20Transform _bpc_playerrangedbasic (Variables|/Game/Projectile/Blueprints/BP_ProjectileArrow.BP_ProjectileArrow_C|GetHitTransform _spawnedarrow))
    (Variables|/Game/Player/Blueprints/BPC_PlayerRangedBasic.BPC_PlayerRangedBasic_C|SetSpawnSet _bpc_playerrangedbasic true)
    (Default|SpawnProjectile _bpc_playerrangedbasic)
    (Variables|/Script/Engine.MovementComponent|SetVelocity _projectilemovement (* (Variables|/Script/Engine.MovementComponent|GetVelocity _projectilemovement) (Math|Vector|MakeVector _returnvalue _returnvalue 1.0)))))

(fn UpgradeAttackSpeedPerKill
  (bind _bp_playercharacter (Variables|Objects|GetBP_PlayerCharacter))
  (bind _enemieskilled (Variables|/Game/Player/Blueprints/BP_PlayerCharacter.BP_PlayerCharacter_C|GetEnemiesKilled _bp_playercharacter))
  (bind _bpc_playercombathandler (Variables|/Game/Player/Blueprints/BP_PlayerCharacter.BP_PlayerCharacter_C|GetBPC_PlayerCombatHandler _bp_playercharacter))
  (bind _returnvalue (* _enemieskilled 0.1))
  (bind _bpc_playermeleebasic (Variables|/Game/Player/Blueprints/BPC_PlayerCombatHandler.BPC_PlayerCombatHandler_C|GetBPC_PlayerMeleeBasic _bpc_playercombathandler))
  (bind _bpc_playerrangedbasic (Variables|/Game/Player/Blueprints/BPC_PlayerCombatHandler.BPC_PlayerCombatHandler_C|GetBPC_PlayerRangedBasic _bpc_playercombathandler))
  (Variables|/Game/Player/Blueprints/BPC_PlayerCombatHandler.BPC_PlayerCombatHandler_C|SetAnimationPlayRate _bpc_playermeleebasic (+ _returnvalue (Variables|/Game/Player/Blueprints/BPC_PlayerCombatHandler.BPC_PlayerCombatHandler_C|GetAnimationPlayRate _bpc_playermeleebasic)))
  (Variables|/Game/Player/Blueprints/BPC_PlayerCombatHandler.BPC_PlayerCombatHandler_C|SetAnimationPlayRate _bpc_playerrangedbasic (+ (Variables|/Game/Player/Blueprints/BPC_PlayerCombatHandler.BPC_PlayerCombatHandler_C|GetAnimationPlayRate _bpc_playerrangedbasic) _returnvalue)))

(fn UpgradeAttackDamagePerKill
  (bind _bp_playercharacter (Variables|Objects|GetBP_PlayerCharacter))
  (bind _bpc_playercombathandler (Variables|/Game/Player/Blueprints/BP_PlayerCharacter.BP_PlayerCharacter_C|GetBPC_PlayerCombatHandler _bp_playercharacter))
  (bind _enemieskilled (Variables|/Game/Player/Blueprints/BP_PlayerCharacter.BP_PlayerCharacter_C|GetEnemiesKilled _bp_playercharacter))
  (bind _returnvalue (* _enemieskilled 1.5))
  (bind _bpc_playermeleebasic (Variables|/Game/Player/Blueprints/BPC_PlayerCombatHandler.BPC_PlayerCombatHandler_C|GetBPC_PlayerMeleeBasic _bpc_playercombathandler))
  (bind _bpc_playerrangedbasic (Variables|/Game/Player/Blueprints/BPC_PlayerCombatHandler.BPC_PlayerCombatHandler_C|GetBPC_PlayerRangedBasic _bpc_playercombathandler))
  (Variables|/Game/Player/Blueprints/BPC_PlayerCombatHandler.BPC_PlayerCombatHandler_C|SetMaxDamage _bpc_playermeleebasic (+ _returnvalue (Variables|/Game/Player/Blueprints/BPC_PlayerCombatHandler.BPC_PlayerCombatHandler_C|GetMaxDamage _bpc_playermeleebasic)))
  (Variables|/Game/Player/Blueprints/BPC_PlayerCombatHandler.BPC_PlayerCombatHandler_C|SetMinDamage _bpc_playermeleebasic (+ _returnvalue (Variables|/Game/Player/Blueprints/BPC_PlayerCombatHandler.BPC_PlayerCombatHandler_C|GetMinDamage _bpc_playermeleebasic)))
  (Variables|/Game/Player/Blueprints/BPC_PlayerCombatHandler.BPC_PlayerCombatHandler_C|SetMaxDamage _bpc_playerrangedbasic (+ _returnvalue (Variables|/Game/Player/Blueprints/BPC_PlayerCombatHandler.BPC_PlayerCombatHandler_C|GetMaxDamage _bpc_playerrangedbasic)))
  (Variables|/Game/Player/Blueprints/BPC_PlayerCombatHandler.BPC_PlayerCombatHandler_C|SetMinDamage _bpc_playerrangedbasic (+ _returnvalue (Variables|/Game/Player/Blueprints/BPC_PlayerCombatHandler.BPC_PlayerCombatHandler_C|GetMinDamage _bpc_playerrangedbasic))))

(fn LoadSpecialUpgrades
  (params (Selection :type E_Upgrades%20Enum :default "NewEnumerator5"))
  (bind _bp_playercharacter (Variables|Objects|GetBP_PlayerCharacter))
  (bind _bpc_playerrangedbasic (Variables|/Game/Player/Blueprints/BP_PlayerCharacter.BP_PlayerCharacter_C|GetBPC_PlayerRangedBasic _bp_playercharacter))
  (bind _bpc_playermeleebasic (Variables|/Game/Player/Blueprints/BP_PlayerCharacter.BP_PlayerCharacter_C|GetBPC_PlayerMeleeBasic _bp_playercharacter))
  (switch Utilities|FlowControl|Switch|SwitchonE_Upgrades Selection
    (:NewEnumerator10
      (EventDispatchers|BindEventtoOnTriggerWeaponTrace _bpc_playermeleebasic (EventDispatchers|CreateEvent :!event UpgradeLifeSteal)))
    (:NewEnumerator12
      (EventDispatchers|BindEventtoOnTriggerSpawnProjectile _bpc_playerrangedbasic (EventDispatchers|CreateEvent :!event UpgradePiercingArrows)))
    (:NewEnumerator13
      (EventDispatchers|BindEventtoOnDash (Variables|/Game/Player/Blueprints/BP_PlayerCharacter.BP_PlayerCharacter_C|GetBPC_PlayerDash _bp_playercharacter) (EventDispatchers|CreateEvent :!event UpgradeDashShield)))
    (:NewEnumerator14
      (EventDispatchers|BindEventtoOnKnockbackUpgrade _bpc_playermeleebasic (EventDispatchers|CreateEvent :!event UpgradeMeleeKnockback)))
    (:NewEnumerator15
      ;[1 1 1] Unused
      (EventDispatchers|BindEventtoOnSplitUpgrade _bpc_playerrangedbasic (EventDispatchers|CreateEvent :!event UpgradeArrowSplit(Unused))))
    (:NewEnumerator16
      (Variables|/Game/Player/Blueprints/BP_PlayerCharacter.BP_PlayerCharacter_C|SetAttackSpeedKillstreak _bp_playercharacter true)
      (EventDispatchers|BindEventtoOnEnemyKillDispatcher _bp_playercharacter (EventDispatchers|CreateEvent :!event UpgradeAttackSpeedPerKill)))
    (:NewEnumerator17
      (Variables|/Game/Player/Blueprints/BP_PlayerCharacter.BP_PlayerCharacter_C|SetAttackDamageKillstreak _bp_playercharacter true)
      (EventDispatchers|BindEventtoOnEnemyKillDispatcher _bp_playercharacter (EventDispatchers|CreateEvent :!event UpgradeAttackDamagePerKill))))
  (Utilities|Array|AddUnique (Variables|Default|GetE_TakenSpecialUpgrades) Selection))