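; Player melee component that plays an attack combo, or a spin attack when dashing, after turning toward the closest enemy.
; When not dashing and far enough from the target location, a looping timer repeatedly launches the character toward the enemy or cursor, with braking friction temporarily overridden.
; Animation-triggered events run a timed socket-to-socket sword trace, damaging each actor once per swing and reducing dash cooldown on each hit.
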(event Custom|TriggerSwordTrace
  ;[0.05098 0.05098 0.05098] Ray traces weapon animation when melee attacking
  (bind _returnvalue (Utilities|Time|SetTimerbyEvent (delegate Custom|SwordTraceLoop) 0.01 true))
  (Variables|Default|SetswordTracingTimerHandle _returnvalue))

(event Custom|SwordTraceLoop
  (bind _actorhitbytrace (Variables|Default|GetactorHitByTrace))
  (bind _sword (Variables|Default|GetSword))
  ;[0.05098 0.05098 0.05098] Ray traces weapon animation when melee attacking
  (bind _outhits (Collision|MultiLineTraceByChannel (Transformation|GetSocketLocation _sword "start") (Transformation|GetSocketLocation _sword "end") "TraceTypeQuery1" false 0 "None"))
  (bind _array_element (Utilities|Array|ForEachLoopwithBreak _outhits)
    (:LoopBody
      (if (not (Utilities|Array|ContainsItem _actorhitbytrace (.HitActor (Collision|BreakHitResult _array_element))))
        (Utilities|Array|Add _actorhitbytrace (.HitActor (Collision|BreakHitResult _array_element)))
        (Class|BPIDamagable|DealDamage(Message) (.HitActor (Collision|BreakHitResult _array_element)) (Utilities|Struct|MakeS_DamageInfo (Math|Random|RandomFloatinRange 9.0 24.0) "NewEnumerator0" "NewEnumerator1"))
        (Default|CallOnReduceDashCD (Variables|Default|GetBPC_PlayerDash) 8.0)))))

(event Custom|StopSwordTrace
  ;[0.05098 0.05098 0.05098] Ray traces weapon animation when melee attacking
  (Utilities|Time|ClearandInvalidateTimerbyHandle (Variables|Default|GetswordTracingTimerHandle))
  (Utilities|Array|Clear (Variables|Default|GetactorHitByTrace)))

(event Custom|ApplyForce
  (params (Strength :type Float%20%28double-precision%29))
  ;[0.05098 0.05098 0.05098] Apply force when melee attacking
  (if (not (Variables|/Game/Player/Blueprints/BPC_PlayerDash.BPC_PlayerDash_C|GetIs%20Dashing (Variables|Default|GetBPC_PlayerDash)))
    (if (>= (Math|Vector|Distance2D(Vector) (Variables|Default|GetTargetEnemyLocation) (Transformation|GetActorLocation (Variables|Default|GetBP_PlayerCharacter))) 225.0)
      (CallFunction|ApplyForceStartTimer)
      (Utilities|SetMousePOS)
      (Utilities|TogglesBrakingFriction))))

(event Custom|CancelSwordApplyForce
  ;[0.05098 0.05098 0.05098] Apply force when melee attacking
  (Utilities|Time|ClearandInvalidateTimerbyHandle (Variables|ApplyForce|GetapplyForceTimerHandle))
  (Variables|ApplyForce|SetapplyForceTimer 0.0))

(event Custom|MeleeAttack
  ;[0.05098 0.05098 0.05098] Attack
  (Variables|/Game/Player/Blueprints/BPC_PlayerCombat.BPC_PlayerCombat_C|SetIsAttacking (Variables|Default|GetBPC_PlayerMelee) true)
  (bind (_targettedenemy _enemylocation) (Default|GetClosestEnemy (Variables|Default|GetBPC_PlayerCombat)))
  (Variables|Default|SetTargetEnemy _targettedenemy)
  (Variables|Default|SetTargetEnemyLocation _enemylocation)
  (Default|ToggleEnableMovementInput (Variables|Default|GetBP_PlayerCharacter) false true)
  (Default|RotateTowardsEnemy (Variables|Default|GetBPC_PlayerCombat))
  (if (Variables|/Game/Player/Blueprints/BPC_PlayerDash.BPC_PlayerDash_C|GetIs%20Dashing (Variables|Default|GetBPC_PlayerDash))
    (CallFunction|MeleeDashAttack)
    (else
      (CallFunction|MeleeNormalAttack))))

(event Custom|MeleeNormalAttack
  ;[0.05098 0.05098 0.05098] Melee attack
  (CallFunction|ApplyForce (+ (Variables|ApplyForce|GetapplyForceStrength) 0.0))
  (Animation|Montage|PlayMontage (Variables|Default|GetPlayerMesh) (Utilities|Array|Get(acopy) (Variables|Default|GetattackAnims) (Variables|Default|GetattackCount)) 3.0
    (:then
      (Math|Integer|IncrementInt (Variables|Default|GetattackCount)))
    (:OnCompleted
      (Variables|Default|SetattackCount 0 :!label _label)
      (CallFunction|FinishedAttacking))
    (:OnInterrupted
      (Utilities|FlowControl|RetriggerableDelay 2.0)
      (goto _label))))

(event Custom|ApplyForceStartTimer
  ;[0.05098 0.05098 0.05098] Apply force when melee attacking
  (bind _returnvalue (Utilities|Time|SetTimerbyEvent (delegate Custom|ApplyForceStartTimer) 0.001 true))
  (CallFunction|ApplyForceTimerFunction _returnvalue)
  (bind (_returnvalue_x _returnvalue_y) (CallFunction|CalculateForce (stale Custom|ApplyForce Strength)))
  (Character|LaunchCharacter (Variables|Default|GetBP_PlayerCharacter) (Math|Vector|MakeVector _returnvalue_x _returnvalue_y 0.0) false false))

(event Custom|MeleeDashAttack
  ;[0.05098 0.05098 0.05098] Melee attack
  (CallFunction|ApplyForce (+ (Variables|ApplyForce|GetapplyForceStrength) 5e+01))
  (Animation|Montage|PlayMontage (Variables|Default|GetPlayerMesh) "/Game/Characters/Mannequins/Animations/Attack_Animations/StandingMeleeAttack360High_UE_Montage.StandingMeleeAttack360High_UE_Montage" 3.0
    (:OnCompleted
      _)
    (:OnInterrupted
      (Utilities|FlowControl|RetriggerableDelay 2.0)))
  (Default|FinishedAttacking (Variables|Default|GetBPC_PlayerCombat)))

(event EventBeginPlay
  ;[0.05098 0.05098 0.05098] Setup
  (|CallParentFunction)
  (Variables|Default|SetSword (Variables|/Game/Player/Blueprints/BP_PlayerCharacter.BP_PlayerCharacter_C|GetSword (Variables|Default|GetBP_PlayerCharacter)))
  (EventDispatchers|BindEventtoOnDashCancelOtherForces (Variables|Default|GetBPC_PlayerDash) (EventDispatchers|CreateEvent :!event Custom|CancelSwordApplyForce)))

(fn ApplyForceTimerFunction
  (params (TimerHandle :type Timer%20Handle%20Structure))
  (Variables|ApplyForce|SetapplyForceTimerHandle TimerHandle)
  (bind _output_get (Variables|ApplyForce|SetapplyForceTimer (+ 0.01 (Variables|ApplyForce|GetapplyForceTimer))))
  (if (>= (Variables|ApplyForce|GetapplyForceDuration) _output_get)
    (return)
    (else
      (CallFunction|CancelSwordApplyForce))))

(fn CheckCanAttack
  (bind _canattack (|CallParentFunction))
  (if _canattack
    (if (Variables|/Game/Player/Blueprints/BPC_PlayerCombat.BPC_PlayerCombat_C|GetCanAttack (Variables|Default|GetBPC_PlayerMelee))
      (if (== (Variables|Default|GetattackCount) 4)
        (return false)
        (else
          (return true)))
      (else
        (return false)))
    (else
      (return false))))

(fn HandleFinishedAttacking
  (bind _bpc_playermelee (Variables|Default|GetBPC_PlayerMelee))
  (|CallParentFunction)
  (Variables|/Game/Player/Blueprints/BPC_PlayerCombat.BPC_PlayerCombat_C|SetCanAttack _bpc_playermelee true)
  (if (>= (Variables|BPC_PlayerMelee_C|GetattackCount _bpc_playermelee) 4)
    (Variables|BPC_PlayerMelee_C|SetattackCount _bpc_playermelee 0)))

(fn CalculateForce
  (params (Strength :type Float%20%28double-precision%29))
  (bind _bp_playercharacter (Variables|Default|GetBP_PlayerCharacter))
  (bind _savedmousepos (Variables|Default|GetSavedMousePOS))
  (bind _targetenemy (Variables|Default|GetTargetEnemy))
  (bind _targetenemylocation (Variables|Default|GetTargetEnemyLocation))
  (bind _returnvalue (Utilities|IsValid _targetenemy))
  (bind _returnvalue_2 (Transformation|GetActorLocation _bp_playercharacter))
  (bind _returnvalue_3 (- _targetenemylocation _returnvalue_2))
  (bind _returnvalue_4 (- _savedmousepos _returnvalue_2))
  (bind _returnvalue_5 (Math|Vector|SelectVector _returnvalue_3 _returnvalue_4 _returnvalue))
  (bind _returnvalue_6 (Math|Vector|Normalize _returnvalue_5))
  (bind _returnvalue_7 (* Strength _returnvalue_6))
  (return (.x _returnvalue_7) (.y _returnvalue_7)))