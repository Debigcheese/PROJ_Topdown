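; Player component for the basic bow attack, firing arrow projectiles at a targeted enemy or the mouse position.
; An attack locks movement input, turns the player to the target or to the cursor's line-plane intersection at bow height, then plays a montage.
; The animation triggers the arrow spawn with randomized damage.
; Attacks require ground movement, and finishing clears un-hovered targets; the max-range check is disconnected.
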(event Custom|SpawnProjectile
  (bind _bp_playercharacter (Variables|Default|GetBP_PlayerCharacter))
  (bind _bpc_playerrangedbasic (Variables|Default|GetBPC_PlayerRangedBasic))
  ;[0.05098 0.05098 0.05098] SpawnProjectile (from animation)
  (Audio|PlaySound2D "/Game/Audio/Player/player_shooting_arrow.player_shooting_arrow" 1.0 1.0 0.0 0 0)
  (if (Variables|Default|GetSpawnSet)
    (Variables|Default|SetRotateLocation (Math|Random|RandomUnitVector))
    (Variables|Default|SetSpawnSet false)
    (else
      (bind _output_get (Variables|Default|SetSpawn%20Transform (Transformation|GetWorldTransform (Variables|/Game/Player/Blueprints/BP_PlayerCharacter.BP_PlayerCharacter_C|GetBowShootPoint _bp_playercharacter))))))
  (bind _returnvalue (Game|SpawnActorfromClass "/Game/Projectile/Blueprints/BP_ProjectileArrow.BP_ProjectileArrow_C" _output_get "Undefined" "MultiplyWithRoot" _bp_playercharacter (Variables|Default|GetTargetEnemy) (Variables|Default|GetRotateLocation) false 0 "0.000000,0.000000,0.000000|0.000000,0.000000,-0.000000|1.000000,1.000000,1.000000" false 3e+03 0.1 false (Utilities|Struct|MakeS_DamageInfo (Math|Random|RandomFloatinRange (Variables|/Game/Player/Blueprints/BPC_PlayerCombatHandler.BPC_PlayerCombatHandler_C|GetMinDamage _bpc_playerrangedbasic) (Variables|/Game/Player/Blueprints/BPC_PlayerCombatHandler.BPC_PlayerCombatHandler_C|GetMaxDamage _bpc_playerrangedbasic)) "NewEnumerator1" "NewEnumerator2" "NewEnumerator0" "NewEnumerator1") false 0 0))
  (bind _output_get_2 (Variables|Default|SetSpawnedArrow _returnvalue))
  (Collision|IgnoreActorwhenMoving (Variables|/Script/Engine.Character|GetCapsuleComponent (Variables|Default|GetBP_PlayerCharacter)) _output_get_2 true)
  (Default|CallOnTriggerSpawnProjectile))

(event Custom|ToggleMaxRangeCircle
  (bind _bp_playercharacter (Variables|Default|GetBP_PlayerCharacter))
  (bind _returnvalue (Actor|GetComponentbyClass _bp_playercharacter "/Script/Niagara.NiagaraComponent"))
  ;[0.05098 0.05098 0.05098] MaxRangeVisibility
  (if (Components|ComponentHasTag _returnvalue "MaxRangeCircle")
    (Rendering|SetVisibility _returnvalue true false)
    (Utilities|FlowControl|RetriggerableDelay 1.4)
    (Rendering|SetVisibility _returnvalue false false)))

(event Custom|RangedBasicAttack
  ;[0.05098 0.05098 0.05098] Attack
  (Default|ToggleEnableMovementInput (Variables|Default|GetBP_PlayerCharacter) false true)
  (bind _targettedenemy (Default|GetTargettedEnemy (Variables|Default|GetBPC_PlayerCombatHandler)))
  (bind _output_get (Variables|Default|SetTargetEnemy _targettedenemy))
  (Utilities|IsValid _output_get
    (:Is%20Valid
      (CallFunction|RotateTowardsSelectedEnemyPOS _output_get))
    (:Is%20Not%20Valid
      (CallFunction|RotateTowardsMousePOS)))
  (Animation|Montage|PlayMontage (Variables|Default|GetPlayerMesh) (Utilities|Array|Get(acopy) (Variables|Default|GetattackAnims) 1) (Variables|/Game/Player/Blueprints/BPC_PlayerCombatHandler.BPC_PlayerCombatHandler_C|GetAnimationPlayRate (Variables|Default|GetBPC_PlayerRangedBasic))
    (:then
      (Audio|PlaySound2D "/Game/Audio/Player/BowChargeSFX.BowChargeSFX" 1.0 1.0 0.0 0 0))))

(event EventBeginPlay
  (bind _bp_playercharacter (Variables|Default|GetBP_PlayerCharacter))
  (bind _returnvalue (Actor|GetComponentbyClass _bp_playercharacter "/Script/Niagara.NiagaraComponent"))
  ;[0.05098 0.05098 0.05098] Setup
  (|CallParentFunction)
  (if (Components|ComponentHasTag _returnvalue "MaxRangeCircle")
    (Rendering|SetVisibility _returnvalue false false)))

(fn CheckCanAttack
  (bind _canattack (|CallParentFunction))
  (if _canattack
    (if (Variables|/Game/Player/Blueprints/BPC_PlayerCombatHandler.BPC_PlayerCombatHandler_C|GetCanAttack (Variables|Default|GetBPC_PlayerRangedBasic))
      (if (AI|Components|NavMovement|IsMovingonGround (Variables|Default|GetCharacterMovement))
        (return true)
        (else
          _))))
  (return false))

(fn HandleFinishedAttacking
  (bind _bpc_playercombathandler (Variables|Default|GetBPC_PlayerCombatHandler))
  (|CallParentFunction)
  (Variables|/Game/Player/Blueprints/BPC_PlayerCombatHandler.BPC_PlayerCombatHandler_C|SetCanAttack (Variables|Default|GetBPC_PlayerRangedBasic) true)
  (bind _asbp_enemy_base (Utilities|Casting|CastToBP_EnemyBase (Variables|/Game/Player/Blueprints/BPC_PlayerCombatHandler.BPC_PlayerCombatHandler_C|GetTargetEnemy _bpc_playercombathandler)))
  (if (not (Variables|/Game/Enemies/Blueprints/BP_EnemyBase.BP_EnemyBase_C|GetIsMouseHovering _asbp_enemy_base))
    (Default|SetTargettedEnemy _bpc_playercombathandler)))

(fn RotateTowardsMousePOS
  (bind _playerrotationz (CallFunction|FindRotationtoMousePOS (Variables|/Game/Player/Blueprints/BP_PlayerCharacter.BP_PlayerCharacter_C|GetBowShootPoint (Variables|Default|GetBP_PlayerCharacter))))
  (Transformation|SetActorRotation (Variables|Default|GetBP_PlayerCharacter) (Math|Rotator|MakeRotator 0.0 0.0 _playerrotationz)))

(fn FindRotationtoMousePOS
  (params (ShootPoint :type Scene%20Component%20Object%20Reference))
  (bind _returnvalue (Game|GetPlayerController 0))
  (bind _bp_playercharacter (Variables|Default|GetBP_PlayerCharacter))
  (bind (_worldlocation _worlddirection) (Game|Player|ConvertMouseLocationToWorldSpace _returnvalue))
  (bind _bowshootpoint (Variables|/Game/Player/Blueprints/BP_PlayerCharacter.BP_PlayerCharacter_C|GetBowShootPoint _bp_playercharacter))
  (bind _returnvalue_2 (Transformation|GetWorldLocation _bowshootpoint))
  (bind _returnvalue_3 (* _worlddirection 1e+04))
  (bind _returnvalue_4 (+ _worldlocation _returnvalue_3))
  (bind _intersection (Class|KismetMathLibrary|LinePlaneIntersectionOriginNormal _worldlocation _returnvalue_4 _returnvalue_2 "0.000000,0.000000,1.000000"))
  (Variables|Default|SetRotateLocation _intersection)
  (return (.yaw (Math|Rotator|FindLookatRotation (Transformation|GetActorLocation (Variables|Default|GetBP_PlayerCharacter)) _intersection))))