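; Player level-up component that accumulates experience and raises the player's level once a threshold is reached.
; An XP gain event adds to the current XP and triggers LevelUp when the total meets or exceeds the threshold.
; LevelUp increments the level and refills the player character's health to maximum through its damage system component.
; The threshold and current XP are not adjusted on level-up.
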(event Custom|LevelUp
  (Development|PrintString "lvld up")
  (Math|Integer|IncrementInt (Variables|Default|GetCurrentPlayerLevel)
    (:%20%20
      (bind _asbp_player_character (Utilities|Casting|CastToBP_PlayerCharacter (Game|Player|GetPlayerPawn 0)))
      (Variables|/Game/DamageSystem/BPC_DamageSystem.BPC_DamageSystem_C|Sethealth (Variables|/Game/Player/Blueprints/BP_PlayerCharacter.BP_PlayerCharacter_C|GetBPC_DamageSystem _asbp_player_character) (Variables|/Game/DamageSystem/BPC_DamageSystem.BPC_DamageSystem_C|GetmaxHealth (Variables|/Game/Player/Blueprints/BP_PlayerCharacter.BP_PlayerCharacter_C|GetBPC_DamageSystem _asbp_player_character))))))

(event Custom|OnXPGain_Event
  (params (XPGain :type Integer))
  (Variables|Default|SetXPGain XPGain)
  (bind _output_get (Variables|Default|SetCurrentXP (+ XPGain (Variables|Default|GetCurrentXP))))
  (Math|Integer|CompareInt _output_get (Variables|Default|GetXPThreshold)
    (:>
      _)
    (:==
      _))
  (CallFunction|LevelUp))