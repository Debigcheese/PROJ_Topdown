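; Player combat component for a charged heavy bow attack that fires a heavy arrow, with its own cooldown and attack gating.
; The attack disables movement and dash, loops an aim montage, and turns the player toward the mouse on a self-looping timer.
; HandleAimingTime stops rotation, then either cancels a too-short aim or spawns an arrow with randomized damage scaled by a stepped charge-time multiplier.
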(event Custom|HandleAimingTime
  (params (Elapsed%20Seconds :type Float%20%28double-precision%29))
  (bind _mintimetoaim (Variables|Default|GetMinTimeToAim))
  ;[0.05098 0.05098 0.05098] CheckChargingTime
  (CallFunction|StopRotating)
  (if (>= Elapsed%20Seconds _mintimetoaim)
    (bind _damagemultiplier (CallFunction|CalculateDamageMultiplier (- Elapsed%20Seconds _mintimetoaim) 0.3 1.5))
    (Variables|Default|SetDamageMultiplier _damagemultiplier)
    (CallFunction|SpawnProjectile)
    (else
      ;;[0.05098 0.05098 0.05098] CancelAimingRangedHeavy (? OPTION1)
      (Animation|StopAnimMontage (Variables|Default|GetBP_PlayerCharacter) 0)
      (Variables|Default|SetStopAimingBow false)
      (Variables|/Game/Player/Blueprints/BPC_PlayerCombatHandler.BPC_PlayerCombatHandler_C|SetCanAttack (Variables|Default|GetBPC_PlayerRangedHeavy) true)
      (CallFunction|HandleFinishedAttacking (Variables|Default|GetBPC_PlayerCombatHandler)))))

(event Custom|LerpActorRotationToMouse
  ;[0.05098 0.05098 0.05098] Rotate player to mouse location
  (bind _returnvalue (Utilities|Time|SetTimerbyEvent (delegate Custom|LerpActorRotationToMouse) 0.01 true))
  (bind _playerrotationz (CallFunction|FindRotationtoMousePOS (Variables|/Game/Player/Blueprints/BP_PlayerCharacter.BP_PlayerCharacter_C|GetBowShootPoint (Variables|Default|GetBP_PlayerCharacter))))
  (Transformation|SetActorRotation (Variables|Default|GetBP_PlayerCharacter) (Math|Rotator|MakeRotator 0.0 0.0 _playerrotationz)))

(event Custom|StopRotating
  ;[0.05098 0.05098 0.05098] Rotate player to mouse location
  (Utilities|Time|ClearandInvalidateTimerbyHandle (stale Custom|LerpActorRotationToMouse _returnvalue))
  (Default|ToggleEnableMovementInput (Variables|Default|GetBP_PlayerCharacter) true true))

(event Custom|SpawnProjectile
  (bind _bp_playercharacter (Variables|Default|GetBP_PlayerCharacter))
  ;[0.05098 0.05098 0.05098] SpawnProjectile - starts when q is released
  (bind _returnvalue (Game|SpawnActorfromClass "/Game/Projectile/Blueprints/BP_ProjectileHeavyArrow.BP_ProjectileHeavyArrow_C" (Transformation|GetWorldTransform (Variables|/Game/Player/Blueprints/BP_PlayerCharacter.BP_PlayerCharacter_C|GetBowShootPoint (Variables|Default|GetBP_PlayerCharacter))) "Undefined" "MultiplyWithRoot" 0 3.8e+03 0.0 false (Utilities|Struct|MakeS_DamageInfo (* (Math|Random|RandomFloatinRange 3e+01 4e+01) (Variables|Default|GetDamageMultiplier)) "NewEnumerator1" "NewEnumerator2") false 0 0))
  (Collision|IgnoreActorwhenMoving (Variables|/Script/Engine.Character|GetCapsuleComponent _bp_playercharacter) _returnvalue true)
  (Collision|IgnoreActorwhenMoving (Variables|/Game/Projectile/Blueprints/BP_ProjectileBase.BP_ProjectileBase_C|GetBoxCollision _returnvalue) _bp_playercharacter true)
  (Variables|Default|SetStopAimingBow true)
  (Animation|Montage|PlayMontage (Variables|Default|GetPlayerMesh) (Utilities|Array|Get(acopy) (Variables|Default|GetattackAnims) 2) 6.0
    (:OnCompleted
      _)
    (:OnInterrupted
      _))
  (Variables|Default|SetStopAimingBow false)
  (Variables|/Game/Player/Blueprints/BPC_PlayerCombatHandler.BPC_PlayerCombatHandler_C|SetCanAttack (Variables|Default|GetBPC_PlayerRangedHeavy) false))

(event Custom|RangedHeavyAttack
  ;[0.05098 0.05098 0.05098] Attack
  (Default|ToggleEnableMovementInput (Variables|Default|GetBP_PlayerCharacter) false false)
  (CallFunction|LerpActorRotationtoMouse)
  (Animation|Montage|PlayMontage (Variables|Default|GetPlayerMesh) (Utilities|Array|Get(acopy) (Variables|Default|GetattackAnims)) 8.0
    (:OnBlendOut
      (Animation|Montage|PlayMontage (Variables|Default|GetPlayerMesh) (Utilities|Array|Get(acopy) (Variables|Default|GetattackAnims) 1) 1.5 :!label _label
        (:OnBlendOut
          (if (not (Variables|Default|GetStopAimingBow))
            (goto _label)))))))

(event EventBeginPlay
  ;[0.05098 0.05098 0.05098] Setup
  (|CallParentFunction)
  (Variables|/Game/Player/Blueprints/BPC_PlayerCombatHandler.BPC_PlayerCombatHandler_C|SetAttackCooldown (Variables|Default|GetBPC_PlayerRangedHeavy) 5.0) ; CD
)

(fn CheckCanAttack
  (bind _canattack (|CallParentFunction))
  (if _canattack
    (if (Variables|/Game/Player/Blueprints/BPC_PlayerCombatHandler.BPC_PlayerCombatHandler_C|GetCanAttack (Variables|Default|GetBPC_PlayerRangedHeavy))
      (return true)
      (else
        _)))
  (return false))

(fn HandleFinishedAttacking
  (|CallParentFunction))

(fn CheckCanReleaseAttack
  (bind _canreleaseattack (|CallParentFunction))
  (if _canreleaseattack
    (if (Variables|/Game/Player/Blueprints/BPC_PlayerCombatHandler.BPC_PlayerCombatHandler_C|GetCanReleaseAttack (Variables|Default|GetBPC_PlayerRangedHeavy))
      (return true)
      (else
        _)))
  (return false))

(fn CalculateDamageMultiplier
  (params (Elapsed%20Seconds :type Float%20%28double-precision%29) (Interval%20Seconds :type Float%20%28double-precision%29) (Multiply%20Damage%20By :type Float%20%28double-precision%29))
  (LocalVariables|SetElapsedSeconds Elapsed%20Seconds)
  (LocalVariables|SetIntervalSeconds Interval%20Seconds)
  (LocalVariables|SetMultiplyDamageBy Multiply%20Damage%20By)
  (if (<= (LocalVariables|GetElapsedSeconds) (LocalVariables|GetIntervalSeconds))
    (return (Utilities|MultiplybyInterval 0.0))
    (elif (and (>= (* (LocalVariables|GetIntervalSeconds) 2.0) (LocalVariables|GetElapsedSeconds)) (<= (LocalVariables|GetElapsedSeconds) (* (LocalVariables|GetIntervalSeconds) 3.0)))
      (return (Utilities|MultiplybyInterval 1.0))
      (elif (and (>= (* (LocalVariables|GetIntervalSeconds) 3.0) (LocalVariables|GetElapsedSeconds)) (<= (LocalVariables|GetElapsedSeconds) (* (LocalVariables|GetIntervalSeconds) 4.0)))
        (return (Utilities|MultiplybyInterval 2.0))
        (else
          (return (Utilities|MultiplybyInterval 3.0)))))))