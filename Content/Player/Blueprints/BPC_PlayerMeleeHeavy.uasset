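; Player melee heavy attack component that locks movement, turns toward the mouse and plays a montage ending in a shockwave.
; A fast looping timer knocks back nearby enemies until the animation triggers the shockwave.
; The shockwave sphere trace deals random-range damage, knocks enemies up, shakes the camera and reduces dash cooldown per hit.
; A self-calling timer event runs the cooldown, then re-enables both melee and ranged heavy attacks.
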(event Custom|TriggerShockWave
  (bind _actorhitbytrace (Variables|Default|GetactorHitByTrace))
  (bind _bpc_playermeleeheavy (Variables|Default|GetBPC_PlayerMeleeHeavy))
  (bind _bp_playercharacter (Variables|Default|GetBP_PlayerCharacter))
  (bind _returnvalue (Transformation|GetActorLocation _bp_playercharacter))
  ;[0.05098 0.05098 0.05098] Ray traces weapon animation when melee attacking
  (CallFunction|StartHeavyAttackCD (Variables|Default|GetBPC_PlayerMeleeHeavy))
  (Utilities|Time|ClearandInvalidateTimerbyHandle (Variables|Default|GetPushTimerHandle)) ; make this stop just a bit before shockwave trigger when anims are implemented
  (bind _outhits (Collision|MultiSphereTraceByChannel _returnvalue _returnvalue 4.5e+02 "TraceTypeQuery1" true 0 "None"))
  (bind _array_element (Utilities|Array|ForEachLoopwithBreak _outhits)
    (:LoopBody
      (if (not (Utilities|Array|ContainsItem _actorhitbytrace (.HitActor (Collision|BreakHitResult _array_element))))
        (Utilities|Array|Add _actorhitbytrace (.HitActor (Collision|BreakHitResult _array_element)))
        (Class|BPIDamagable|DealDamage(Message) (.HitActor (Collision|BreakHitResult _array_element)) (Utilities|Struct|MakeS_DamageInfo (Math|Random|RandomFloatinRange (Variables|/Game/Player/Blueprints/BPC_PlayerCombatHandler.BPC_PlayerCombatHandler_C|GetMinDamage _bpc_playermeleeheavy) (Variables|/Game/Player/Blueprints/BPC_PlayerCombatHandler.BPC_PlayerCombatHandler_C|GetMaxDamage _bpc_playermeleeheavy)) "NewEnumerator0" "NewEnumerator1" "NewEnumerator3" "NewEnumerator0" 1.5))
        (Default|CallOnReduceDashCD (Variables|Default|GetBPC_PlayerDash) 8.0)
        (Class|LegacyCameraShake|StartLegacyCameraShake (Game|GetPlayerCameraManager 0) "/Game/UI/CameraShake/BP_HeavyAttackCameraShake.BP_HeavyAttackCameraShake_C" 2.0 "World" "0, 0, 0")
        (bind _filteredarray (Utilities|Array|FilterArray (Variables|Default|GetactorHitByTrace) "/Game/Enemies/Blueprints/BP_EnemyBase.BP_EnemyBase_C"))
        (for _array_element_2 _filteredarray
          (Default|Knockup _array_element_2 1.1e+03))))
    (:Completed
      (Utilities|Array|Clear (Variables|Default|GetactorHitByTrace)))))

(event Custom|MeleeHeavyPush
  (bind _bp_playercharacter (Variables|Default|GetBP_PlayerCharacter))
  ;[0.05098 0.05098 0.05098] Knockback enemies while jumping
  (bind _returnvalue (Utilities|Time|SetTimerbyEvent (delegate Custom|MeleeHeavyPush) 0.001 true))
  (Variables|Default|SetPushTimerHandle _returnvalue)
  (bind (_outactors _returnvalue_2) (Collision|SphereOverlapActors (Transformation|GetActorLocation _bp_playercharacter) 1.6e+02 (Utilities|Array|MakeArray "ObjectTypeQuery3") "/Game/Enemies/Blueprints/BP_EnemyBase.BP_EnemyBase_C" (Utilities|Array|MakeArray _bp_playercharacter)))
  (if _returnvalue_2
    (bind _filteredarray (Utilities|Array|FilterArray _outactors "/Game/Enemies/Blueprints/BP_EnemyBase.BP_EnemyBase_C"))
    (for _array_element _filteredarray
      (Default|Knockback _array_element 8e+01))))

(event Custom|StartHeavyAttackCD
  (bind _bpc_playermeleeheavy (Variables|Default|GetBPC_PlayerMeleeHeavy))
  ;[0.05098 0.05098 0.05098] AttackCooldown
  (bind _returnvalue (Utilities|Time|SetTimerbyEvent (delegate Custom|StartHeavyAttackCD) (Variables|/Game/Player/Blueprints/BPC_PlayerCombatHandler.BPC_PlayerCombatHandler_C|GetAttackCooldown (Variables|Default|GetBPC_PlayerMeleeHeavy))))
  (if (Utilities|Time|IsValidTimerHandle (stale _output_get))
    (Utilities|Time|ClearandInvalidateTimerbyHandle (Variables|/Game/Player/Blueprints/BPC_PlayerCombatHandler.BPC_PlayerCombatHandler_C|GetCooldownTimerHandle _bpc_playermeleeheavy))
    (Utilities|Time|ClearandInvalidateTimerbyHandle (Variables|Default|GetPushTimerHandle))
    (Variables|/Game/Player/Blueprints/BPC_PlayerCombatHandler.BPC_PlayerCombatHandler_C|SetCanAttack _bpc_playermeleeheavy true)
    (Variables|/Game/Player/Blueprints/BPC_PlayerCombatHandler.BPC_PlayerCombatHandler_C|SetCanAttack (Variables|Default|GetBPC_PlayerRangedHeavy) true)
    (else
      (bind _output_get (Variables|/Game/Player/Blueprints/BPC_PlayerCombatHandler.BPC_PlayerCombatHandler_C|SetCooldownTimerHandle (Variables|Default|GetBPC_PlayerMeleeHeavy) _returnvalue)))))

(event Custom|MeleeHeavyAttack
  (bind _bpc_playermeleeheavy (Variables|Default|GetBPC_PlayerMeleeHeavy))
  ;[0.05098 0.05098 0.05098] Attack
  (Default|ToggleEnableMovementInput (Variables|Default|GetBP_PlayerCharacter) false false)
  (CallFunction|RotateTowardsMousePOS)
  (CallFunction|MeleeHeavyPush)
  (Animation|Montage|PlayMontage (Variables|Default|GetPlayerMesh) (Utilities|Array|Get(acopy) (Variables|Default|GetattackAnims)) (Variables|/Game/Player/Blueprints/BPC_PlayerCombatHandler.BPC_PlayerCombatHandler_C|GetAnimationPlayRate (Variables|Default|GetBPC_PlayerMeleeHeavy))
    (:OnInterrupted
      (if (Variables|/Game/Player/Blueprints/BPC_PlayerCombatHandler.BPC_PlayerCombatHandler_C|GetCanAttack _bpc_playermeleeheavy)
        (CallFunction|StartHeavyAttackCD _bpc_playermeleeheavy)
        (CallFunction|HandleFinishedAttacking _bpc_playermeleeheavy)))))

(event EventBeginPlay
  ;[0.05098 0.05098 0.05098] Setup
  (|CallParentFunction))

(fn CheckCanAttack
  (bind _canattack (|CallParentFunction))
  (if _canattack
    (if (Variables|/Game/Player/Blueprints/BPC_PlayerCombatHandler.BPC_PlayerCombatHandler_C|GetCanAttack (Variables|Default|GetBPC_PlayerMeleeHeavy))
      (return true)
      (else
        (return false)))
    (else
      (return false))))

(fn HandleFinishedAttacking
  (|CallParentFunction)
  (Utilities|Time|ClearandInvalidateTimerbyHandle (Variables|Default|GetPushTimerHandle)) ; make this stop just a bit before shockwave trigger when anims are implemented
  (Default|CallOnUpdateHeavyCDWidget))

(fn SetUpgradeVariables)

(fn DilateTime
  (Default|TimeDilation (Variables|Default|GetBP_ThirdPersonGameMode) "/Game/UI/TimeDilation/HeavyAttackCurve.HeavyAttackCurve"))