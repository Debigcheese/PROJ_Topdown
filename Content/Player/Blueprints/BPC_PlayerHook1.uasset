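; Player attack component for a grappling hook ability, aimed at the mouse while Q is held and fired on release.
; Self-looping timers rotate the player during aim, then SpawnProjectile launches a damaging BP_ProjectileHook that expires shortly if nothing is hit.
; On HookLanded, brief time dilation plays and a timer pulls the player toward the enemy with VInterpTo, camera lag disabled.
; HookFinished restores movement and dash and notifies the combat handler.
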(event Custom|SpawnProjectile
  (bind _bp_playercharacter (Variables|Default|GetBP_PlayerCharacter))
  (bind _bpc_playerhook (Variables|Default|GetBPC_PlayerHook))
  (bind _bp_playercharacter_2 (Variables|Default|GetBP_PlayerCharacter))
  ;[0.05098 0.05098 0.05098] SpawnProjectile - starts when q is released
  (CallFunction|StopRotating)
  (bind _returnvalue (Game|SpawnActorfromClass "/Game/Projectile/Blueprints/BP_ProjectileHook.BP_ProjectileHook_C" (Transformation|GetWorldTransform (Variables|/Game/Player/Blueprints/BP_PlayerCharacter.BP_PlayerCharacter_C|GetHookShootPoint _bp_playercharacter)) "Undefined" "MultiplyWithRoot" _bp_playercharacter 3.3e+03 0.0 false (Utilities|Struct|MakeS_DamageInfo (Math|Random|RandomFloatinRange (Variables|/Game/Player/Blueprints/BPC_PlayerCombatHandler.BPC_PlayerCombatHandler_C|GetMinDamage _bpc_playerhook) (Variables|/Game/Player/Blueprints/BPC_PlayerCombatHandler.BPC_PlayerCombatHandler_C|GetMaxDamage _bpc_playerhook)) "NewEnumerator4" "NewEnumerator2" "NewEnumerator3" "NewEnumerator0" 0.75) false 0 0))
  (bind _output_get (Variables|Default|SetBP_ProjectileHook _returnvalue))
  (Collision|IgnoreActorwhenMoving (Variables|/Script/Engine.Character|GetCapsuleComponent _bp_playercharacter_2) _output_get true)
  (Collision|IgnoreActorwhenMoving (Variables|/Game/Projectile/Blueprints/BP_ProjectileBase.BP_ProjectileBase_C|GetWallHit _output_get) _bp_playercharacter_2 true)
  (Collision|IgnoreActorwhenMoving (Variables|/Game/Projectile/Blueprints/BP_ProjectileBase.BP_ProjectileBase_C|GetActorCollision _output_get) _bp_playercharacter_2 true)
  (Utilities|FlowControl|Delay 0.43)
  (bind _bp_projectilehook (Variables|Default|GetBP_ProjectileHook)
    (:then
      (if (not (Variables|/Game/Projectile/Blueprints/BP_ProjectileBase.BP_ProjectileBase_C|GetHasCollided _bp_projectilehook))
        (CallFunction|HookFinished)
        (Actor|DestroyActor _bp_projectilehook)))
    (:else)))

(event Custom|LerpActorRotationToMouse
  ;[0.05098 0.05098 0.05098] Rotate player to mouse location
  (bind _returnvalue (Utilities|Time|SetTimerbyEvent (delegate Custom|LerpActorRotationToMouse) 0.001 true))
  (bind _playerrotationz (CallFunction|FindRotationtoMousePOS (Variables|/Game/Player/Blueprints/BP_PlayerCharacter.BP_PlayerCharacter_C|GetHookShootPoint (Variables|Default|GetBP_PlayerCharacter))))
  (Transformation|SetActorRotation (Variables|Default|GetBP_PlayerCharacter) (Math|Rotator|MakeRotator 0.0 0.0 _playerrotationz)))

(event Custom|StopRotating
  ;[0.05098 0.05098 0.05098] Rotate player to mouse location
  (Utilities|Time|ClearandInvalidateTimerbyHandle (stale Custom|LerpActorRotationToMouse _returnvalue)))

(event Custom|HookHit
  ;[0.05098 0.05098 0.05098] HookHit - starts when hook hit an enemy
  (bind _returnvalue (Utilities|Time|SetTimerbyEvent (delegate Custom|HookHit) 0.01 true))
  (Variables|HookHit|SetHookHitTimerHandle _returnvalue)
  (bind (_vinterpto _distance) (Utilities|LerpLocationtoEnemy))
  (if (<= _distance 2e+02)
    (Utilities|Time|ClearandInvalidateTimerbyHandle (Variables|HookHit|GetHookHitTimerHandle))
    (Variables|HookHit|SetHookHitTimer 0.0)
    (Variables|/Script/Engine.SpringArmComponent|SetbEnableCameraLag (Variables|/Game/Player/Blueprints/BP_PlayerCharacter.BP_PlayerCharacter_C|GetSpringArm (Variables|Default|GetBP_PlayerCharacter)) true)
    (CallFunction|HookFinished)
    (Utilities|FlowControl|Delay 0.1)
    (bind _bp_projectilehook (Variables|Default|GetBP_ProjectileHook)
      (:then
        (Actor|DestroyActor _bp_projectilehook))
      (:else))
    (else
      (Transformation|SetActorLocation (Variables|Default|GetBP_PlayerCharacter) _vinterpto false false))))

(event Custom|HookFinished
  ;[0.05098 0.05098 0.05098] HookFinished - starts when hook hit nothing or when enemy got hit and player is close to enemy
  (Default|ToggleEnableMovementInput (Variables|Default|GetBP_PlayerCharacter) true true)
  (Default|FinishedAttacking (Variables|Default|GetBPC_PlayerCombatHandler))
  (Utilities|Time|ClearandInvalidateTimerbyHandle (Variables|HookHit|GetHookHitTimerHandle)))

(event Custom|HookAttack
  ;[0.05098 0.05098 0.05098] Attack - played when q is pressed
  (Default|ToggleEnableMovementInput (Variables|Default|GetBP_PlayerCharacter) false false)
  (CallFunction|LerpActorRotationtoMouse)
  (Animation|Montage|PlayMontage (Variables|Default|GetPlayerMesh) "/Game/Characters/Mannequins/Animations/Bow_Animations/StandingEquipBow_UE_Montage.StandingEquipBow_UE_Montage" (Variables|/Game/Player/Blueprints/BPC_PlayerCombatHandler.BPC_PlayerCombatHandler_C|GetAnimationPlayRate (Variables|Default|GetBPC_PlayerHook))))

(event Custom|HookLanded
  (params (EnemyHit :type Actor%20Object%20Reference))
  ;[0.05098 0.05098 0.05098] HookLanded - starts when BP_ProjectileHook collides with something
  (bind _output_get (Variables|Default|SetTargetEnemy EnemyHit))
  (Variables|/Script/Engine.SpringArmComponent|SetbEnableCameraLag (Variables|/Game/Player/Blueprints/BP_PlayerCharacter.BP_PlayerCharacter_C|GetSpringArm (Variables|Default|GetBP_PlayerCharacter)) false)
  (Transformation|SetActorRotation (Variables|Default|GetBP_PlayerCharacter) (Math|Rotator|MakeRotator 0.0 0.0 (.yaw (Math|Rotator|FindLookatRotation (Transformation|GetActorLocation (Variables|Default|GetBP_PlayerCharacter)) (Transformation|GetActorLocation _output_get)))))
  (CallFunction|HookHit)
  (CallFunction|StopRotating)
  (Default|TimeDilation (Variables|/Game/Player/Blueprints/BP_PlayerCharacter.BP_PlayerCharacter_C|GetBPC_DamageSystem (Variables|Default|GetBP_PlayerCharacter)) 0.02 0.37 0.0))

(event EventBeginPlay
  ;[0.05098 0.05098 0.05098] Setup
  (|CallParentFunction)
  (Variables|/Game/Player/Blueprints/BPC_PlayerCombatHandler.BPC_PlayerCombatHandler_C|SetAttackCooldown (Variables|Default|GetBPC_PlayerHook) 2.0) ; CD
)

(fn ApplyForceTimerFunction
  (params (TimerHandle :type Timer%20Handle%20Structure))
  (Variables|HookHit|SetHookHitTimerHandle TimerHandle)
  (bind _output_get (Variables|HookHit|SetHookHitTimer (+ 0.01 (Variables|HookHit|GetHookHitTimer))))
  (if (>= 0.0 _output_get)
    (return)
    (else
      (Utilities|Time|ClearandInvalidateTimerbyHandle (Variables|HookHit|GetHookHitTimerHandle))
      (Variables|HookHit|SetHookHitTimer 0.0))))

(fn CheckCanAttack
  (bind _canattack (|CallParentFunction))
  (if _canattack
    (if (Variables|/Game/Player/Blueprints/BPC_PlayerCombatHandler.BPC_PlayerCombatHandler_C|GetCanAttack (Variables|Default|GetBPC_PlayerHook))
      (return true)
      (else
        _)))
  (return false))

(fn CheckCanReleaseAttack
  (bind _canreleaseattack (|CallParentFunction))
  (if _canreleaseattack
    (if (Variables|/Game/Player/Blueprints/BPC_PlayerCombatHandler.BPC_PlayerCombatHandler_C|GetCanReleaseAttack (Variables|Default|GetBPC_PlayerHook))
      (return true)
      (else
        _)))
  (return false))

(fn HandleFinishedAttacking
  (|CallParentFunction)
  (CallFunction|StopRotating)
  (Default|ToggleEnableMovementInput (Variables|Default|GetBP_PlayerCharacter) true true))