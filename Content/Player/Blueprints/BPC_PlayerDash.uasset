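; Player dash component that launches the character in a camera-relative input direction, gated by state and cooldown, cancelling bow attacks.
; Self-re-arming timers drive the repeated launches and the cooldown, which sword hits during a dash shorten.
; The capsule ignores pawns while dashing, and overlap tests lengthen the dash until its predicted end clears enemies.
; Afterwards it restores collision and friction, turning toward the nearest enemy if the sword is attacking.
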(event Custom|ApplyDashForce
  (bind _dashforce (Variables|Force|GetDashForce))
  ;[0.05098 0.05098 0.05098] ApplyDashForce
  (bind _returnvalue (Utilities|Time|SetTimerbyEvent (delegate Custom|ApplyDashForce) 0.001 true))
  (Variables|Force|SetDashForceTimerHandle _returnvalue)
  (bind _output_get (Variables|Force|SetDashTimer (+ (Variables|Force|GetDashTimer) 0.1)))
  (if (>= _output_get (Variables|Default|GetDashDurationTemp))
    (Utilities|Time|ClearandInvalidateTimerbyHandle (Variables|Force|GetDashForceTimerHandle))
    (Utilities|FlowControl|Delay 0.1)
    (Utilities|ResetVariables)
    (Collision|SetCollisionResponsetoChannel (Variables|Default|GetCapsule%20Component) "ECC_Pawn" "ECR_Block")
    (if (Variables|/Game/Player/Blueprints/BPC_PlayerCombatHandler.BPC_PlayerCombatHandler_C|GetIsAttacking (Variables|Default|GetBPC%20Player%20Sword))
      (CallFunction|RotatetoClosestEnemy))
    (else
      (Character|LaunchCharacter (Variables|Components|GetBP%20Player%20Character) (Math|Vector|MakeVector (.x _dashforce) (.y _dashforce) 0.0) false false))))

(event Custom|ReduceDashCD
  (params (ReduceByPercentage :type Float%20%28double-precision%29))
  ;[0.05098 0.05098 0.05098] ReduceDashCD when player hits an enemy (with melee sword attack)
  (if (Variables|Bools|GetIs%20Dashing)
    (Variables|Cooldown|SetDash%20CDTimer (+ (Variables|Cooldown|GetDash%20CDTimer) (* (/ ReduceByPercentage 1e+02) (Variables|Cooldown|GetDash%20CDDuration))))))

(event Custom|StartDashCD
  ;[0.05098 0.05098 0.05098] StartDashCooldown
  (Variables|/Game/DamageSystem/BPC_DamageSystem.BPC_DamageSystem_C|SetisInvincible (Variables|/Game/Player/Blueprints/BP_PlayerCharacter.BP_PlayerCharacter_C|GetBPC_DamageSystem (Variables|Components|GetBP%20Player%20Character)) false)
  (bind _returnvalue (Utilities|Time|SetTimerbyEvent (delegate Custom|StartDashCD) 0.1 true))
  (Variables|Cooldown|SetDashCDTimerHandle _returnvalue)
  (bind _output_get (Variables|Cooldown|SetDash%20CDTimer (+ (Variables|Cooldown|GetDash%20CDTimer) 0.1)))
  (if (>= _output_get (Variables|Cooldown|GetDash%20CDDuration))
    (Utilities|Time|ClearandInvalidateTimerbyHandle (Variables|Cooldown|GetDashCDTimerHandle))
    (Variables|Cooldown|SetDash%20CDTimer 0.0)
    (Variables|Bools|SetDashOnCooldown false)))

(event Input|EnhancedActionEvents|EnhancedInputActionIA_Dash
  (params (ActionValue :type Boolean) (ElapsedSeconds :type Float%20%28double-precision%29) (TriggeredSeconds :type Float%20%28double-precision%29) (InputAction :type Input%20Action%20Object%20Reference :default "/Game/Player/Input/Actions/IA_Dash.IA_Dash"))
  ;[0.05098 0.05098 0.05098] Dash
  (:Started
    (Utilities|CanDashHandler)
    (if (Variables|/Game/Player/Blueprints/BPC_PlayerCombatHandler.BPC_PlayerCombatHandler_C|GetIsAttacking (Variables|Default|GetBPC%20Player%20Bow))
      (CallFunction|CancelAttack))
    (Variables|Bools|SetIs%20Dashing true)
    (Variables|Bools|SetDashOnCooldown true)
    (Audio|PlaySound2D "/Game/Audio/Player/dash2.dash2" 1.0 1.0 0.0 0 0)
    (Variables|/Script/Engine.CharacterMovementComponent|SetBrakingFrictionFactor (Variables|Default|GetCharacter%20Movement) 1.0)
    (Default|CallOnDashCancelOtherForces)
    (Variables|/Script/Engine.MovementComponent|SetVelocity (Variables|Default|GetCharacter%20Movement) "0, 0, 0")
    (Collision|SetCollisionResponsetoChannel (Variables|Default|GetCapsule%20Component) "ECC_Pawn" "ECR_Ignore")
    (CallFunction|CalculateDashForce)
    (CallFunction|HandleDashEnemyCollision)
    (CallFunction|ApplyDashForce)
    (CallFunction|StartDashCD)
    (Default|OnDashChangeMaterial (Variables|/Game/Player/Blueprints/BP_PlayerCharacter.BP_PlayerCharacter_C|GetBPC_DamageSystem (Variables|Components|GetBP%20Player%20Character)))
    (Default|CallOnDash)))

(event EventBeginPlay
  ;[0.05098 0.05098 0.05098] Setup
  (Utilities|GetComponents)
  (EventDispatchers|BindEventtoOnReduceDashCD (EventDispatchers|CreateEvent :!event Custom|ReduceDashCD))
  (Variables|Default|SetDashDurationTemp (Variables|Default|GetDashDuration)))

(fn HandleDashEnemyCollision
  (bind _dashforce (Variables|Force|GetDashForce))
  (bind _bp_player_character (Variables|Components|GetBP%20Player%20Character))
  (bind _capsule_component (Variables|Default|GetCapsule%20Component))
  (bind _returnvalue (Transformation|GetActorLocation _bp_player_character))
  (bind _returnvalue_2 (Transformation|GetWorldTransform _capsule_component))
  (while (Variables|Bools|GetDashCollidedWithEnemy)
    ;[0.05098 0.05098 0.05098] Calculates endposition of dash
    (LocalVariables|SetEndPosition (Math|Vector|MakeVector (+ (.x _returnvalue) (* (.x _dashforce) (Variables|Default|GetDashDurationTemp))) (+ (* (.y _dashforce) (Variables|Default|GetDashDurationTemp)) (.y _returnvalue)) 0.0))
    ;[0.05098 0.05098 0.05098] increase dashduration if endposition of dash is inside an enemy
    (Variables|Default|SetDashDurationTemp (+ (Variables|Default|GetDashDurationTemp) (/ (Variables|Default|GetDashDuration) 2e+01)))
    (bind _returnvalue_3 (Collision|ComponentOverlapActors _capsule_component (Math|Transform|MakeTransform (LocalVariables|GetEndPosition) (.rotation _returnvalue_2) (* (.scale _returnvalue_2) "20.000000,20.000000,20.000000")) (Utilities|Array|MakeArray "ObjectTypeQuery3") "/Game/Enemies/Blueprints/BP_EnemyBase.BP_EnemyBase_C" (Utilities|Array|MakeArray (Variables|Components|GetBP%20Player%20Character))))
    (Variables|Bools|SetDashCollidedWithEnemy _returnvalue_3))
  (return))

(fn CalculateDashForce
  (bind _spring_arm (Variables|Default|GetSpring%20Arm))
  (bind _bp_player_character (Variables|Components|GetBP%20Player%20Character))
  (bind _dashstrength (Variables|Default|GetDashStrength))
  (bind _returnvalue (Class|SpringArmComponent|GetTargetRotation _spring_arm))
  (bind _ia_moveactionvalues (Variables|/Game/Player/Blueprints/BP_PlayerCharacter.BP_PlayerCharacter_C|GetIA_MoveActionValues _bp_player_character))
  (bind _returnvalue_2 (Math|Rotator|MakeRotator 0.0 0.0 (.yaw _returnvalue)))
  (bind _returnvalue_3 (Math|Float|Clamp(Float) (.y _ia_moveactionvalues) -1.0))
  (bind _returnvalue_4 (Math|Float|Clamp(Float) (.x _ia_moveactionvalues) -1.0))
  (bind _returnvalue_5 (Math|Vector|GetForwardVector _returnvalue_2))
  (bind _returnvalue_6 (Math|Vector|GetRightVector _returnvalue_2))
  (bind _returnvalue_7 (* _returnvalue_5 _dashstrength _returnvalue_3))
  (bind _returnvalue_8 (* _returnvalue_6 _dashstrength _returnvalue_4))
  (bind _returnvalue_9 (+ _returnvalue_8 _returnvalue_7))
  (Variables|Force|SetDashForce (Math|Vector|SelectVector (/ _returnvalue_9 1.64) _returnvalue_9 (and (!= _returnvalue_4 0.0) (!= _returnvalue_3 0.0))))
  (return))

(fn CancelAttack
  (bind _bp_player_character (Variables|Components|GetBP%20Player%20Character))
  (Default|FinishedAttacking (Variables|Default|GetBPC%20Player%20Combat%20Handler))
  (Default|ToggleEnableMovementInput _bp_player_character true true)
  (Animation|StopAnimMontage _bp_player_character 0))

(fn ToggleEnableMovementInput
  (params (EnableMovementInput :type Boolean) (EnableDash :type Boolean)))

(fn RotatetoClosestEnemy
  (bind _bp_player_character (Variables|Components|GetBP%20Player%20Character))
  (bind _bp_player_character_2 (Variables|Components|GetBP%20Player%20Character))
  (bind _returnvalue (Transformation|GetActorLocation _bp_player_character_2))
  (bind _returnvalue_2 (Transformation|GetActorLocation _bp_player_character))
  (bind _outactors (Collision|SphereOverlapActors _returnvalue 4e+02 (Utilities|Array|MakeArray "ObjectTypeQuery3") "/Game/Enemies/Blueprints/BP_EnemyBase.BP_EnemyBase_C" (Utilities|Array|MakeArray (Variables|Components|GetBP%20Player%20Character))))
  (Rendering|Debug|DrawDebugSphere _returnvalue 0.0 12 "(R=1.000000,G=1.000000,B=1.000000,A=1.000000)" 1.0 1.0)
  (if (Utilities|Array|IsNotEmpty _outactors)
    (for _array_element _outactors
      (if (< (Math|Vector|Distance(Vector) (Transformation|GetActorLocation _array_element) _returnvalue_2) (LocalVariables|GetClosestDistance))
        (LocalVariables|SetClosestDistance (Math|Vector|Distance(Vector) (Transformation|GetActorLocation _array_element) _returnvalue_2))
        (LocalVariables|SetClosestEnemy _array_element)))
    (Transformation|SetActorRotation _bp_player_character (Math|Rotator|FindLookatRotation _returnvalue_2 (Transformation|GetActorLocation (LocalVariables|GetClosestEnemy))))
    (return)
    (else
      (return))))