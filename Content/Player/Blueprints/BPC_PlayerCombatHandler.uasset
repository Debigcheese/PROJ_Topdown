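; Player combat component that routes melee, ranged and hook input to separate attack components and swaps sword or bow visibility by attack type.
; Hold time selects basic or heavy attacks, with macros gating each through shared attacking flags and handling press-release for heavy ranged and hook.
; FinishedAttacking notifies the active component, then runs cooldowns for heavy attacks and hook.
; Also provides aiming helpers for rotating toward the cursor or nearest enemy in that direction.
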(event Custom|FinishedAttacking
  (bind _bpc_playerrangedheavy (Variables|Default|GetBPC_PlayerRangedHeavy))
  (bind _bpc_playermeleeheavy (Variables|Default|GetBPC_PlayerMeleeHeavy))
  (bind _bpc_playerhook (Variables|Default|GetBPC_PlayerHook))
  ;[0.05098 0.05098 0.05098] Finished attacking
  (switch Utilities|FlowControl|Switch|SwitchonE_AttackType (Variables|BPC_PlayerCombatHandler_C|GetAttackType (Variables|Default|GetBPC_PlayerCombatHandler))
    (:NewEnumerator1
      (CallFunction|HandleFinishedAttacking (Variables|Default|GetBPC_PlayerMeleeBasic)))
    (:NewEnumerator5
      (CallFunction|HandleFinishedAttacking (Variables|Default|GetBPC_PlayerMeleeHeavy))
      ;[0.05098 0.05098 0.05098] Cooldowns (Can not attack with this ability until cooldown is finished)
      (Utilities|FlowControl|Delay (Variables|BPC_PlayerCombatHandler_C|GetAttackCooldown _bpc_playermeleeheavy))
      (Variables|BPC_PlayerCombatHandler_C|SetCanAttack _bpc_playermeleeheavy true))
    (:NewEnumerator2
      (CallFunction|HandleFinishedAttacking (Variables|Default|GetBPC_PlayerRangedBasic)))
    (:NewEnumerator6
      (CallFunction|HandleFinishedAttacking (Variables|Default|GetBPC_PlayerRangedHeavy))
      (Utilities|FlowControl|Delay (Variables|BPC_PlayerCombatHandler_C|GetAttackCooldown _bpc_playerrangedheavy))
      (Variables|BPC_PlayerCombatHandler_C|SetCanAttack _bpc_playerrangedheavy true))
    (:NewEnumerator3
      (CallFunction|HandleFinishedAttacking (Variables|Default|GetBPC_PlayerHook))
      (Utilities|FlowControl|Delay (Variables|BPC_PlayerCombatHandler_C|GetAttackCooldown _bpc_playerhook))
      (Variables|BPC_PlayerCombatHandler_C|SetCanAttack _bpc_playerhook true))))

(event Input|EnhancedActionEvents|EnhancedInputActionIA_MeleeAttack
  (params (ActionValue :type Boolean) (ElapsedSeconds :type Float%20%28double-precision%29) (TriggeredSeconds :type Float%20%28double-precision%29) (InputAction :type Input%20Action%20Object%20Reference :default "/Game/Player/Input/Actions/IA_MeleeAttack.IA_MeleeAttack"))
  (bind _bpc_playercombathandler (Variables|Default|GetBPC_PlayerCombatHandler))
  ;[0.05098 0.05098 0.05098] Check if attack is allowed & sets "attack style" depending on input
  (:Started
    (if (not (Variables|BPC_PlayerCombatHandler_C|GetCanAttack (Variables|Default|GetBPC_PlayerMeleeHeavy)))
      (Utilities|CanAttackHandler (Variables|Default|GetBPC_PlayerMeleeBasic) :!label _label
        (:AttackAllowed
          (Variables|BPC_PlayerCombatHandler_C|SetAttackType (Variables|Default|GetBPC_PlayerCombatHandler) "NewEnumerator1")
          (Default|MeleeBasicAttack (Variables|Default|GetBPC_PlayerMeleeBasic))
          (CallFunction|ChangeWeaponType _bpc_playercombathandler :!label _label_2)
          (Variables|BPC_PlayerCombatHandler_C|SetIsAttacking _bpc_playercombathandler true)))))
  (:Ongoing
    (if (not (>= (Variables|HoldingTime|GetMinimumHoldingTime) ElapsedSeconds))
      (Utilities|CanAttackHandler (Variables|Default|GetBPC_PlayerMeleeHeavy)
        (:AttackAllowed
          (Variables|BPC_PlayerCombatHandler_C|SetAttackType (Variables|Default|GetBPC_PlayerCombatHandler) "NewEnumerator5")
          (Default|MeleeHeavyAttack (Variables|Default|GetBPC_PlayerMeleeHeavy))
          (goto _label_2)))))
  (:Completed
    (goto _label)))

(event Input|EnhancedActionEvents|EnhancedInputActionIA_RangedAttack
  (params (ActionValue :type Boolean) (ElapsedSeconds :type Float%20%28double-precision%29) (TriggeredSeconds :type Float%20%28double-precision%29) (InputAction :type Input%20Action%20Object%20Reference :default "/Game/Player/Input/Actions/IA_RangedAttack.IA_RangedAttack"))
  (bind _bpc_playercombathandler (Variables|Default|GetBPC_PlayerCombatHandler))
  ;[0.05098 0.05098 0.05098] Check if attack is allowed & sets "attack style" depending on input
  (:Started
    (if (not (Variables|BPC_PlayerCombatHandler_C|GetCanAttack (Variables|Default|GetBPC_PlayerRangedHeavy)))
      (Utilities|CanAttackHandler (Variables|Default|GetBPC_PlayerRangedBasic) :!label _label
        (:AttackAllowed
          (Variables|BPC_PlayerCombatHandler_C|SetAttackType (Variables|Default|GetBPC_PlayerCombatHandler) "NewEnumerator2")
          (Default|RangedBasicAttack (Variables|Default|GetBPC_PlayerRangedBasic))
          (CallFunction|ChangeWeaponType _bpc_playercombathandler :!label _label_2)
          (Variables|BPC_PlayerCombatHandler_C|SetIsAttacking _bpc_playercombathandler true)))))
  (:Ongoing
    (Variables|Default|SetElapsed%20Seconds ElapsedSeconds)
    (if (not (>= (Variables|HoldingTime|GetMinimumHoldingTime) (Variables|Default|GetElapsed%20Seconds)))
      (Utilities|CanReleaseAttackHandler (Variables|Default|GetBPC_PlayerRangedHeavy) :!label _label_3
        (:OnPress
          (Variables|BPC_PlayerCombatHandler_C|SetAttackType (Variables|Default|GetBPC_PlayerCombatHandler) "NewEnumerator6")
          (Default|RangedHeavyAttack (Variables|Default|GetBPC_PlayerRangedHeavy))
          (goto _label_2))
        (:OnRelease
          (Default|HandleAimingTime (Variables|Default|GetBPC_PlayerRangedHeavy) (- (Variables|Default|GetElapsed%20Seconds) (Variables|HoldingTime|GetMinimumHoldingTime)))))))
  (:Canceled
    (if (>= (Variables|HoldingTime|GetMinimumHoldingTime) (Variables|Default|GetElapsed%20Seconds)) :!label _label_4
      (goto _label)
      (else
        (goto _label_3 Released))))
  (:Completed
    (goto _label_4)))

(event Input|EnhancedActionEvents|EnhancedInputActionIA_HookAttack
  (params (ActionValue :type Boolean) (ElapsedSeconds :type Float%20%28double-precision%29) (TriggeredSeconds :type Float%20%28double-precision%29) (InputAction :type Input%20Action%20Object%20Reference :default "/Game/Player/Input/Actions/IA_HookAttack.IA_HookAttack"))
  (bind _bpc_playercombathandler (Variables|Default|GetBPC_PlayerCombatHandler))
  ;[0.05098 0.05098 0.05098] Check if attack is allowed & sets "attack style" depending on input
  (:Started
    (Utilities|CanReleaseAttackHandler (Variables|Default|GetBPC_PlayerHook) :!label _label
      (:OnPress
        (Variables|BPC_PlayerCombatHandler_C|SetAttackType (Variables|Default|GetBPC_PlayerCombatHandler) "NewEnumerator3")
        (Default|HookAttack (Variables|Default|GetBPC_PlayerHook))
        (CallFunction|ChangeWeaponType _bpc_playercombathandler)
        (Variables|BPC_PlayerCombatHandler_C|SetIsAttacking _bpc_playercombathandler true))
      (:OnRelease
        (Default|SpawnProjectile (Variables|Default|GetBPC_PlayerHook)))))
  (:Canceled
    (goto _label Released))
  (:Completed
    (goto _label Released)))

(event EventBeginPlay
  ;[0.05098 0.05098 0.05098] Setup
  (Utilities|GetActorComponents)
  (Utilities|GetMeshes)
  (Variables|BPC_PlayerCombatHandler_C|SetPreviousWeapon (Variables|Default|GetBPC_PlayerCombatHandler) (.Value (Utilities|Map|Find (Variables|WeaponType|GetWeaponMeshes) "NewEnumerator2")))
  (CallFunction|ChangeWeaponType))

(fn FindRotationtoMousePOS
  (params (ShootPoint :type Scene%20Component%20Object%20Reference))
  (bind _returnvalue (Game|GetPlayerController 0))
  (bind (_worldlocation _worlddirection) (Game|Player|ConvertMouseLocationToWorldSpace _returnvalue))
  (return (.yaw (Math|Rotator|FindLookatRotation (Transformation|GetActorLocation (Variables|Components|GetBP_PlayerCharacter)) (.Intersection (Class|KismetMathLibrary|LinePlaneIntersectionOriginNormal _worldlocation (+ _worldlocation (* _worlddirection 1e+04)) (Transformation|GetWorldLocation ShootPoint) "0.000000,0.000000,1.000000"))))))

(fn FindRotationtoSelectedEnemyPOS
  (bind _targettedenemy (CallFunction|GetTargettedEnemy))
  (return (.yaw (Math|Rotator|FindLookatRotation (Transformation|GetActorLocation (Variables|Components|GetBP_PlayerCharacter)) (Transformation|GetActorLocation _targettedenemy)))))

(fn RotateTowardsMousePOS
  (bind _playerrotationz (CallFunction|FindRotationtoMousePOS (Variables|/Game/Player/Blueprints/BP_PlayerCharacter.BP_PlayerCharacter_C|GetHookShootPoint (Variables|Components|GetBP_PlayerCharacter))))
  (Transformation|SetActorRotation (Variables|Components|GetBP_PlayerCharacter) (Math|Rotator|MakeRotator 0.0 0.0 _playerrotationz)))

(fn FindRotationtoClosestEnemy
  (bind _returnvalue (Game|GetPlayerController 0))
  (bind _hitresult (Game|Player|GetHitResultUnderCursorbyChannel _returnvalue "TraceTypeQuery1" true))
  (bind (_targettedenemy _enemylocation) (Melee|GetClosestEnemy))
  (return (.z (Math|Vector|SelectVector (+ (.yaw (Math|Rotator|FindLookatRotation (Transformation|GetActorLocation (Variables|Components|GetBP_PlayerCharacter)) (Math|Vector|SelectVector _enemylocation (.location _hitresult) (Utilities|IsValid _targettedenemy)))) 1.8e+02) (Math|Conversions|ToVector(Float) (.yaw (Math|Rotator|FindLookatRotation (Transformation|GetActorLocation (Variables|Components|GetBP_PlayerCharacter)) (Math|Vector|SelectVector _enemylocation (.location _hitresult) (Utilities|IsValid _targettedenemy))))) (== (.hitactor _hitresult) (Variables|Components|GetBP_PlayerCharacter))))))

(fn RotatetoClosestEnemy
  (bind _playerrotationz (Melee|FindRotationtoClosestEnemy))
  (Transformation|SetActorRotation (Variables|Components|GetBP_PlayerCharacter) (Math|Rotator|MakeRotator 0.0 0.0 _playerrotationz)))

(fn GetTargettedEnemy
  (bind _targetenemy (Variables|TargetEnemy|GetTargetEnemy))
  (Utilities|IsValid _targetenemy
    (:Is%20Valid
      (return _targetenemy))
    (:Is%20Not%20Valid
      (return 0))))

(fn SetTargettedEnemy
  (params (TargettedEnemy :type Actor%20Object%20Reference))
  (Utilities|IsValid TargettedEnemy
    (:Is%20Valid
      (Variables|TargetEnemy|SetTargetEnemy TargettedEnemy))
    (:Is%20Not%20Valid
      (Variables|TargetEnemy|SetTargetEnemy 0))))

(fn GetClosestEnemy
  (bind _playerrotationz (CallFunction|FindRotationtoMousePOS))
  (bind _output_get (LocalVariables|SetFrontPoint (+ (Transformation|GetActorLocation (Variables|Components|GetBP_PlayerCharacter)) (* (Math|Vector|GetForwardVector (Math|Rotator|MakeRotator 0.0 0.0 _playerrotationz)) 1.4e+02))))
  (bind _outactors (Collision|SphereOverlapActors _output_get 9e+01 (Utilities|Array|MakeArray "ObjectTypeQuery3") "/Game/Enemies/Blueprints/BP_EnemyBase.BP_EnemyBase_C" (Utilities|Array|MakeArray (Variables|Components|GetBP_PlayerCharacter))))
  (Rendering|Debug|DrawDebugSphere (LocalVariables|GetFrontPoint) 0.0 12 "(R=1.000000,G=1.000000,B=1.000000,A=1.000000)" 1.0 1.0)
  (if (Utilities|Array|IsNotEmpty _outactors)
    (for _array_element _outactors
      (if (< (Math|Vector|Distance(Vector) (Transformation|GetActorLocation _array_element) (LocalVariables|GetFrontPoint)) (LocalVariables|GetClosestDistance))
        (LocalVariables|SetClosestDistance (Math|Vector|Distance(Vector) (Transformation|GetActorLocation _array_element) (LocalVariables|GetFrontPoint)))
        (LocalVariables|SetClosestEnemy _array_element)))
    (return (LocalVariables|GetClosestEnemy) (Transformation|GetActorLocation (LocalVariables|GetClosestEnemy)))
    (else
      (return 0 "0, 0, 0"))))

(fn CheckCanAttack
  (if (Variables|BPC_PlayerCombatHandler_C|GetIsAttacking (Variables|Default|GetBPC_PlayerCombatHandler))
    (return false)
    (else
      (return true))))

(fn CheckCanReleaseAttack
  (if (Variables|BPC_PlayerCombatHandler_C|GetCanReleaseAttack (Variables|Default|GetBPC_PlayerCombatHandler))
    (return true)
    (else
      (return false))))

(fn ChangeWeaponType
  (bind _attacktype (Variables|WeaponType|GetAttackType))
  (bind _weaponmeshes (Variables|WeaponType|GetWeaponMeshes))
  (bind _bpc_playercombathandler (Variables|Default|GetBPC_PlayerCombatHandler))
  (bind _value (Utilities|Map|Find _weaponmeshes _attacktype))
  (if (Utilities|Map|Contains _weaponmeshes _attacktype)
    (Rendering|SetVisibility _value true false)
    (if (!= (Variables|BPC_PlayerCombatHandler_C|GetPreviousWeapon _bpc_playercombathandler) _value)
      (Rendering|SetVisibility (Variables|BPC_PlayerCombatHandler_C|GetPreviousWeapon _bpc_playercombathandler) false false)
      (Variables|BPC_PlayerCombatHandler_C|SetPreviousWeapon _bpc_playercombathandler _value))
    (return)))

(fn HandleFinishedAttacking
  (Utilities|ToggleChildrenIsAttacking false)
  (Variables|BPC_PlayerCombatHandler_C|SetCanReleaseAttack (Variables|Default|GetBPC_PlayerCombatHandler) false)
  (Variables|AttackChecks|SetCanReleaseAttack false)
  (Variables|WeaponType|SetAttackType "NewEnumerator1")
  (CallFunction|ChangeWeaponType))