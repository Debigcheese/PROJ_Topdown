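; Player combat component for the hook attack, which fires a hook projectile and pulls the player to the enemy it hits.
; Pressing Q turns the player toward the mouse; release spawns BP_ProjectileHook, destroyed shortly after if it hooks nothing.
; A hit moves the player toward the enemy with camera lag off, then plays a follow-up attack montage up close.
; Self-repeating timers drive rotation, pull and cooldown.
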(event Custom|SpawnProjectile
  (bind _bpc_playerhook (Variables|Default|GetBPC_PlayerHook))
  (bind _bp_playercharacter (Variables|Default|GetBP_PlayerCharacter))
  (bind _bp_playercharacter_2 (Variables|Default|GetBP_PlayerCharacter))
  ;[0.05098 0.05098 0.05098] SpawnProjectile - starts when q is released
  (CallFunction|StopRotating)
  (bind _returnvalue (Game|SpawnActorfromClass "/Game/Projectile/Blueprints/BP_ProjectileHook.BP_ProjectileHook_C" (Math|Transform|MakeTransform (Transformation|GetWorldLocation (Variables|/Script/Engine.Actor|GetRootComponent _bp_playercharacter)) (Transformation|GetWorldRotation (Variables|/Script/Engine.Actor|GetRootComponent _bp_playercharacter))) "Undefined" "MultiplyWithRoot" _bp_playercharacter 3.3e+03 0.0 false (Utilities|Struct|MakeS_DamageInfo (Math|Random|RandomFloatinRange (Variables|/Game/Player/Blueprints/BPC_PlayerCombatHandler.BPC_PlayerCombatHandler_C|GetMinDamage _bpc_playerhook) (Variables|/Game/Player/Blueprints/BPC_PlayerCombatHandler.BPC_PlayerCombatHandler_C|GetMaxDamage _bpc_playerhook)) "NewEnumerator4" "NewEnumerator2" "NewEnumerator3" "NewEnumerator0" 0.75) false 0 0))
  (bind _output_get (Variables|Default|SetBP_ProjectileHook _returnvalue))
  (Collision|IgnoreActorwhenMoving (Variables|/Script/Engine.Character|GetCapsuleComponent _bp_playercharacter_2) _output_get true)
  (Collision|IgnoreActorwhenMoving (Variables|/Game/Projectile/Blueprints/BP_ProjectileBase.BP_ProjectileBase_C|GetWallHit _output_get) _bp_playercharacter_2 true)
  (Utilities|FlowControl|Delay 0.43)
  (bind _bp_projectilehook (Variables|Default|GetBP_ProjectileHook)
    (:then
      (if (not (Variables|/Game/Projectile/Blueprints/BP_ProjectileHook.BP_ProjectileHook_C|GetEnemyHooked _bp_projectilehook))
        (CallFunction|HookFinished)
        (Actor|DestroyActor _bp_projectilehook)))
    (:else)))

(event Custom|HookSpecialAttack
  (Default|ToggleEnableMovementInput (Variables|Default|GetBP_PlayerCharacter) true false)
  (Animation|Montage|PlayMontage (Variables|Default|GetPlayerMesh) (Utilities|Array|Get(acopy) (Variables|Default|GetAttackAnims)) 3.4
    (:OnBlendOut
      (CallFunction|HookFinished (Variables|Default|GetBPC_PlayerHook)))))

(event Custom|LerpActorRotationToMouse
  ;[0.05098 0.05098 0.05098] Rotate player to mouse location
  (bind _returnvalue (Utilities|Time|SetTimerbyEvent (delegate Custom|LerpActorRotationToMouse) 0.001 true))
  (bind _playerrotationz (CallFunction|FindRotationtoMousePOS (Variables|/Game/Player/Blueprints/BP_PlayerCharacter.BP_PlayerCharacter_C|GetHookShootPoint (Variables|Default|GetBP_PlayerCharacter))))
  (Transformation|SetActorRotation (Variables|Default|GetBP_PlayerCharacter) (Math|Rotator|MakeRotator 0.0 0.0 _playerrotationz)))

(event Custom|StopRotating
  ;[0.05098 0.05098 0.05098] Rotate player to mouse location
  (Utilities|Time|ClearandInvalidateTimerbyHandle (stale Custom|LerpActorRotationToMouse _returnvalue)))

(event Custom|HookHit
  ;[0.05098 0.05098 0.05098] HookHit - starts when hook hit an enemy
  (bind _returnvalue (Utilities|Time|SetTimerbyEvent (delegate Custom|HookHit) 0.01 true))
  (Variables|HookHit|SetHookHitTimerHandle _returnvalue)
  (bind (_vinterpto _distance) (Utilities|LerpLocationtoEnemy))
  (if (<= _distance 3.5e+02)
    (CallFunction|HookSpecialAttack)
    (Utilities|Time|ClearandInvalidateTimerbyHandle (Variables|HookHit|GetHookHitTimerHandle))
    (Variables|HookHit|SetHookHitTimer 0.0)
    (Variables|/Script/Engine.SpringArmComponent|SetbEnableCameraLag (Variables|/Game/Player/Blueprints/BP_PlayerCharacter.BP_PlayerCharacter_C|GetSpringArm (Variables|Default|GetBP_PlayerCharacter)) true)
    (Utilities|FlowControl|Delay 0.1)
    (bind _bp_projectilehook (Variables|Default|GetBP_ProjectileHook)
      (:then
        (Actor|DestroyActor _bp_projectilehook))
      (:else))
    (else
      (Transformation|SetActorLocation (Variables|Default|GetBP_PlayerCharacter) _vinterpto false false))))

(event Custom|HookFinished
  ;[0.05098 0.05098 0.05098] HookFinished - starts when hook hit nothing or when enemy got hit and player is close to enemy
  (Default|ToggleEnableMovementInput (Variables|Default|GetBP_PlayerCharacter) true true)
  (CallFunction|StartHookAttackCD (Variables|Default|GetBPC_PlayerHook))
  (Default|FinishedAttacking (Variables|Default|GetBPC_PlayerCombatHandler))
  (Utilities|Time|ClearandInvalidateTimerbyHandle (Variables|HookHit|GetHookHitTimerHandle)))

(event Custom|StartHookAttackCD
  (bind _bpc_playerhook (Variables|Default|GetBPC_PlayerHook))
  (bind _bpc_playerhook_2 (Variables|Default|GetBPC_PlayerHook))
  ;[0.05098 0.05098 0.05098] AttackCooldown
  (bind _returnvalue (Utilities|Time|SetTimerbyEvent (delegate Custom|StartHookAttackCD) 0.01 true))
  (Variables|/Game/Player/Blueprints/BPC_PlayerCombatHandler.BPC_PlayerCombatHandler_C|SetCooldownTimerHandle _bpc_playerhook_2 _returnvalue)
  (bind _output_get (Variables|/Game/Player/Blueprints/BPC_PlayerCombatHandler.BPC_PlayerCombatHandler_C|SetCooldownTimer (Variables|Default|GetBPC_PlayerHook) (+ 0.01 (Variables|/Game/Player/Blueprints/BPC_PlayerCombatHandler.BPC_PlayerCombatHandler_C|GetCooldownTimer _bpc_playerhook_2))))
  (if (>= _output_get (Variables|/Game/Player/Blueprints/BPC_PlayerCombatHandler.BPC_PlayerCombatHandler_C|GetAttackCooldown (Variables|Default|GetBPC_PlayerHook)))
    (Variables|/Game/Player/Blueprints/BPC_PlayerCombatHandler.BPC_PlayerCombatHandler_C|SetCooldownTimer _bpc_playerhook 0.0)
    (Utilities|Time|ClearandInvalidateTimerbyHandle (Variables|/Game/Player/Blueprints/BPC_PlayerCombatHandler.BPC_PlayerCombatHandler_C|GetCooldownTimerHandle _bpc_playerhook))
    (Variables|/Game/Player/Blueprints/BPC_PlayerCombatHandler.BPC_PlayerCombatHandler_C|SetCanAttack (Variables|Default|GetBPC_PlayerHook) true)))

(event Custom|HookAttack
  ;[0.05098 0.05098 0.05098] Attack - played when q is pressed
  (Audio|PlaySound2D "/Game/Audio/hookswag.hookswag" 1.0 1.0 0.0 0 0)
  (Default|ToggleEnableMovementInput (Variables|Default|GetBP_PlayerCharacter) true false)
  (CallFunction|LerpActorRotationtoMouse)
  (Animation|Montage|PlayMontage (Variables|Default|GetPlayerMesh) "/Game/Characters/Arissa/Animations/Attacks/StandingEquipBow_UE_Montage.StandingEquipBow_UE_Montage" (Variables|/Game/Player/Blueprints/BPC_PlayerCombatHandler.BPC_PlayerCombatHandler_C|GetAnimationPlayRate (Variables|Default|GetBPC_PlayerHook))))

(event Custom|HookLanded
  (params (EnemyHit :type Actor%20Object%20Reference))
  ;[0.05098 0.05098 0.05098] HookLanded - starts when BP_ProjectileHook collides with something
  (bind _output_get (Variables|Default|SetTargetEnemy EnemyHit))
  (Variables|/Script/Engine.SpringArmComponent|SetbEnableCameraLag (Variables|/Game/Player/Blueprints/BP_PlayerCharacter.BP_PlayerCharacter_C|GetSpringArm (Variables|Default|GetBP_PlayerCharacter)) false)
  (Transformation|SetActorRotation (Variables|Default|GetBP_PlayerCharacter) (Math|Rotator|MakeRotator 0.0 0.0 (.yaw (Math|Rotator|FindLookatRotation (Transformation|GetActorLocation (Variables|Default|GetBP_PlayerCharacter)) (Transformation|GetActorLocation _output_get)))))
  (CallFunction|HookHit)
  (CallFunction|StopRotating))

(event EventBeginPlay
  ;[0.05098 0.05098 0.05098] Setup
  (|CallParentFunction)
  (Variables|/Game/Player/Blueprints/BPC_PlayerCombatHandler.BPC_PlayerCombatHandler_C|SetAttackCooldown (Variables|Default|GetBPC_PlayerHook) 2.0) ; CD
)

(fn ApplyForceTimerFunction
  (params (TimerHandle :type Timer%20Handle%20Structure))
  (Variables|HookHit|SetHookHitTimerHandle TimerHandle)
  (bind _output_get (Variables|HookHit|SetHookHitTimer (+ 0.01 (Variables|HookHit|GetHookHitTimer))))
  (if (>= 0.0 _output_get)
    (return)
    (else
      (Utilities|Time|ClearandInvalidateTimerbyHandle (Variables|HookHit|GetHookHitTimerHandle))
      (Variables|HookHit|SetHookHitTimer 0.0))))

(fn CheckCanAttack
  (bind _canattack (|CallParentFunction))
  (if _canattack
    (if (Variables|/Game/Player/Blueprints/BPC_PlayerCombatHandler.BPC_PlayerCombatHandler_C|GetCanAttack (Variables|Default|GetBPC_PlayerHook))
      (return true)
      (else
        _)))
  (return false))

(fn CheckCanReleaseAttack
  (bind _canreleaseattack (|CallParentFunction))
  (if _canreleaseattack
    (if (Variables|/Game/Player/Blueprints/BPC_PlayerCombatHandler.BPC_PlayerCombatHandler_C|GetCanReleaseAttack (Variables|Default|GetBPC_PlayerHook))
      (return true)
      (else
        _)))
  (return false))

(fn HandleFinishedAttacking
  (|CallParentFunction)
  (CallFunction|StopRotating (Variables|Default|GetBPC_PlayerHook))
  (Default|ToggleEnableMovementInput (Variables|Default|GetBP_PlayerCharacter) true true)
  (Variables|/Script/Engine.SpringArmComponent|SetbEnableCameraLag (Variables|/Game/Player/Blueprints/BP_PlayerCharacter.BP_PlayerCharacter_C|GetSpringArm (Variables|Default|GetBP_PlayerCharacter)) true))