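; Player melee component that runs a combo of basic sword attacks, plus a spin attack variant while dashing.
; Attacks face the closest enemy or the mouse, with a timer-driven LaunchCharacter lunge toward that point when far enough away.
; Animation-triggered capsule traces along the sword damage each actor once per swing and reduce dash cooldown.
; Hits on enemies at a specific combo step trigger brief time dilation.
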(event Custom|TriggerWeaponTrace
  ;[0.05098 0.05098 0.05098] Ray traces weapon animation when melee attacking
  (bind _returnvalue (Utilities|Time|SetTimerbyEvent (delegate Custom|WeaponTraceLoop) 0.01 true))
  (Variables|Default|SetswordTracingTimerHandle _returnvalue))

(event Custom|WeaponTraceLoop
  (bind _actorhitbytrace (Variables|Default|GetactorHitByTrace))
  (bind _bpc_playercombathandler (Variables|Default|GetBPC_PlayerCombatHandler))
  (bind _bpc_playermeleebasic (Variables|Default|GetBPC_PlayerMeleeBasic))
  (bind _sword (Variables|/Game/Player/Blueprints/BPC_PlayerCombatHandler.BPC_PlayerCombatHandler_C|GetSword _bpc_playercombathandler))
  ;[0.05098 0.05098 0.05098] Ray traces weapon animation when melee attacking
  (bind _outhits (Class|KismetSystemLibrary|CapsuleTraceMulti (Transformation|GetSocketLocation _sword "start") (Transformation|GetSocketLocation _sword "end") 55.0 0.0 "TraceTypeQuery1" false 0 "None" true))
  (bind _array_element (Utilities|Array|ForEachLoopwithBreak _outhits)
    (:LoopBody
      (if (not (Utilities|Array|ContainsItem _actorhitbytrace (.HitActor (Collision|BreakHitResult _array_element))))
        (Utilities|Array|Add _actorhitbytrace (.HitActor (Collision|BreakHitResult _array_element)))
        (Class|BPIDamagable|DealDamage(Message) (.HitActor (Collision|BreakHitResult _array_element)) (Utilities|Struct|MakeS_DamageInfo (Math|Random|RandomFloatinRange (Variables|/Game/Player/Blueprints/BPC_PlayerCombatHandler.BPC_PlayerCombatHandler_C|GetMinDamage _bpc_playermeleebasic) (Variables|/Game/Player/Blueprints/BPC_PlayerCombatHandler.BPC_PlayerCombatHandler_C|GetMaxDamage _bpc_playermeleebasic)) "NewEnumerator3" "NewEnumerator1"))
        (Default|CallOnReduceDashCD (Variables|Default|GetBPC_PlayerDash) 8.0)
        (if (== (Variables|Default|GetattackCount) 3)
          (if (Class|GameplayStatics|ObjectIsA (.HitActor (Collision|BreakHitResult _array_element)) "/Game/Enemies/Blueprints/BP_EnemyBase.BP_EnemyBase_C")
            (Class|BPIDamagable|TimeDilation(Message) (Variables|/Game/Player/Blueprints/BP_PlayerCharacter.BP_PlayerCharacter_C|GetBPC_DamageSystem (Variables|Default|GetBP_PlayerCharacter)) 0.08 0.2)))))))

(event Custom|StopWeaponTrace
  ;[0.05098 0.05098 0.05098] Ray traces weapon animation when melee attacking
  (Utilities|Time|ClearandInvalidateTimerbyHandle (Variables|Default|GetswordTracingTimerHandle))
  (Utilities|Array|Clear (Variables|Default|GetactorHitByTrace)))

(event Custom|ApplyForce
  (params (Strength :type Float%20%28double-precision%29))
  ;[0.05098 0.05098 0.05098] Apply force when melee attacking
  (if (not (Variables|/Game/Player/Blueprints/BPC_PlayerDash.BPC_PlayerDash_C|GetIs%20Dashing (Variables|Default|GetBPC_PlayerDash)))
    (if (>= (Math|Vector|Distance2D(Vector) (Variables|Default|GetTargetEnemyLocation) (Transformation|GetActorLocation (Variables|Default|GetBP_PlayerCharacter))) 225.0)
      (CallFunction|ApplyForceStartTimer)
      (Utilities|SetMousePOS)
      (Utilities|TogglesBrakingFriction))))

(event Custom|CancelApplyForce
  ;[0.05098 0.05098 0.05098] Apply force when melee attacking
  (Utilities|Time|ClearandInvalidateTimerbyHandle (Variables|ApplyForce|GetapplyForceTimerHandle))
  (Variables|ApplyForce|SetapplyForceTimer 0.0))

(event Custom|MeleeBasicAttack
  ;[0.05098 0.05098 0.05098] Attack
  (bind _targettedenemy (Default|GetClosestEnemy (Variables|Default|GetBPC_PlayerCombatHandler)))
  (Utilities|IsValid _targettedenemy
    (:Is%20Valid
      (bind _output_get (Variables|Default|SetTargetEnemy _targettedenemy))
      (Variables|Default|SetTargetEnemyLocation (Transformation|GetActorLocation _output_get))
      (Default|RotatetoClosestEnemy (Variables|Default|GetBPC_PlayerCombatHandler)))
    (:Is%20Not%20Valid
      (CallFunction|RotateTowardsMousePOS)))
  (Default|ToggleEnableMovementInput (Variables|Default|GetBP_PlayerCharacter) false true)
  (if (Variables|/Game/Player/Blueprints/BPC_PlayerDash.BPC_PlayerDash_C|GetIs%20Dashing (Variables|Default|GetBPC_PlayerDash))
    (CallFunction|BasicDashAttack)
    (else
      (CallFunction|BasicAttack))))

(event Custom|BasicAttack
  ;[0.05098 0.05098 0.05098] Melee attack
  (CallFunction|ApplyForce (+ (Variables|ApplyForce|GetapplyForceStrength) 0.0))
  (Animation|Montage|PlayMontage (Variables|Default|GetPlayerMesh) (Utilities|Array|Get(acopy) (Variables|Default|GetattackAnims) (Variables|Default|GetattackCount)) (Variables|/Game/Player/Blueprints/BPC_PlayerCombatHandler.BPC_PlayerCombatHandler_C|GetAnimationPlayRate (Variables|Default|GetBPC_PlayerMeleeBasic))
    (:then
      (Math|Integer|IncrementInt (Variables|Default|GetattackCount)))
    (:OnCompleted
      (Variables|Default|SetattackCount 0 :!label _label)
      (CallFunction|FinishedAttacking))
    (:OnInterrupted
      (Utilities|FlowControl|RetriggerableDelay 2.0)
      (goto _label))))

(event Custom|ApplyForceStartTimer
  ;[0.05098 0.05098 0.05098] Apply force when melee attacking
  (bind _returnvalue (Utilities|Time|SetTimerbyEvent (delegate Custom|ApplyForceStartTimer) 0.001 true))
  (CallFunction|ApplyForceTimerFunction _returnvalue)
  (bind (_returnvalue_x _returnvalue_y) (CallFunction|CalculateForce (stale Custom|ApplyForce Strength)))
  (Character|LaunchCharacter (Variables|Default|GetBP_PlayerCharacter) (Math|Vector|MakeVector _returnvalue_x _returnvalue_y 0.0) false false))

(event Custom|BasicDashAttack
  ;[0.05098 0.05098 0.05098] Melee attack
  (CallFunction|ApplyForce (+ (Variables|ApplyForce|GetapplyForceStrength) 5e+01))
  (Animation|Montage|PlayMontage (Variables|Default|GetPlayerMesh) "/Game/Characters/Mannequins/Animations/Attack_Animations/StandingMeleeAttack360High_UE_Montage.StandingMeleeAttack360High_UE_Montage" 3.1
    (:OnCompleted
      _)
    (:OnInterrupted
      (Utilities|FlowControl|RetriggerableDelay 2.0)))
  (Default|FinishedAttacking (Variables|Default|GetBPC_PlayerCombatHandler)))

(event EventBeginPlay
  ;[0.05098 0.05098 0.05098] Setup
  (|CallParentFunction)
  (EventDispatchers|BindEventtoOnDashCancelOtherForces (Variables|Default|GetBPC_PlayerDash) (EventDispatchers|CreateEvent :!event Custom|CancelApplyForce)))

(fn ApplyForceTimerFunction
  (params (TimerHandle :type Timer%20Handle%20Structure))
  (Variables|ApplyForce|SetapplyForceTimerHandle TimerHandle)
  (bind _output_get (Variables|ApplyForce|SetapplyForceTimer (+ 0.01 (Variables|ApplyForce|GetapplyForceTimer))))
  (if (>= (Variables|ApplyForce|GetapplyForceDuration) _output_get)
    (return)
    (else
      (CallFunction|CancelApplyForce))))

(fn CheckCanAttack
  (bind _canattack (|CallParentFunction))
  (if _canattack
    (if (Variables|/Game/Player/Blueprints/BPC_PlayerCombatHandler.BPC_PlayerCombatHandler_C|GetCanAttack (Variables|Default|GetBPC_PlayerMeleeBasic))
      (if (== (Variables|Default|GetattackCount) 4)
        (return false)
        (else
          (return true)))
      (else
        (return false)))
    (else
      (return false))))

(fn HandleFinishedAttacking
  (bind _bpc_playermeleebasic (Variables|Default|GetBPC_PlayerMeleeBasic))
  (|CallParentFunction)
  (Variables|/Game/Player/Blueprints/BPC_PlayerCombatHandler.BPC_PlayerCombatHandler_C|SetCanAttack _bpc_playermeleebasic true)
  (if (>= (Variables|BPC_PlayerMeleeBasic_C|GetattackCount _bpc_playermeleebasic) 4)
    (Variables|BPC_PlayerMeleeBasic_C|SetattackCount _bpc_playermeleebasic 0)))

(fn CalculateForce
  (params (Strength :type Float%20%28double-precision%29))
  (bind _bp_playercharacter (Variables|Default|GetBP_PlayerCharacter))
  (bind _savedmousepos (Variables|Default|GetSavedMousePOS))
  (bind _targetenemy (Variables|Default|GetTargetEnemy))
  (bind _targetenemylocation (Variables|Default|GetTargetEnemyLocation))
  (bind _returnvalue (Utilities|IsValid _targetenemy))
  (bind _returnvalue_2 (Transformation|GetActorLocation _bp_playercharacter))
  (bind _returnvalue_3 (- _targetenemylocation _returnvalue_2))
  (bind _returnvalue_4 (- _savedmousepos _returnvalue_2))
  (bind _returnvalue_5 (Math|Vector|SelectVector _returnvalue_3 _returnvalue_4 _returnvalue))
  (bind _returnvalue_6 (Math|Vector|Normalize _returnvalue_5))
  (bind _returnvalue_7 (* Strength _returnvalue_6))
  (return (.x _returnvalue_7) (.y _returnvalue_7)))