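; Player upgrade component that pauses the game to offer three upgrade choices and applies the chosen one.
; On BeginPlay it caches player and game mode, binds events and puts a pop-up in the player's widget component.
; Choices always lead with max HP, then two random picks drawn without duplicates from a temporary array.
; Choosing unpauses with a time-dilation fade, resets attacks and boosts health, melee, ranged or dash stats.
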(event Custom|UpgradeChosen
  (params (UpgradeChosen :type E_Upgrades%20Enum :default "NewEnumerator0"))
  ;[0.5294 0.5294 0.5294] Called When upgrade has been choosen (OnClick) and upgrades depending on upgrade chosen
  (Game|SetGamePaused false)
  (Default|CallFadeTimeDilation (Variables|Objects|GetBP_ThirdPersonGameMode) true 0.02 0.0)
  (Utilities|ToggleUpgradeWidget false)
  (Default|ResetAllAttacks (Variables|/Game/Player/Blueprints/BP_PlayerCharacter.BP_PlayerCharacter_C|GetBPC_PlayerCombatHandler (Variables|Objects|GetBP_PlayerCharacter)))
  (switch Utilities|FlowControl|Switch|SwitchonE_Upgrades UpgradeChosen
    (:NewEnumerator1
      (CallFunction|UpgradeHP))
    (:NewEnumerator2
      (CallFunction|UpgradeBasicMelee))
    (:NewEnumerator4
      (CallFunction|UpgradeBasicRanged))
    (:NewEnumerator3
      (CallFunction|UpgradeDash))))

(event Custom|ShowUpgrades
  ;[0.5294 0.5294 0.5294] Shows upgrade widget
  (Game|SetGamePaused true)
  (Utilities|ToggleUpgradeWidget true)
  (CallFunction|GenerateRandomUpgrades self)
  (Default|CallShowUpgradeWidget (Variables|Objects|GetWB_UpgradeWidget) (Variables|Default|GetE_UpgradePerChoice)))

(event EventBeginPlay
  ;[0.5294 0.5294 0.5294] Setup
  (|GetObjects)
  (|BindEvents)
  (bind _returnvalue (UserInterface|CreateWidget "/Game/Upgrades/Blueprints/WB_UpgradePopUp.WB_UpgradePopUp_C" (Game|GetPlayerController 0) (Variables|Objects|GetBP_PlayerCharacter) (Variables|Default|GetE_UpgradePerChoice)))
  (bind _output_get (Variables|Objects|SetWB_UpgradeWidget _returnvalue))
  (UserInterface|SetWidget (Variables|/Game/Player/Blueprints/BP_PlayerCharacter.BP_PlayerCharacter_C|GetUpgrade%20%28Widget%29 (Variables|Objects|GetBP_PlayerCharacter)) _output_get)
  (Utilities|ToggleUpgradeWidget false))

(fn UpgradeBasicMelee
  (bind _bp_playercharacter (Variables|Objects|GetBP_PlayerCharacter))
  (bind _bpc_playermeleebasic (Variables|/Game/Player/Blueprints/BP_PlayerCharacter.BP_PlayerCharacter_C|GetBPC_PlayerMeleeBasic _bp_playercharacter))
  (Variables|/Game/Player/Blueprints/BPC_PlayerCombatHandler.BPC_PlayerCombatHandler_C|SetMinDamage _bpc_playermeleebasic (+ (Variables|/Game/Player/Blueprints/BPC_PlayerCombatHandler.BPC_PlayerCombatHandler_C|GetMinDamage _bpc_playermeleebasic) 1e+01))
  (Variables|/Game/Player/Blueprints/BPC_PlayerCombatHandler.BPC_PlayerCombatHandler_C|SetMaxDamage _bpc_playermeleebasic (+ (Variables|/Game/Player/Blueprints/BPC_PlayerCombatHandler.BPC_PlayerCombatHandler_C|GetMaxDamage _bpc_playermeleebasic) 1e+01)))

(fn UpgradeBasicRanged
  (bind _bp_playercharacter (Variables|Objects|GetBP_PlayerCharacter))
  (bind _bpc_playerrangedbasic (Variables|/Game/Player/Blueprints/BP_PlayerCharacter.BP_PlayerCharacter_C|GetBPC_PlayerRangedBasic _bp_playercharacter))
  (Variables|/Game/Player/Blueprints/BPC_PlayerCombatHandler.BPC_PlayerCombatHandler_C|SetMinDamage _bpc_playerrangedbasic (+ (Variables|/Game/Player/Blueprints/BPC_PlayerCombatHandler.BPC_PlayerCombatHandler_C|GetMinDamage _bpc_playerrangedbasic) 1e+01))
  (Variables|/Game/Player/Blueprints/BPC_PlayerCombatHandler.BPC_PlayerCombatHandler_C|SetMaxDamage _bpc_playerrangedbasic (+ (Variables|/Game/Player/Blueprints/BPC_PlayerCombatHandler.BPC_PlayerCombatHandler_C|GetMaxDamage _bpc_playerrangedbasic) 1e+01)))

(fn UpgradeDash
  (bind _bp_playercharacter (Variables|Objects|GetBP_PlayerCharacter))
  (bind _bpc_playerdash (Variables|/Game/Player/Blueprints/BP_PlayerCharacter.BP_PlayerCharacter_C|GetBPC_PlayerDash _bp_playercharacter))
  (Variables|/Game/Player/Blueprints/BPC_PlayerDash.BPC_PlayerDash_C|SetDash%20CDDuration _bpc_playerdash (- (Variables|/Game/Player/Blueprints/BPC_PlayerDash.BPC_PlayerDash_C|GetDash%20CDDuration _bpc_playerdash) 0.4)))

(fn UpgradeHP
  (bind _bp_playercharacter (Variables|Objects|GetBP_PlayerCharacter))
  (bind _bpc_damagesystem (Variables|/Game/Player/Blueprints/BP_PlayerCharacter.BP_PlayerCharacter_C|GetBPC_DamageSystem _bp_playercharacter))
  (bind _output_get (Variables|/Game/DamageSystem/BPC_DamageSystem.BPC_DamageSystem_C|SetmaxHealth _bpc_damagesystem (+ (Variables|/Game/DamageSystem/BPC_DamageSystem.BPC_DamageSystem_C|GetmaxHealth _bpc_damagesystem) 75.0)))
  (Variables|/Game/DamageSystem/BPC_DamageSystem.BPC_DamageSystem_C|Sethealth _bpc_damagesystem _output_get))

(fn GenerateRandomUpgrades
  ;[0.5294 0.5294 0.5294] Sets TEMPUpgrades so i can remove upgrade indexes from array and prevent duplicates
  (LocalVariables|SetTEMPUpgrades (Variables|Default|GetE_Upgrades))
  ;[0.5294 0.5294 0.5294 1 19] Find & set TEMPRandomUpgrade -> add into map with choice x as key -> remove TEMPRandomUpgrade index from TEMPUpgrades -> repeat
  (LocalVariables|SetTEMPRandomUpgrade (.OutItem (Utilities|Array|Random (LocalVariables|GetTEMPUpgrades))))
  (Utilities|Map|Add (Variables|Default|GetE_UpgradePerChoice) "NewEnumerator0" "NewEnumerator1")
  (Utilities|Array|RemoveItem (LocalVariables|GetTEMPUpgrades) "NewEnumerator1")
  (bind _output_get (LocalVariables|SetTEMPRandomUpgrade (.OutItem (Utilities|Array|Random (LocalVariables|GetTEMPUpgrades)))))
  (Utilities|Map|Add (Variables|Default|GetE_UpgradePerChoice) "NewEnumerator1" _output_get)
  (Utilities|Array|RemoveItem (LocalVariables|GetTEMPUpgrades) _output_get)
  (bind _output_get_2 (LocalVariables|SetTEMPRandomUpgrade (.OutItem (Utilities|Array|Random (LocalVariables|GetTEMPUpgrades)))))
  (Utilities|Map|Add (Variables|Default|GetE_UpgradePerChoice) "NewEnumerator2" _output_get_2))