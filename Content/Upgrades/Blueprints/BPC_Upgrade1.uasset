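; Upgrade component that offers the player three random upgrades in a widget and applies the chosen one to health, dash and combat components.
; Showing upgrades runs a game-mode time-dilation curve, then pauses the game; choosing unpauses and reverses it.
; Choices draw without duplicates, excluding one-time upgrades already taken (WIP lifesteal and piercing arrows, bound to attack events).
; Stat upgrades increment a tier; only dash cooldown and melee damage are written to BP_SaveGame.
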(event Custom|UpgradeChosen
  (params (UpgradeChosen :type E_Upgrades%20Enum :default "NewEnumerator0"))
  (bind _bp_playercharacter (Variables|Objects|GetBP_PlayerCharacter))
  (bind _e_takenupgrades (Variables|Default|GetE_TakenUpgrades))
  ;[0.03529 0.03529 0.03529] Called When upgrade has been choosen (OnClick) and upgrades depending on upgrade chosen
  (Game|SetGamePaused false)
  (Rendering|SetVisibility (Variables|/Game/Player/Blueprints/BP_PlayerCharacter.BP_PlayerCharacter_C|GetHealthBar%20%28Widget%29 (Variables|Objects|GetBP_PlayerCharacter)) true false)
  (Default|TimeDilationDelay (Variables|Objects|GetBP_ThirdPersonGameMode) "/Game/UI/TimeDilation/UpgradeCurve.UpgradeCurve" true)
  (Utilities|ToggleUpgradeWidget false)
  (Default|ResetAllAttacks (Variables|/Game/Player/Blueprints/BP_PlayerCharacter.BP_PlayerCharacter_C|GetBPC_PlayerCombatHandler (Variables|Objects|GetBP_PlayerCharacter)))
  (switch Utilities|FlowControl|Switch|SwitchonE_Upgrades UpgradeChosen
    (:NewEnumerator1
      (CallFunction|UpgradeHP "NewEnumerator1"))
    (:NewEnumerator3
      (CallFunction|UpgradeDash "NewEnumerator3"))
    (:NewEnumerator2
      (CallFunction|UpgradeMeleeDamage "NewEnumerator2"))
    (:NewEnumerator4
      (CallFunction|UpgradeRangedDamage "NewEnumerator4"))
    (:NewEnumerator9
      (CallFunction|UpgradeSlam "NewEnumerator9"))
    (:NewEnumerator8
      (CallFunction|UpgradeHookDamage "NewEnumerator8"))
    (:NewEnumerator6
      (CallFunction|UpgradeMeleeAttackSpeed "NewEnumerator6"))
    (:NewEnumerator7
      (CallFunction|UpgradeRangedAttackSpeed "NewEnumerator7"))
    (:NewEnumerator10
      (EventDispatchers|BindEventtoOnTriggerWeaponTrace (Variables|/Game/Player/Blueprints/BP_PlayerCharacter.BP_PlayerCharacter_C|GetBPC_PlayerMeleeBasic _bp_playercharacter) (EventDispatchers|CreateEvent :!event UpgradeLifeSteal))
      (Utilities|Array|AddUnique _e_takenupgrades UpgradeChosen))
    (:NewEnumerator12
      (EventDispatchers|BindEventtoOnTriggerSpawnProjectile (Variables|/Game/Player/Blueprints/BP_PlayerCharacter.BP_PlayerCharacter_C|GetBPC_PlayerRangedBasic _bp_playercharacter) (EventDispatchers|CreateEvent :!event UpgradePiercingArrows))
      (Utilities|Array|AddUnique _e_takenupgrades UpgradeChosen))))

(event Custom|DelayFinished
  ;[0.03529 0.03529 0.03529] Shows upgrade widget
  (Utilities|ToggleUpgradeWidget true)
  (CallFunction|GenerateRandomUpgrades self)
  (Default|CallShowUpgradeWidget (Variables|Objects|GetWB_UpgradeWidget) (Variables|Default|GetE_UpgradePerChoice))
  (Game|SetGamePaused true))

(event Custom|ShowUpgrades
  ;[0.03529 0.03529 0.03529] Shows upgrade widget
  (Default|TimeDilationDelay (Variables|Objects|GetBP_ThirdPersonGameMode) "/Game/UI/TimeDilation/UpgradeCurve.UpgradeCurve" false)
  (Utilities|FlowControl|Delay 0.3)
  (Rendering|SetVisibility (Variables|/Game/Player/Blueprints/BP_PlayerCharacter.BP_PlayerCharacter_C|GetHealthBar%20%28Widget%29 (Variables|Objects|GetBP_PlayerCharacter)) false false))

(event EventBeginPlay
  ;[0.03529 0.03529 0.03529] Setup
  (|GetObjects)
  (|BindEvents)
  (bind _returnvalue (UserInterface|CreateWidget "/Game/Upgrades/Blueprints/WB_UpgradePopUp.WB_UpgradePopUp_C" (Game|GetPlayerController 0) (Variables|Objects|GetBP_PlayerCharacter) (Variables|Default|GetE_UpgradePerChoice)))
  (bind _output_get (Variables|Objects|SetWB_UpgradeWidget _returnvalue))
  (UserInterface|SetWidget (Variables|/Game/Player/Blueprints/BP_PlayerCharacter.BP_PlayerCharacter_C|GetUpgrade%20%28Widget%29 (Variables|Objects|GetBP_PlayerCharacter)) _output_get)
  (Utilities|ToggleUpgradeWidget false))

(fn GenerateRandomUpgrades
  ;[0.03529 0.03529 0.03529] Sets TEMPUpgrades so i can remove upgrade indexes from array and prevent duplicates
  (bind _output_get (LocalVariables|SetTEMPUpgrades (Variables|Default|GetE_Upgrades)))
  ;[0.03529 0.03529 0.03529] Remove special upgrades that can only be taken once. Empty per default
  (for _array_element (Variables|Default|GetE_TakenUpgrades)
    (Utilities|Array|RemoveItem _output_get _array_element))
  ;[0.03529 0.03529 0.03529 1 19] Find & set TEMPRandomUpgrade -> add into map with choice x as key -> remove TEMPRandomUpgrade index from TEMPUpgrades -> repeat
  (bind _output_get_2 (LocalVariables|SetTEMPRandomUpgrade (.OutItem (Utilities|Array|Random (LocalVariables|GetTEMPUpgrades)))))
  (Utilities|Map|Add (Variables|Default|GetE_UpgradePerChoice) "NewEnumerator0" _output_get_2)
  (Utilities|Array|RemoveItem (LocalVariables|GetTEMPUpgrades) _output_get_2)
  (bind _output_get_3 (LocalVariables|SetTEMPRandomUpgrade (.OutItem (Utilities|Array|Random (LocalVariables|GetTEMPUpgrades)))))
  (Utilities|Map|Add (Variables|Default|GetE_UpgradePerChoice) "NewEnumerator1" _output_get_3)
  (Utilities|Array|RemoveItem (LocalVariables|GetTEMPUpgrades) _output_get_3)
  (bind _output_get_4 (LocalVariables|SetTEMPRandomUpgrade (.OutItem (Utilities|Array|Random (LocalVariables|GetTEMPUpgrades)))))
  (Utilities|Map|Add (Variables|Default|GetE_UpgradePerChoice) "NewEnumerator2" _output_get_4))

(fn UpgradeHP
  (params (E_Upgrade :type E_Upgrades%20Enum :default "NewEnumerator5"))
  (bind _bp_playercharacter (Variables|Objects|GetBP_PlayerCharacter))
  (bind _s_upgradeinfo (Variables|Default|GetS_UpgradeInfo))
  (bind _value (Utilities|Map|Find _s_upgradeinfo E_Upgrade))
  (bind _bpc_damagesystem (Variables|/Game/Player/Blueprints/BP_PlayerCharacter.BP_PlayerCharacter_C|GetBPC_DamageSystem _bp_playercharacter))
  (bind (_upgradetier _upgradevalue) (Utilities|Struct|BreakS_Upgrades _value))
  (Math|Integer|IncrementInt _upgradetier
    (:%20%20
      (bind _output_get (LocalVariables|SetNewMaxHealth (* (+ (/ _upgradevalue 1e+02) 1.0) (Variables|/Game/DamageSystem/BPC_DamageSystem.BPC_DamageSystem_C|GetmaxHealth (Variables|/Game/Player/Blueprints/BP_PlayerCharacter.BP_PlayerCharacter_C|GetBPC_DamageSystem (Variables|Objects|GetBP_PlayerCharacter))))))
      ;[0.08854 0.08854 0.08854] Set current Health to (NewMaxHealth - MaxHealth) + Health
      ; This will add the hp gained from the upgrade to current health
      (Variables|/Game/DamageSystem/BPC_DamageSystem.BPC_DamageSystem_C|Sethealth _bpc_damagesystem (+ (- _output_get (Variables|/Game/DamageSystem/BPC_DamageSystem.BPC_DamageSystem_C|GetmaxHealth _bpc_damagesystem)) (Variables|/Game/DamageSystem/BPC_DamageSystem.BPC_DamageSystem_C|Gethealth _bpc_damagesystem)))
      (Variables|/Game/DamageSystem/BPC_DamageSystem.BPC_DamageSystem_C|SetmaxHealth _bpc_damagesystem _output_get))))

(fn UpgradeDash
  (params (E_Upgrade :type E_Upgrades%20Enum :default "NewEnumerator5"))
  (bind _s_upgradeinfo (Variables|Default|GetS_UpgradeInfo))
  (bind _bp_playercharacter (Variables|Objects|GetBP_PlayerCharacter))
  (bind _value (Utilities|Map|Find _s_upgradeinfo E_Upgrade))
  (bind _bpc_playerdash (Variables|/Game/Player/Blueprints/BP_PlayerCharacter.BP_PlayerCharacter_C|GetBPC_PlayerDash _bp_playercharacter))
  (bind (_upgradetier _upgradevalue) (Utilities|Struct|BreakS_Upgrades _value))
  (Math|Integer|IncrementInt _upgradetier
    (:%20%20
      (bind _output_get (Variables|/Game/Player/Blueprints/BPC_PlayerDash.BPC_PlayerDash_C|SetDash%20CDDuration _bpc_playerdash (+ (Variables|/Game/Player/Blueprints/BPC_PlayerDash.BPC_PlayerDash_C|GetDash%20CDDuration _bpc_playerdash) _upgradevalue)))
      (bind _asbp_save_game (Utilities|Casting|CastToBP_SaveGame (Game|GetGameInstance)))
      (Variables|/Game/SaveSystem/BP_SaveGame.BP_SaveGame_C|SetDashCDDuration _asbp_save_game _output_get))))

(fn UpgradeMeleeDamage
  (params (E_Upgrade :type E_Upgrades%20Enum :default "NewEnumerator5"))
  (bind _s_upgradeinfo (Variables|Default|GetS_UpgradeInfo))
  (bind _bp_playercharacter (Variables|Objects|GetBP_PlayerCharacter))
  (bind _value (Utilities|Map|Find _s_upgradeinfo E_Upgrade))
  (bind _bpc_playermeleebasic (Variables|/Game/Player/Blueprints/BP_PlayerCharacter.BP_PlayerCharacter_C|GetBPC_PlayerMeleeBasic _bp_playercharacter))
  (bind (_upgradetier _upgradevalue) (Utilities|Struct|BreakS_Upgrades _value))
  (Math|Integer|IncrementInt _upgradetier
    (:%20%20
      (bind _output_get (Variables|/Game/Player/Blueprints/BPC_PlayerCombatHandler.BPC_PlayerCombatHandler_C|SetMinDamage _bpc_playermeleebasic (+ _upgradevalue (Variables|/Game/Player/Blueprints/BPC_PlayerCombatHandler.BPC_PlayerCombatHandler_C|GetMinDamage _bpc_playermeleebasic))))
      (bind _output_get_2 (Variables|/Game/Player/Blueprints/BPC_PlayerCombatHandler.BPC_PlayerCombatHandler_C|SetMaxDamage _bpc_playermeleebasic (+ _upgradevalue (Variables|/Game/Player/Blueprints/BPC_PlayerCombatHandler.BPC_PlayerCombatHandler_C|GetMaxDamage _bpc_playermeleebasic))))
      (Development|PrintString (Utilities|String|ToString(Float) (Variables|/Game/Player/Blueprints/BPC_PlayerCombatHandler.BPC_PlayerCombatHandler_C|GetMaxDamage _bpc_playermeleebasic)))
      (bind _asbp_save_game (Utilities|Casting|CastToBP_SaveGame (Game|GetGameInstance)))
      (Variables|/Game/SaveSystem/BP_SaveGame.BP_SaveGame_C|SetMeleeDamageMin _asbp_save_game _output_get)
      (Variables|/Game/SaveSystem/BP_SaveGame.BP_SaveGame_C|SetMeleeDamageMax _asbp_save_game _output_get_2))))

(fn UpgradeRangedDamage
  (params (E_Upgrade :type E_Upgrades%20Enum :default "NewEnumerator5"))
  (bind _bp_playercharacter (Variables|Objects|GetBP_PlayerCharacter))
  (bind _s_upgradeinfo (Variables|Default|GetS_UpgradeInfo))
  (bind _value (Utilities|Map|Find _s_upgradeinfo E_Upgrade))
  (bind _bpc_playerrangedbasic (Variables|/Game/Player/Blueprints/BP_PlayerCharacter.BP_PlayerCharacter_C|GetBPC_PlayerRangedBasic _bp_playercharacter))
  (bind (_upgradetier _upgradevalue) (Utilities|Struct|BreakS_Upgrades _value))
  (Math|Integer|IncrementInt _upgradetier
    (:%20%20
      (Variables|/Game/Player/Blueprints/BPC_PlayerCombatHandler.BPC_PlayerCombatHandler_C|SetMinDamage _bpc_playerrangedbasic (+ _upgradevalue (Variables|/Game/Player/Blueprints/BPC_PlayerCombatHandler.BPC_PlayerCombatHandler_C|GetMinDamage _bpc_playerrangedbasic)))
      (Variables|/Game/Player/Blueprints/BPC_PlayerCombatHandler.BPC_PlayerCombatHandler_C|SetMaxDamage _bpc_playerrangedbasic (+ _upgradevalue (Variables|/Game/Player/Blueprints/BPC_PlayerCombatHandler.BPC_PlayerCombatHandler_C|GetMaxDamage _bpc_playerrangedbasic))))))

(fn UpgradeSlam
  (params (E_Upgrade :type E_Upgrades%20Enum :default "NewEnumerator5"))
  (bind _bp_playercharacter (Variables|Objects|GetBP_PlayerCharacter))
  (bind _s_upgradeinfo (Variables|Default|GetS_UpgradeInfo))
  (bind _value (Utilities|Map|Find _s_upgradeinfo E_Upgrade))
  (bind _bpc_playermeleeheavy (Variables|/Game/Player/Blueprints/BP_PlayerCharacter.BP_PlayerCharacter_C|GetBPC_PlayerMeleeHeavy _bp_playercharacter))
  (bind (_upgradetier _upgradevalue) (Utilities|Struct|BreakS_Upgrades _value))
  (Math|Integer|IncrementInt _upgradetier
    (:%20%20
      (Variables|/Game/Player/Blueprints/BPC_PlayerCombatHandler.BPC_PlayerCombatHandler_C|SetMinDamage _bpc_playermeleeheavy (+ _upgradevalue (Variables|/Game/Player/Blueprints/BPC_PlayerCombatHandler.BPC_PlayerCombatHandler_C|GetMinDamage _bpc_playermeleeheavy)))
      (Variables|/Game/Player/Blueprints/BPC_PlayerCombatHandler.BPC_PlayerCombatHandler_C|SetMaxDamage _bpc_playermeleeheavy (+ _upgradevalue (Variables|/Game/Player/Blueprints/BPC_PlayerCombatHandler.BPC_PlayerCombatHandler_C|GetMaxDamage _bpc_playermeleeheavy))))))

(fn UpgradeHookDamage
  (params (E_Upgrade :type E_Upgrades%20Enum :default "NewEnumerator5"))
  (bind _s_upgradeinfo (Variables|Default|GetS_UpgradeInfo))
  (bind _bp_playercharacter (Variables|Objects|GetBP_PlayerCharacter))
  (bind _value (Utilities|Map|Find _s_upgradeinfo E_Upgrade))
  (bind _bpc_playerhook (Variables|/Game/Player/Blueprints/BP_PlayerCharacter.BP_PlayerCharacter_C|GetBPC_PlayerHook _bp_playercharacter))
  (bind (_upgradetier _upgradevalue) (Utilities|Struct|BreakS_Upgrades _value))
  (Math|Integer|IncrementInt _upgradetier
    (:%20%20
      (Variables|/Game/Player/Blueprints/BPC_PlayerCombatHandler.BPC_PlayerCombatHandler_C|SetMinDamage _bpc_playerhook (+ _upgradevalue (Variables|/Game/Player/Blueprints/BPC_PlayerCombatHandler.BPC_PlayerCombatHandler_C|GetMinDamage _bpc_playerhook)))
      (Variables|/Game/Player/Blueprints/BPC_PlayerCombatHandler.BPC_PlayerCombatHandler_C|SetMaxDamage _bpc_playerhook (+ _upgradevalue (Variables|/Game/Player/Blueprints/BPC_PlayerCombatHandler.BPC_PlayerCombatHandler_C|GetMaxDamage _bpc_playerhook))))))

(fn UpgradeMeleeAttackSpeed
  (params (E_Upgrade :type E_Upgrades%20Enum :default "NewEnumerator5"))
  (bind _bp_playercharacter (Variables|Objects|GetBP_PlayerCharacter))
  (bind _s_upgradeinfo (Variables|Default|GetS_UpgradeInfo))
  (bind _value (Utilities|Map|Find _s_upgradeinfo E_Upgrade))
  (bind _bpc_playermeleebasic (Variables|/Game/Player/Blueprints/BP_PlayerCharacter.BP_PlayerCharacter_C|GetBPC_PlayerMeleeBasic _bp_playercharacter))
  (bind (_upgradetier _upgradevalue) (Utilities|Struct|BreakS_Upgrades _value))
  (Math|Integer|IncrementInt _upgradetier
    (:%20%20
      (Variables|/Game/Player/Blueprints/BPC_PlayerCombatHandler.BPC_PlayerCombatHandler_C|SetAnimationPlayRate _bpc_playermeleebasic (* (+ (/ _upgradevalue 1e+02) 1.0) (Variables|/Game/Player/Blueprints/BPC_PlayerCombatHandler.BPC_PlayerCombatHandler_C|GetAnimationPlayRate _bpc_playermeleebasic))))))

(fn UpgradeRangedAttackSpeed
  (params (E_Upgrade :type E_Upgrades%20Enum :default "NewEnumerator5"))
  (bind _s_upgradeinfo (Variables|Default|GetS_UpgradeInfo))
  (bind _bp_playercharacter (Variables|Objects|GetBP_PlayerCharacter))
  (bind _value (Utilities|Map|Find _s_upgradeinfo E_Upgrade))
  (bind _bpc_playerrangedbasic (Variables|/Game/Player/Blueprints/BP_PlayerCharacter.BP_PlayerCharacter_C|GetBPC_PlayerRangedBasic _bp_playercharacter))
  (bind (_upgradetier _upgradevalue) (Utilities|Struct|BreakS_Upgrades _value))
  (Math|Integer|IncrementInt _upgradetier
    (:%20%20
      (Variables|/Game/Player/Blueprints/BPC_PlayerCombatHandler.BPC_PlayerCombatHandler_C|SetAnimationPlayRate _bpc_playerrangedbasic (* (+ (/ _upgradevalue 1e+02) 1.0) (Variables|/Game/Player/Blueprints/BPC_PlayerCombatHandler.BPC_PlayerCombatHandler_C|GetAnimationPlayRate _bpc_playerrangedbasic))))))

(fn UpgradeLifeSteal
  (bind _bp_playercharacter (Variables|Objects|GetBP_PlayerCharacter))
  (bind _bpc_damagesystem (Variables|/Game/Player/Blueprints/BP_PlayerCharacter.BP_PlayerCharacter_C|GetBPC_DamageSystem _bp_playercharacter))
  (bind _maxhealth (Variables|/Game/DamageSystem/BPC_DamageSystem.BPC_DamageSystem_C|GetmaxHealth _bpc_damagesystem))
  (Development|PrintString "LifeStealActivated")
  (for _array_element (Variables|/Game/Player/Blueprints/BPC_PlayerMeleeBasic.BPC_PlayerMeleeBasic_C|GetactorHitByTrace (Variables|/Game/Player/Blueprints/BP_PlayerCharacter.BP_PlayerCharacter_C|GetBPC_PlayerMeleeBasic _bp_playercharacter))
    (Development|PrintString "life stolen")
    (Math|Float|CompareFloat (+ (Variables|/Game/DamageSystem/BPC_DamageSystem.BPC_DamageSystem_C|Gethealth _bpc_damagesystem) (/ _maxhealth 1e+02)) _maxhealth
      (:>
        (Variables|/Game/DamageSystem/BPC_DamageSystem.BPC_DamageSystem_C|Sethealth _bpc_damagesystem _maxhealth :!label _label))
      (:==
        (goto _label))
      (:<
        (Variables|/Game/DamageSystem/BPC_DamageSystem.BPC_DamageSystem_C|Sethealth _bpc_damagesystem (+ (Variables|/Game/DamageSystem/BPC_DamageSystem.BPC_DamageSystem_C|Gethealth _bpc_damagesystem) (/ _maxhealth 1e+02)))))))

(fn UpgradePiercingArrows
  (Variables|/Game/Projectile/Blueprints/BP_ProjectileArrow.BP_ProjectileArrow_C|SetIsPiercing (Variables|/Game/Player/Blueprints/BPC_PlayerRangedBasic.BPC_PlayerRangedBasic_C|GetSpawnedArrow (Variables|/Game/Player/Blueprints/BP_PlayerCharacter.BP_PlayerCharacter_C|GetBPC_PlayerRangedBasic (Variables|Objects|GetBP_PlayerCharacter))) true))