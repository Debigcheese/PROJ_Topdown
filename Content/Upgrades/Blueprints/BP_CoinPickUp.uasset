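; Coin pickup actor that automatically flies to the player and credits coins, with no contact required.
; Tick waits through a delay, then plays a timeline that lerps the Cube from its current location toward the player character.
; A shorter delay, started from the timeline update, calls AddCoins on the player's BPCCoins component and destroys the actor.
; The Sphere overlap only checks the Player tag and triggers nothing.
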(event OnComponentBeginOverlap(Sphere)
  (params (OverlappedComponent :type Primitive%20Component%20Object%20Reference) (OtherActor :type Actor%20Object%20Reference) (OtherComp :type Primitive%20Component%20Object%20Reference) (OtherBodyIndex :type Integer) (bFromSweep :type Boolean) (SweepResult :type Hit%20Result%20Structure%20%28by%20ref%29))
  (if (Actor|ActorHasTag OtherActor "Player")
    _))

(event EventTick
  (params (DeltaSeconds :type Float%20%28single-precision%29))
  (Utilities|FlowControl|Delay 1.0)
  (bind _asbp_player_character (Utilities|Casting|CastToBP_PlayerCharacter (Game|Player|GetPlayerPawn 0)))
  (bind _newtrack_0 (Timeline|Timeline Play)
    (:Update
      (Transformation|SetWorldLocation (Variables|Default|GetCube) (Math|Vector|Lerp(Vector) (Transformation|GetWorldLocation (Variables|Default|GetCube)) (Transformation|GetActorLocation _asbp_player_character) _newtrack_0) false false)
      (Utilities|FlowControl|Delay 0.5)
      (Default|AddCoins (Variables|/Game/Player/Blueprints/BP_PlayerCharacter.BP_PlayerCharacter_C|GetBPC_Coins _asbp_player_character))
      (Actor|DestroyActor))))

(fn ConstructionScript)