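; BP_XPPickUp is an experience pickup that homes in on the player and grants XP when collected.
; On BeginPlay a timeline lerps it from its current location toward the player character, while a 0.65-second delay arms collection.
; Each Tick checks whether its sphere overlaps the player's capsule and, once armed, passes the XP amount to the player's level-up component and destroys the pickup.
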(event EventBeginPlay
  (Utilities|FlowControl|Sequence
    (:then_0
      (Utilities|FlowControl|Delay 0.65)
      (Variables|Default|SetCanGain true))
    (:then_1
      (bind _positionalpha (Timeline|Timeline PlayFromStart)
        (:Update
          (Transformation|SetActorLocation (Math|Vector|Lerp(Vector) (Transformation|GetActorLocation) (Transformation|GetActorLocation (Variables|Default|GetBP_PlayerCharacter)) _positionalpha) false false))))))

(event EventTick
  (params (DeltaSeconds :type Float%20%28single-precision%29))
  (if (Class|PrimitiveComponent|IsOverlappingComponent (Variables|Default|GetSphere) (Variables|/Script/Engine.Character|GetCapsuleComponent (Variables|Default|GetBP_PlayerCharacter)))
    (if (Variables|Default|GetCanGain)
      (Default|OnXPGainEvent (Variables|/Game/Player/Blueprints/BP_PlayerCharacter.BP_PlayerCharacter_C|GetBPC_LevelUp (Variables|Default|GetBP_PlayerCharacter)) (Variables|Default|GetxpGainAmount))
      (Actor|DestroyActor))))

(fn ConstructionScript)