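; BP_SwarmingEnemy is a dagger-wielding goblin enemy running BT_SwarmingEnemy, starting passive unless spawner-created.
; Attacks alternate two stab montages via FlipFlop, reporting attack end on completion or interruption.
; A fast looping timer capsule-traces between dagger sockets, damaging the player once per swing.
; Death decrements the player's enemy count if counted, but proximity-based counting is disconnected and the spawner-only player-search timer's StartSearchingPlayer event is empty.
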(event Custom|GoblinTriggerAttackTrace
  (bind _returnvalue (Utilities|Time|SetTimerbyEvent (delegate Custom|GoblinSwipeTraceLoop) 0.01 true))
  (Variables|Default|SetSwipeTracingTimerHandle _returnvalue))

(event Custom|GoblinSwipeTraceLoop
  (bind _dagger__skeletelmesh_ (Variables|Default|GetDagger%20%28SkeletelMesh%29))
  (bind _actorhitbytrace (Variables|Default|GetActorHitByTrace))
  (bind _outhits (Class|KismetSystemLibrary|CapsuleTraceMulti (Transformation|GetSocketLocation _dagger__skeletelmesh_ "start") (Transformation|GetSocketLocation _dagger__skeletelmesh_ "end") 12.0 0.0 "TraceTypeQuery1" false (Variables|Default|GetEnemyActors) "None" true))
  (bind _array_element (Utilities|Array|ForEachLoopwithBreak _outhits)
    (:LoopBody
      (if (not (Utilities|Array|ContainsItem _actorhitbytrace (.HitActor (Collision|BreakHitResult _array_element))))
        (Utilities|Array|Add _actorhitbytrace (.HitActor (Collision|BreakHitResult _array_element)))
        (Utilities|Casting|CastToBP_PlayerCharacter (.HitActor (Collision|BreakHitResult _array_element)))
        (Class|BPIDamagable|DealDamage(Message) (.HitActor (Collision|BreakHitResult _array_element)) (Utilities|Struct|MakeS_DamageInfo 13.0 "NewEnumerator5" "NewEnumerator1"))))))

(event Custom|GoblinStopSwipeTrace
  (Utilities|Time|ClearandInvalidateTimerbyHandle (Variables|Default|GetSwipeTracingTimerHandle))
  (Utilities|Array|Clear (Variables|Default|GetActorHitByTrace)))

(event Custom|StartSearchingPlayer
  ;[0.07812 0.07812 0.07812] Check amount of enemies
)

(event EventBeginPlay
  (bind _attackanim (Variables|Default|GetAttackAnim))
  (|CallParentFunction)
  (Variables|Default|SetBTAsset "/Game/Enemies/AI/BehaviourTrees/BT_SwarmingEnemy.BT_SwarmingEnemy")
  (Utilities|Array|Add _attackanim "/Game/Characters/Enemies/GoblinEnemy/Animations/Attacks/Stabbing_1__UE_Montage.Stabbing_1__UE_Montage")
  (Utilities|Array|Add _attackanim "/Game/Characters/Enemies/GoblinEnemy/Animations/Attacks/Stabbing_UE_Montage.Stabbing_UE_Montage")
  (Utilities|FlowControl|Delay 0.15)
  (if (Variables|Default|GetIsFromEnemySpawner)
    (bind _returnvalue (Utilities|Time|SetTimerbyEvent (EventDispatchers|CreateEvent :!event Custom|StartSearchingPlayer) 0.5 true true))
    (Variables|Default|SetSearchingPlayerTimer _returnvalue)
    (else
      (Default|SetStateasPassive (Variables|Default|GetAIController)))))

(event EventDeath
  ;[0.07812 0.07812 0.07812] Check amount of enemies
  (|CallParentFunction)
  (if (Variables|Default|GetCountedIn)
    (Math|Integer|DecrementInt (Variables|/Game/Player/Blueprints/BP_PlayerCharacter.BP_PlayerCharacter_C|GetEnemyCount (Variables|Default|GetBP_PlayerCharacter))
      (:%20%20
        (Variables|Default|SetCountedIn false)))))

(event EventAttack
  (bind _attackcount (Variables|Default|GetAttackCount))
  (Animation|Montage|PlayMontage (Variables|Character|GetMesh) (Utilities|Array|Get(acopy) (Variables|Default|GetAttackAnim) (Variables|Default|GetAttackCount)) (Variables|Default|GetAttack%20Play%20Rate)
    (:OnCompleted
      _)
    (:OnInterrupted
      _))
  (Default|CallOnAttackEnd)
  (Utilities|FlowControl|FlipFlop
    (:A
      (Math|Integer|IncrementInt _attackcount))
    (:B
      (Math|Integer|DecrementInt _attackcount))))

(fn ConstructionScript
  (|CallParentFunction))

(fn IsDead
  (bind _isdead (|CallParentFunction))
  (return _isdead))