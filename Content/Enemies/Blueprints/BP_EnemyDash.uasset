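; BP_EnemyDash is an enemy that runs a dash-variant behavior tree and damages the player by dashing through them.
; EnemyDash slows its time dilation, sets a capsule channel to overlap and plays the montage, restoring blocking and signaling completion afterward.
; AppliedDash restores normal time and starts a looping timer that polls capsule overlap, dealing randomized damage gated by CanDashDealDamage.
; The LaunchCharacter and high-gravity dash physics are disconnected.
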(event Custom|DashDealDamage
  (bind _bpc_damagesystem (Variables|Default|GetBPC_DamageSystem))
  (bind _damageamount (Variables|/Game/DamageSystem/BPC_DamageSystem.BPC_DamageSystem_C|GetDamageAmount _bpc_damagesystem))
  ;[1 1 1] Dash Physics
  (if (Class|PrimitiveComponent|IsOverlappingComponent (Variables|Default|GetCapsuleComponent) (Variables|/Script/Engine.Character|GetCapsuleComponent (Variables|Default|GetBP_PlayerCharacter)))
    (if (Variables|Default|GetCanDashDealDamage)
      (Class|BPIDamagable|DealDamage(Message) (Variables|Default|GetBP_PlayerCharacter) (Utilities|Struct|MakeS_DamageInfo (Math|Random|RandomFloatinRange _damageamount (+ _damageamount 1e+01)) "NewEnumerator5" "NewEnumerator1"))
      (Variables|Default|SetCanDashDealDamage false))))

(event Custom|Applied%20Dash
  ;[1 1 1] Dash Physics
  (Variables|Default|SetCustomTimeDilation 1.0)
  (Utilities|Time|SetTimerbyEvent (delegate Custom|DashDealDamage) 0.01 true)
  (CallFunction|DashDealDamage))

(event Custom|Enemy%20Dash
  ;[1 1 1] Dash Animation and Trigger
  (Variables|Default|SetCustomTimeDilation 0.75)
  (Collision|SetCollisionResponsetoChannel (Variables|Default|GetCapsuleComponent) "ECC_GameTraceChannel2" "ECR_Overlap")
  (Animation|Montage|PlayMontage (Variables|Character|GetMesh) (Variables|Default|GetDashAnime) 2.0
    (:OnCompleted
      _)
    (:OnInterrupted
      _))
  (Default|CallOnDashComplete)
  (Collision|SetCollisionResponsetoChannel (Variables|Default|GetCapsuleComponent) "ECC_GameTraceChannel2" "ECR_Block")
  (Variables|/Script/Engine.CharacterMovementComponent|SetGravityScale (Variables|Character|GetCharacterMovement) 2.8))

(event EventBeginPlay
  (|CallParentFunction)
  (Variables|Default|SetBTAsset "/Game/Enemies/AI/BehaviourTrees/BT_EnemyBaseDashVariant.BT_EnemyBaseDashVariant"))

(fn ConstructionScript
  (|CallParentFunction))

(fn GetMaxHealth
  (return (Variables|/Game/DamageSystem/BPC_DamageSystem.BPC_DamageSystem_C|GetmaxHealth (Variables|Default|GetBPC_DamageSystem))))

(fn GetCurrentHealth
  (return (Variables|/Game/DamageSystem/BPC_DamageSystem.BPC_DamageSystem_C|Gethealth (Variables|Default|GetBPC_DamageSystem))))