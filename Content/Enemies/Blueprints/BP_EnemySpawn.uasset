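; Enemy spawn point that creates queued enemy classes one at a time at its own transform.
; AddEnemyToQueue appends a class and calls SpawnEnemy immediately if no BP_RangedEnemyBase overlaps its Sphere.
; SpawnEnemy spawns and removes the first entry, then sets a short timer by function name to call itself again, without rechecking the overlap.
; It returns whether an enemy was available to spawn.
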(event EventBeginPlay)

(event Collision|EventActorBeginOverlap
  (params (OtherActor :type Actor%20Object%20Reference)))

(event EventTick
  (params (DeltaSeconds :type Float%20%28single-precision%29)))

(fn ConstructionScript)

(fn SpawnEnemy
  (if (Utilities|Array|IsValidIndex (Variables|Default|GetEnemyQueue))
    (Game|SpawnActorfromClass (Utilities|Array|Get(acopy) (Variables|Default|GetEnemyQueue)) (Transformation|GetActorTransform) "Undefined" "MultiplyWithRoot" 0 0)
    (Utilities|Array|RemoveIndex (Variables|Default|GetEnemyQueue))
    (Utilities|Time|SetTimerbyFunctionName 0 "SpawnEnemy" 2.0)
    (return true)
    (else
      (return false))))

(fn AddEnemytoQueue
  (params (EnemyClass :type BP%20Ranged%20Enemy%20Base%20Class%20Reference%20%28by%20ref%29))
  (Utilities|Array|Add (Variables|Default|GetEnemyQueue) EnemyClass)
  (if (not (Utilities|Array|IsValidIndex (Collision|GetOverlappingActors (Variables|Default|GetSphere) "/Game/Enemies/Blueprints/BP_RangedEnemyBase.BP_RangedEnemyBase_C" :!class /Script/Engine.PrimitiveComponent)))
    (CallFunction|SpawnEnemy)))