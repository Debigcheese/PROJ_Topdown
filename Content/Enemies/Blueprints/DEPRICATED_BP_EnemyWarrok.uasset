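; Deprecated Warrok enemy Blueprint with an animation-triggered melee swipe attack.
; While a swipe is active, a looping timer runs multi-line traces between two mesh sockets, ignoring other enemies.
; A hit list, cleared when the swipe stops, limits damage to once per swipe on the player character.
; Health getters read from the damage system component, but any incoming AnyDamage event destroys the actor outright.
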(event Custom|TriggerSwipeTrace
  (bind _returnvalue (Utilities|Time|SetTimerbyEvent (delegate Custom|SwipeTraceLoop) 0.01 true))
  (Variables|Default|SetSwipeTracingTimerHandle _returnvalue))

(event Custom|SwipeTraceLoop
  (bind _mesh (Variables|Character|GetMesh))
  (bind _actorhitbytrace (Variables|Default|GetActorHitByTrace))
  (bind _outhits (Collision|MultiLineTraceByChannel (Transformation|GetSocketLocation _mesh "start") (Transformation|GetSocketLocation _mesh "end") "TraceTypeQuery1" false (Variables|Default|GetEnemyActors) "None"))
  (bind _array_element (Utilities|Array|ForEachLoopwithBreak _outhits)
    (:LoopBody
      (if (not (Utilities|Array|ContainsItem _actorhitbytrace (.HitActor (Collision|BreakHitResult _array_element))))
        (Utilities|Array|Add _actorhitbytrace (.HitActor (Collision|BreakHitResult _array_element)))
        (Utilities|Casting|CastToBP_PlayerCharacter (.HitActor (Collision|BreakHitResult _array_element)))
        (Class|BPIDamagable|DealDamage(Message) (.HitActor (Collision|BreakHitResult _array_element)) (Utilities|Struct|MakeS_DamageInfo 2e+01 "NewEnumerator5" "NewEnumerator1"))))))

(event Custom|StopSwipeTrace
  (Utilities|Time|ClearandInvalidateTimerbyHandle (Variables|Default|GetSwipeTracingTimerHandle))
  (Utilities|Array|Clear (Variables|Default|GetActorHitByTrace)))

(event EventBeginPlay
  (|CallParentFunction)
  (Variables|Default|SetRotationOffset -25.0))

(event Game|Damage|EventAnyDamage
  (params (Damage :type Float%20%28single-precision%29) (DamageType :type Damage%20Type%20Object%20Reference) (InstigatedBy :type Controller%20Object%20Reference) (DamageCauser :type Actor%20Object%20Reference))
  (Actor|DestroyActor)
  (Default|CallOnDestroyed))

(fn ConstructionScript
  (|CallParentFunction))

(fn GetMaxHealth
  (return (Variables|/Game/DamageSystem/BPC_DamageSystem.BPC_DamageSystem_C|GetmaxHealth (Variables|Default|GetBPC_DamageSystem))))

(fn GetCurrentHealth
  (return (Variables|/Game/DamageSystem/BPC_DamageSystem.BPC_DamageSystem_C|Gethealth (Variables|Default|GetBPC_DamageSystem))))