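; Base enemy character with mouse-hover targeting and highlight, montage attacks that turn toward the player, and health and bow-stack widgets.
; BPCDamageSystem handles health and drives death, block, damage, stun and knockback events through bindings made in the construction script.
; A Melee Basic hit consumes full RangedBasic stacks to stun the enemy by pausing its behavior tree.
; Death ragdolls the mesh, drops coin and XP pickups, then destroys the actor.
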(event Custom|Knockback
  (params (Strength :type Float%20%28double-precision%29))
  (bind _returnvalue (Transformation|GetActorLocation))
  (bind _bp_playercharacter (Variables|Default|GetBP_PlayerCharacter))
  (bind _returnvalue_2 (Transformation|GetActorLocation _bp_playercharacter))
  (bind _returnvalue_3 (- _returnvalue _returnvalue_2))
  (bind _returnvalue_4 (Math|Vector|Normalize _returnvalue_3))
  (bind _returnvalue_5 (* Strength _returnvalue_4))
  ;[0.05208 0.05208 0.05208] Knockback
  (Character|LaunchCharacter self (Math|Vector|MakeVector (.x _returnvalue_5) (.y _returnvalue_5) (.z _returnvalue_5)) false false))

(event Custom|Knockup
  (params (Strength :type Float%20%28double-precision%29))
  (bind _returnvalue (Transformation|GetActorLocation))
  (bind _returnvalue_2 (/ Strength 4e+01))
  (bind _bp_playercharacter (Variables|Default|GetBP_PlayerCharacter))
  (bind _returnvalue_3 (Transformation|GetActorLocation _bp_playercharacter))
  (bind _returnvalue_4 (- _returnvalue _returnvalue_3))
  (bind _returnvalue_5 (Math|Vector|Normalize _returnvalue_4))
  ;[0.05208 0.05208 0.05208] Knockup
  (Variables|/Script/Engine.MovementComponent|SetVelocity (Variables|Character|GetCharacterMovement) "0, 0, 0")
  (Character|LaunchCharacter self (Math|Vector|MakeVector (* _returnvalue_2 (.x _returnvalue_5)) (* _returnvalue_2 (.y _returnvalue_5)) Strength) false false))

(event Custom|Stunned
  (params (Duration :type Float%20%28double-precision%29))
  (bind _aicontroller (Variables|Default|GetAIController))
  ;[0.05208 0.05208 0.05208] Called when stunned
  (AI|Logic|StopLogic (Variables|/Script/AIModule.AIController|GetBrainComponent _aicontroller) "")
  (Animation|StopAnimMontage self 0)
  (Utilities|FlowControl|Delay Duration)
  (AI|RunBehaviorTree _aicontroller (Variables|Default|GetBTAsset)))

(event Custom|Blocked
  (params (CanBeParried :type Boolean))
  ;[0.05208 0.05208 0.05208] Called when attack gets block
)

(event Custom|RotateToPlayer
  ;[0.05208 0.05208 0.05208] Called when attacking - lerp rotation towards player - change rotation duration & offset depending on enemy type
  (bind _returnvalue (Utilities|Time|SetTimerbyEvent (delegate Custom|RotateToPlayerLerp) 0.01 true))
  (Utilities|FlowControl|Delay (Variables|Default|GetRotationDuration))
  (Utilities|Time|ClearandInvalidateTimerbyHandle _returnvalue))

(event Custom|Attack
  ;[0.05208 0.05208 0.05208] Called on attack
  (CallFunction|RotatetoPlayer)
  (Animation|Montage|PlayMontage (Variables|Character|GetMesh) "/Game/Characters/Mannequins/Warrok/Animations/Mutant_Swiping_Montage.Mutant_Swiping_Montage" (Variables|Default|GetAttack%20Play%20Rate)
    (:OnCompleted
      _)
    (:OnInterrupted
      _))
  (Default|CallOnAttackEnd))

(event Custom|Death
  ;[0.05208 0.05208 0.05208] Called on death
  (Default|IsDead (Variables|Default|GetBPC_DamageSystem))
  (Physics|SetSimulatePhysics (Variables|Character|GetMesh) true)
  (Collision|SetCollisionEnabled (Variables|Collision|GetCapsuleComponent) "PhysicsOnly")
  (Collision|SetCollisionEnabled (Variables|Default|GetCapsule%20Component%20%28MouseCollision%29) "NoCollision")
  (Default|OnHitChangeMaterial (Variables|Default|GetBPC_DamageSystem))
  (Default|SetTargettedEnemy (Variables|Default|GetBPC_PlayerCombat))
  (Game|SpawnActorfromClass "/Game/Upgrades/Blueprints/BP_CoinPickUp.BP_CoinPickUp_C" (Transformation|GetActorTransform) "Undefined" "MultiplyWithRoot" 0 0)
  (Game|SpawnActorfromClass "/Game/Upgrades/Blueprints/BP_XPPickUp.BP_XPPickUp_C" (Math|Conversions|ToTransform(Vector) (Math|Transform|TransformLocation (Transformation|GetActorTransform) "35.000000,5.000000,0.000000")) "Undefined" "MultiplyWithRoot" 0 0)
  (Utilities|FlowControl|Delay 1.0)
  (Actor|DestroyActor))

(event Custom|DamageResponse
  (params (DamageResponse :type E_DamageResponse%20Enum :default "NewEnumerator0") (DamageType :type E_DamageType%20Enum :default "NewEnumerator3"))
  ;[0.05208 0.05208 0.05208] Called when damaged
  (Class|AISenseDamage|ReportDamageEvent self (Game|GetPlayerController 0) 0.0 "0, 0, 0" "0, 0, 0" "None")
  (Default|OnHitChangeMaterial (Variables|Default|GetBPC_DamageSystem))
  (if (Variables|Default|GetIsMouseHovering)
    (Utilities|ChangetoHitMaterial :!label _label)
    (Utilities|PopupDamage)
    (else
      (goto _label ChangeToNone))))

(event Custom|Stack
  (params (DamageType :type E_DamageType%20Enum :default "NewEnumerator0"))
  ;[0.05208 0.05208 0.05208] Called when damaged & checks which damagetype can proc a specific stacktype
  (switch Utilities|FlowControl|Switch|SwitchonE_DamageType DamageType
    (:NewEnumerator3
      (Utilities|CheckifFullyStackedMacro "NewEnumerator1"
        (:then
          (Default|CallOnStackFinished (Variables|Default|GetBPC_DamageSystem) DamageType)
          (CallFunction|Stunned 1.5))))))

(event Custom|RotateToPlayerLerp
  ;[0.05208 0.05208 0.05208] Called when attacking - lerp rotation towards player - change rotation duration & offset depending on enemy type
  (Transformation|SetActorRotation (Math|Rotator|MakeRotator 0.0 0.0 (.yaw (Math|Interpolation|RInterpTo (Transformation|GetActorRotation) (Math|Rotator|MakeRotator 0.0 0.0 (+ (.yaw (Math|Rotator|FindLookatRotation (Transformation|GetActorLocation) (Transformation|GetActorLocation (Variables|Default|GetBP_PlayerCharacter)))) (Variables|Default|GetRotationOffset))) (Utilities|Time|GetWorldDeltaSeconds) 7.0)))))

(event EventTick
  (params (DeltaSeconds :type Float%20%28single-precision%29))
  (Rendering|SetVisibility (Variables|Default|GetBowStack%20%28Widget%29) false false))

(event EventBeginPlay
  ;[0.05208 0.05208 0.05208] Setup
  (Utilities|CreateandSetWidgets)
  (Utilities|GetObjects))

(event MouseInput|EventActorBeginCursorOver
  ;[0.05208 0.05208 0.05208] Change material on mouse hover
  (Variables|Default|SetIsMouseHovering true)
  (if (not (Variables|/Game/DamageSystem/BPC_DamageSystem.BPC_DamageSystem_C|Getis%20Dead (Variables|Default|GetBPC_DamageSystem)))
    (Default|SetTargettedEnemy (Variables|Default|GetBPC_PlayerCombat) self)
    (if (not (Variables|Default|GetIsChangingMaterial))
      (Utilities|ChangetoHitMaterial))))

(event MouseInput|EventActorEndCursorOver
  ;[0.05208 0.05208 0.05208] Change material on mouse hover
  (Variables|Default|SetIsMouseHovering false)
  (Default|SetTargettedEnemy (Variables|Default|GetBPC_PlayerCombat))
  (if (not (Variables|Default|GetIsChangingMaterial))
    (Utilities|ChangetoHitMaterial) ; enters at ChangeToNone
  ))

(fn ConstructionScript
  (bind _bpc_damagesystem (Variables|Default|GetBPC_DamageSystem))
  (EventDispatchers|BindEventtoOnDeath _bpc_damagesystem (EventDispatchers|CreateEvent :!event Custom|Death))
  (EventDispatchers|BindEventtoOnBlocked _bpc_damagesystem (EventDispatchers|CreateEvent :!event Custom|Blocked))
  (EventDispatchers|BindEventtoOnDamageResponse _bpc_damagesystem (EventDispatchers|CreateEvent :!event Custom|DamageResponse))
  (EventDispatchers|BindEventtoOnStunned _bpc_damagesystem (EventDispatchers|CreateEvent :!event Custom|Stunned))
  (EventDispatchers|BindEventtoOnKnockback _bpc_damagesystem (EventDispatchers|CreateEvent :!event Custom|Knockback)))

(fn GetIsMouseHovering
  (return (Variables|Default|GetIsMouseHovering)))

(fn DealDamage
  (params (DamageInfo :type S%20Damage%20Info%20Structure))
  (bind _wasdamaged (Default|DealDamage (Variables|Default|GetBPC_DamageSystem) DamageInfo))
  (return _wasdamaged))

(fn GetCurrentHealth
  (return (Variables|/Game/DamageSystem/BPC_DamageSystem.BPC_DamageSystem_C|Gethealth (Variables|Default|GetBPC_DamageSystem))))

(fn GetDamage
  (return 0.0))

(fn GetMaxHealth
  (return (Variables|/Game/DamageSystem/BPC_DamageSystem.BPC_DamageSystem_C|GetmaxHealth (Variables|Default|GetBPC_DamageSystem))))

(fn GetPatrolRoute
  (return (Variables|Default|GetPatrolRoute)))

(fn Heal
  (params (Amount :type Float%20%28double-precision%29))
  (bind _new_health (Default|Heal (Variables|Default|GetBPC_DamageSystem) Amount))
  (return _new_health))

(fn IsDead
  (return (Variables|/Game/DamageSystem/BPC_DamageSystem.BPC_DamageSystem_C|Getis%20Dead (Variables|Default|GetBPC_DamageSystem))))

(fn Respawn
  (return false))

(fn SetMovementSpeed
  (params (Speed :type E_MovementSpeed%20Enum :default "NewEnumerator0"))
  (bind _output_get (Variables|/Script/Engine.CharacterMovementComponent|SetMaxWalkSpeed (Variables|Character|GetCharacterMovement) (Utilities|Select :Index Speed :NewEnumerator0 0.0 :NewEnumerator1 1.8e+02 :NewEnumerator2 3.5e+02 :NewEnumerator3 4e+02 :NewEnumerator4 1e+05)))
  (return _output_get))