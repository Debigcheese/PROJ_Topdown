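; Base enemy character that attacks, takes damage, can be stunned or launched, and ragdolls and drops XP on death.
; BPCDamageSystem owns health and drives death, damage, stun and knockback events, feeding health bar and bow-stack widgets plus damage popups.
; Cursor hover highlights the enemy and sets it as the player's combat target.
; Melee hits consume full ranged stacks to stun, which halts and restarts the AIC_EnemyBase behavior tree.
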(event Custom|Knockback
  (params (Strength :type Float%20%28double-precision%29))
  (bind _returnvalue (Transformation|GetActorLocation))
  (bind _bp_playercharacter (Variables|Components|GetBP_PlayerCharacter))
  (bind _returnvalue_2 (Transformation|GetActorLocation _bp_playercharacter))
  (bind _returnvalue_3 (- _returnvalue _returnvalue_2))
  (bind _returnvalue_4 (Math|Vector|Normalize _returnvalue_3))
  (bind _returnvalue_5 (* Strength _returnvalue_4))
  ;[0.05208 0.05208 0.05208] Knockback
  (Character|LaunchCharacter self (Math|Vector|MakeVector (.x _returnvalue_5) (.y _returnvalue_5) (.z _returnvalue_5)) false false))

(event Custom|ShowUpgrades
  ;[0.05208 0.05208 0.05208] Toggle healthbar visibility when player upgrade
  (Utilities|FlowControl|Delay 0.3)
  (Rendering|SetVisibility (Variables|Default|GetHealthBar%20%28Widget%29) false false))

(event Custom|UpgradeChosen
  (params (UpgradeChosen :type E_Upgrades%20Enum :default "NewEnumerator1"))
  ;[0.05208 0.05208 0.05208] Toggle healthbar visibility when player upgrade
  (Rendering|SetVisibility (Variables|Default|GetHealthBar%20%28Widget%29) true false))

(event Custom|Knockup
  (params (Strength :type Float%20%28double-precision%29))
  (bind _returnvalue (Transformation|GetActorLocation))
  (bind _returnvalue_2 (/ Strength 4e+01))
  (bind _bp_playercharacter (Variables|Components|GetBP_PlayerCharacter))
  (bind _returnvalue_3 (Transformation|GetActorLocation _bp_playercharacter))
  (bind _returnvalue_4 (- _returnvalue _returnvalue_3))
  (bind _returnvalue_5 (Math|Vector|Normalize _returnvalue_4))
  ;[0.05208 0.05208 0.05208] Knockup
  (Variables|/Script/Engine.MovementComponent|SetVelocity (Variables|Character|GetCharacterMovement) "0, 0, 0")
  (Character|LaunchCharacter self (Math|Vector|MakeVector (* _returnvalue_2 (.x _returnvalue_5)) (* _returnvalue_2 (.y _returnvalue_5)) Strength) false false))

(event Custom|Stunned
  (params (Duration :type Float%20%28double-precision%29))
  (bind _aicontroller (Variables|AI|GetAIController))
  (bind _braincomponent (Variables|/Script/AIModule.AIController|GetBrainComponent _aicontroller))
  ;[0.05208 0.05208 0.05208] Called when stunned
  (AI|Logic|StopLogic _braincomponent "")
  (Animation|StopAnimMontage self 0)
  (Utilities|FlowControl|Delay Duration)
  (Class|BrainComponent|RestartLogic _braincomponent)
  (AI|RunBehaviorTree _aicontroller (Variables|AI|GetBTAsset)))

(event Custom|Blocked
  (params (CanBeParried :type Boolean))
  ;[0.05208 0.05208 0.05208] Called when attack gets block
)

(event Custom|Attack
  ;[0.05208 0.05208 0.05208] Called on attack
  (Animation|Montage|PlayMontage (Variables|Character|GetMesh) "/Game/Characters/Mannequins/Warrok/Animations/Mutant_Swiping_Montage.Mutant_Swiping_Montage" (Variables|Default|GetAttack%20Play%20Rate)
    (:OnCompleted
      _)
    (:OnInterrupted
      _))
  (Default|CallOnAttackEnd))

(event Custom|Death
  (bind _mesh (Variables|Character|GetMesh))
  ;[0.05208 0.05208 0.05208] Called on death
  (Default|IsDead (Variables|Default|GetBPC_DamageSystem))
  (Physics|SetSimulatePhysics _mesh true)
  (Collision|SetCollisionEnabled _mesh "PhysicsOnly")
  (Collision|SetCollisionEnabled (Variables|Default|GetCapsule%20Component%20%28MouseCollision%29) "NoCollision")
  (Default|OnHitChangeMaterial (Variables|Default|GetBPC_DamageSystem))
  (Default|SetTargettedEnemy (Variables|Default|GetBPC_PlayerCombat))
  (Game|SpawnActorfromClass "/Game/Upgrades/Blueprints/BP_XPPickUp.BP_XPPickUp_C" (Math|Conversions|ToTransform(Vector) (Math|Transform|TransformLocation (Transformation|GetActorTransform) "35.000000,5.000000,0.000000")) "Undefined" "MultiplyWithRoot" 0 (Variables|Components|GetBP_PlayerCharacter) (Variables|Default|GetXPValue) 0)
  (Utilities|FlowControl|Delay 1.0)
  (Actor|DestroyActor))

(event Custom|DamageResponse
  (params (DamageResponse :type E_DamageResponse%20Enum :default "NewEnumerator0") (DamageType :type E_DamageType%20Enum :default "NewEnumerator3"))
  ;[0.05208 0.05208 0.05208] Called when damaged
  (Class|AISenseDamage|ReportDamageEvent self (Game|GetPlayerController 0) 0.0 "0, 0, 0" "0, 0, 0" "None")
  (Default|OnHitChangeMaterial (Variables|Default|GetBPC_DamageSystem))
  (if (Variables|Default|GetIsMouseHovering)
    (Utilities|ChangetoHitMaterial :!label _label)
    (Utilities|PopupDamage)
    (else
      (goto _label ChangeToNone))))

(event Custom|Stack
  (params (DamageType :type E_DamageType%20Enum :default "NewEnumerator0"))
  ;[0.05208 0.05208 0.05208] Called when damaged & checks which damagetype can proc a specific stacktype
  (switch Utilities|FlowControl|Switch|SwitchonE_DamageType DamageType
    (:NewEnumerator3
      (Utilities|CheckifFullyStackedMacro "NewEnumerator1"
        (:then
          (Default|CallOnStackFinished (Variables|Default|GetBPC_DamageSystem) DamageType)
          (CallFunction|Stunned 1.5))))))

(event EventBeginPlay
  (bind _bp_playercharacter (Variables|Components|GetBP_PlayerCharacter))
  (bind _bpc_upgrade (Variables|/Game/Player/Blueprints/BP_PlayerCharacter.BP_PlayerCharacter_C|GetBPC_Upgrade _bp_playercharacter))
  ;[0.05208 0.05208 0.05208] Setup
  (Utilities|CreateandSetWidgets)
  (Utilities|GetObjects)
  (EventDispatchers|BindEventtoOnShowUpgrades _bpc_upgrade (EventDispatchers|CreateEvent :!event Custom|ShowUpgrades))
  (EventDispatchers|BindEventtoOnUpgradeChosen _bpc_upgrade (EventDispatchers|CreateEvent :!event Custom|UpgradeChosen)))

(event MouseInput|EventActorBeginCursorOver
  ;[0.05208 0.05208 0.05208] Change material on mouse hover
  (Variables|Default|SetIsMouseHovering true)
  (if (not (Variables|/Game/DamageSystem/BPC_DamageSystem.BPC_DamageSystem_C|Getis%20Dead (Variables|Default|GetBPC_DamageSystem)))
    (Default|SetTargettedEnemy (Variables|Default|GetBPC_PlayerCombat) self)
    (if (not (Variables|Default|GetIsChangingMaterial))
      (Utilities|ChangetoHitMaterial))))

(event MouseInput|EventActorEndCursorOver
  ;[0.05208 0.05208 0.05208] Change material on mouse hover
  (Variables|Default|SetIsMouseHovering false)
  (Default|SetTargettedEnemy (Variables|Default|GetBPC_PlayerCombat))
  (if (not (Variables|Default|GetIsChangingMaterial))
    (Utilities|ChangetoHitMaterial) ; enters at ChangeToNone
  ))

(fn ConstructionScript
  (bind _bpc_damagesystem (Variables|Default|GetBPC_DamageSystem))
  (EventDispatchers|BindEventtoOnDeath _bpc_damagesystem (EventDispatchers|CreateEvent :!event Custom|Death))
  (EventDispatchers|BindEventtoOnBlocked _bpc_damagesystem (EventDispatchers|CreateEvent :!event Custom|Blocked))
  (EventDispatchers|BindEventtoOnDamageResponse _bpc_damagesystem (EventDispatchers|CreateEvent :!event Custom|DamageResponse))
  (EventDispatchers|BindEventtoOnStunned _bpc_damagesystem (EventDispatchers|CreateEvent :!event Custom|Stunned))
  (EventDispatchers|BindEventtoOnKnockback _bpc_damagesystem (EventDispatchers|CreateEvent :!event Custom|Knockback)))

(fn GetIsMouseHovering
  (return (Variables|Default|GetIsMouseHovering)))

(fn DealDamage
  (params (DamageInfo :type S%20Damage%20Info%20Structure))
  (bind _wasdamaged (Default|DealDamage (Variables|Default|GetBPC_DamageSystem) DamageInfo))
  (return _wasdamaged))

(fn GetCurrentHealth
  (return (Variables|/Game/DamageSystem/BPC_DamageSystem.BPC_DamageSystem_C|Gethealth (Variables|Default|GetBPC_DamageSystem))))

(fn GetDamage
  (return 0.0))

(fn GetMaxHealth
  (return (Variables|/Game/DamageSystem/BPC_DamageSystem.BPC_DamageSystem_C|GetmaxHealth (Variables|Default|GetBPC_DamageSystem))))

(fn GetPatrolRoute
  (return (Variables|Default|GetPatrolRoute)))

(fn Heal
  (params (Amount :type Float%20%28double-precision%29))
  (bind _new_health (Default|Heal (Variables|Default|GetBPC_DamageSystem) Amount))
  (return _new_health))

(fn IsDead
  (return (Variables|/Game/DamageSystem/BPC_DamageSystem.BPC_DamageSystem_C|Getis%20Dead (Variables|Default|GetBPC_DamageSystem))))

(fn Respawn
  (return false))

(fn SetMovementSpeed
  (params (Speed :type E_MovementSpeed%20Enum :default "NewEnumerator0"))
  (bind _output_get (Variables|/Script/Engine.CharacterMovementComponent|SetMaxWalkSpeed (Variables|Character|GetCharacterMovement) (Utilities|Select :Index Speed :NewEnumerator0 0.0 :NewEnumerator1 1.8e+02 :NewEnumerator2 3.5e+02 :NewEnumerator3 4e+02 :NewEnumerator6 5.5e+02 :NewEnumerator5 7e+02 :NewEnumerator7 1e+03 :NewEnumerator4 1e+05)))
  (return _output_get))