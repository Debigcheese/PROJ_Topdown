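; Wave-based enemy spawner that closes a door when the player enters its trigger and moves an exit door after the last wave.
; Each wave randomly fills an enemy queue from its class-to-amount map, then spawns enemies at random positions clear of player and enemies, retrying by timer.
; Spawned enemies enter combat, and their deaths update the player's HUD and start the next wave.
; Key 7 forces the ending; the spawner reset is marked broken.
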(event OnComponentBeginOverlap(TriggerSpawnerCollider)
  (params (OverlappedComponent :type Primitive%20Component%20Object%20Reference) (OtherActor :type Actor%20Object%20Reference) (OtherComp :type Primitive%20Component%20Object%20Reference) (OtherBodyIndex :type Integer) (bFromSweep :type Boolean) (SweepResult :type Hit%20Result%20Structure%20%28by%20ref%29))
  (bind _doortocloseonstart (Variables|Default|GetDoorToCloseOnStart))
  (bind _relativelocation (Variables|/Script/Engine.SceneComponent|GetRelativeLocation _doortocloseonstart))
  ;[0.08333 0.08333 0.08333] Trigger start wave
  (if (not (Variables|Default|GetSpawnerActivated))
    (if (== OtherActor (Variables|Components|GetBP_PlayerCharacter))
      (Rendering|SetVisibility (Variables|/Game/Player/Blueprints/BP_PlayerCharacter.BP_PlayerCharacter_C|GetEnemySpawner%20%28Widget%29 (Variables|Components|GetBP_PlayerCharacter)) true false)
      (CallFunction|StartNextWave)
      (Variables|Default|SetSpawnerActivated true)
      (Audio|PlaySound2D "/Game/Audio/door-closing.door-closing" 1.0 1.0 0.0 0 0)
      (bind _newtrack_1 (Timeline|Timeline_0 Play)
        (:Update
          (Transformation|SetRelativeLocation _doortocloseonstart (Math|Vector|MakeVector (.x _relativelocation) (.y _relativelocation) (Math|Float|Lerp (.z _relativelocation) (Variables|DoorPosition|GetDoorStartLerpToPositionZ) _newtrack_1)) false false))))))

(event Custom|QueueEnemies
  ;[0.08333 0.08333 0.08333] Queue Enemies
  ;;[0.08333 0.08333 0.08333] Sets S_CurrentWaveInfo to the current wave index
  (for (_array_element _array_index) (Variables|Waves|GetS_WaveInfo)
    (if (== _array_index (- (Variables|Waves|GetCurrentWave) 1))
      (Variables|Waves|SetS_CurrentWaveInfo _array_element)
      (CallFunction|SetTotalEnemiesforCurrentWave)
      (CallFunction|FillEnemyQueueforCurrentWave)
      (CallFunction|SpawnEnemies)
      (Utilities|FlowControl|Delay 1e-05)
      (Default|CallOnUpdateEnemiesLeft (Variables|Components|GetBP_PlayerCharacter) (Variables|EnemyQueue|GetEnemiesLeft)))))

(event Custom|SpawnEnemies
  (bind _currentspawnposition (Variables|SpawnPosition|GetCurrentSpawnPosition))
  ;[0.08333 0.08333 0.08333] Spawn Enemies
  (Utilities|FlowControl|Delay (Variables|EnemyQueue|GetEnemySpawnDelay))
  (bind _returnvalue (Utilities|Time|SetTimerbyEvent (delegate Custom|SpawnEnemies) (Variables|EnemyQueue|GetEnemySpawnDelay) true))
  (bind _spawnposavailable (SpawnPosition|SpawnPositionHandler))
  (if _spawnposavailable
    (Utilities|Time|ClearandInvalidateTimerbyHandle _returnvalue)
    (if (Utilities|Array|IsNotEmpty (Variables|EnemyQueue|GetEnemyQueue))
      (Niagara|SpawnSystematLocation "/Game/VFX/NS/NS_EnemySpawn.NS_EnemySpawn" (Variables|SpawnPosition|GetCurrentSpawnPosition))
      ;;[0.08333 0.08333 0.08333] Spawns index 0 from enemy queue & sets transform
      (Utilities|FlowControl|Delay 0.5)
      (bind _returnvalue_2 (Game|SpawnActorfromClass (Utilities|Array|Get(acopy) (Variables|EnemyQueue|GetEnemyQueue)) (Math|Transform|MakeTransform _currentspawnposition (Math|Rotator|FindLookatRotation _currentspawnposition (Transformation|GetActorLocation (Variables|Components|GetBP_PlayerCharacter))) "1.000000,1.000000,1.000000") "AlwaysSpawn" "MultiplyWithRoot" 0 false 0))
      ;;[0.08333 0.08333 0.08333] bind enemies OnDeath event to call UpdateEnemyCount function
      (EventDispatchers|BindEventtoOnDeath (Variables|/Game/Enemies/Blueprints/BP_EnemyBase.BP_EnemyBase_C|GetBPC_DamageSystem _returnvalue_2) (EventDispatchers|CreateEvent :!event Custom|UpdateEnemyCount))
      ;;[0.08333 0.08333 0.08333] Update spawn POS & removes spawned enemy from index 0 in queue
      (Variables|SpawnPosition|SetPreviousSpawnPosition (Variables|SpawnPosition|GetCurrentSpawnPosition))
      (Utilities|Array|RemoveIndex (Variables|EnemyQueue|GetEnemyQueue))
      (CallFunction|SpawnEnemies)
      (Variables|/Game/Enemies/Blueprints/BP_EnemyBase.BP_EnemyBase_C|SetIsFromEnemySpawner _returnvalue_2 true)
      ;[0.08333 0.08333 0.08333] Set enemy to combat state
      (Utilities|FlowControl|Delay 0.1)
      (Default|SetStateasCombat (Variables|/Game/Enemies/Blueprints/BP_EnemyBase.BP_EnemyBase_C|GetAIController _returnvalue_2) (Variables|/Game/Enemies/Blueprints/BP_EnemyBase.BP_EnemyBase_C|GetBP_PlayerCharacter _returnvalue_2)))))

(event Custom|ResetSpawner
  (bind _doortounlockonfinish (Variables|Default|GetDoorToUnlockOnFinish))
  (bind _doortocloseonstart (Variables|Default|GetDoorToCloseOnStart))
  (bind _relativelocation (Variables|/Script/Engine.SceneComponent|GetRelativeLocation _doortounlockonfinish))
  (bind _relativelocation_2 (Variables|/Script/Engine.SceneComponent|GetRelativeLocation _doortocloseonstart))
  ;[0.08333 0.08333 0.08333] Reset Spawner on player death (doesnt work)
  (Variables|Default|SetSpawnerActivated false)
  (Variables|Waves|SetS_WaveInfo (Variables|Waves|GetS_DefaultWaveInfo))
  (Utilities|Array|Clear (Variables|EnemyQueue|GetEnemyQueue))
  (Transformation|SetRelativeLocation _doortocloseonstart (Math|Vector|MakeVector (.x _relativelocation_2) (.y _relativelocation_2) (+ (.z _relativelocation_2) -5e+02)) false false)
  (Transformation|SetRelativeLocation _doortounlockonfinish (Math|Vector|MakeVector (.x _relativelocation) (.y _relativelocation) (- (.z _relativelocation) (Variables|DoorPosition|GetDoorFinishLerpToPositionZ))) false false)
  (Development|PrintString "reset spawner"))

(event Custom|StartNextWave
  (bind _currentwave (Variables|Waves|GetCurrentWave))
  (bind _bp_playercharacter (Variables|Components|GetBP_PlayerCharacter))
  ;[0.08333 0.08333 0.08333] Starts next wave if available
  (bind _result (Math|Integer|IncrementInt (Variables|Waves|GetCurrentWave))
    (:%20%20
      (if (<= _result (Variables|Waves|GetTotalWaves))
        (CallFunction|QueueEnemies)
        (Utilities|FlowControl|Delay 1e-05)
        (Default|CallOnUpdateWaveAmount _bp_playercharacter _currentwave)
        (else
          (CallFunction|EndSpawner)
          (Default|CallOnUpdateWaveAmount _bp_playercharacter _currentwave))))))

(event Custom|EndSpawner
  (bind _doortounlockonfinish (Variables|Default|GetDoorToUnlockOnFinish))
  (bind _relativelocation (Variables|/Script/Engine.SceneComponent|GetRelativeLocation _doortounlockonfinish))
  ;[0.08333 0.08333 0.08333] Called when CurrentWave > TotalWaves
  (Development|PrintString "EndSpawner")
  (Rendering|SetVisibility (Variables|/Game/Player/Blueprints/BP_PlayerCharacter.BP_PlayerCharacter_C|GetEnemySpawner%20%28Widget%29 (Variables|Components|GetBP_PlayerCharacter)) false false)
  (Audio|PlaySound2D "/Game/Audio/door-closing.door-closing" 1.0 1.0 0.0 0 0)
  (bind _newtrack_1 (Timeline|Timeline PlayFromStart)
    (:Update
      (Transformation|SetRelativeLocation _doortounlockonfinish (Math|Vector|MakeVector (.x _relativelocation) (.y _relativelocation) (Math|Float|Lerp (.z _relativelocation) (Variables|DoorPosition|GetDoorFinishLerpToPositionZ) _newtrack_1)) false false))))

(event Custom|UpdateEnemyCount
  (bind _enemiesleft (Variables|EnemyQueue|GetEnemiesLeft))
  ;[0.08333 0.08333 0.08333] Called when a spawned enemy dies, updates EnemiesLeft or starts next wave if all enemies are dead
  (if (> _enemiesleft 1)
    (Math|Integer|DecrementInt _enemiesleft
      (:%20%20
        (Default|CallOnUpdateEnemiesLeft (Variables|Components|GetBP_PlayerCharacter) (Variables|EnemyQueue|GetEnemiesLeft))))
    (else
      (CallFunction|StartNextWave))))

(event EventBeginPlay
  (bind _doortocloseonstart (Variables|Default|GetDoorToCloseOnStart))
  (bind _relativelocation (Variables|/Script/Engine.SceneComponent|GetRelativeLocation _doortocloseonstart))
  ;[0.08333 0.08333 0.08333] Setup
  (bind _returnvalue (Actor|GetActorOfClass "/Game/Player/Blueprints/BP_PlayerCharacter.BP_PlayerCharacter_C"))
  (Variables|Components|SetBP_PlayerCharacter _returnvalue)
  (|BindEvents)
  (Rendering|SetVisibility (Variables|/Game/Player/Blueprints/BP_PlayerCharacter.BP_PlayerCharacter_C|GetEnemySpawner%20%28Widget%29 (Variables|Components|GetBP_PlayerCharacter)) false false)
  (bind _output_get (Variables|SpawnPosition|SetCurrentSpawnPosition (.OutItem (Utilities|Array|Random (Variables|SpawnPosition|GetAllSpawnPositions)))))
  (Variables|SpawnPosition|SetPreviousSpawnPosition _output_get)
  (for _array_element (Variables|Waves|GetS_WaveInfo)
    (Math|Integer|IncrementInt (Variables|Waves|GetTotalWaves)))
  (Transformation|SetRelativeLocation _doortocloseonstart (Math|Vector|MakeVector (.x _relativelocation) (.y _relativelocation) (+ (.z _relativelocation) -5e+02)) false false)
  (Variables|Waves|SetS_DefaultWaveInfo (Variables|Waves|GetS_WaveInfo)))

(event Input|KeyboardEvents|7
  (params (Key :type Key%20Structure :default "None"))
  (bind _doortounlockonfinish (Variables|Default|GetDoorToUnlockOnFinish))
  (bind _relativelocation (Variables|/Script/Engine.SceneComponent|GetRelativeLocation _doortounlockonfinish))
  ;[0.08333 0.08333 0.08333] Called when CurrentWave > TotalWaves
  (:Pressed
    (Development|PrintString "EndSpawner")
    (Rendering|SetVisibility (Variables|/Game/Player/Blueprints/BP_PlayerCharacter.BP_PlayerCharacter_C|GetEnemySpawner%20%28Widget%29 (Variables|Components|GetBP_PlayerCharacter)) false false)
    (Audio|PlaySound2D "/Game/Audio/door-closing.door-closing" 1.0 1.0 0.0 0 0)
    (bind _newtrack_1 (Timeline|Timeline PlayFromStart)
      (:Update
        (Transformation|SetRelativeLocation _doortounlockonfinish (Math|Vector|MakeVector (.x _relativelocation) (.y _relativelocation) (Math|Float|Lerp (.z _relativelocation) (Variables|DoorPosition|GetDoorFinishLerpToPositionZ) _newtrack_1)) false false)))))

(fn ConstructionScript)

(fn SetTotalEnemiesforCurrentWave
  ;[0.08333 0.08333 0.08333] Count total enemies for specific wave
  (Variables|EnemyQueue|SetTotalEnemies 0)
  (Variables|EnemyQueue|SetEnemiesLeft 0)
  (bind _values (Utilities|Map|Values (Utilities|Struct|BreakS_WaveInfo (Variables|Waves|GetS_CurrentWaveInfo))))
  (for _array_element _values
    (Variables|EnemyQueue|SetTotalEnemies (+ _array_element (Variables|EnemyQueue|GetTotalEnemies))))
  (Variables|EnemyQueue|SetEnemiesLeft (Variables|EnemyQueue|GetTotalEnemies)))

(fn FillEnemyQueueforCurrentWave
  (bind _randomenemyclass (Variables|EnemyQueue|GetRandomEnemyClass))
  ;[0.08333 0.08333 0.08333] Gets random enemies from the EnemyAmount map
  (for _index (range 1 (Variables|EnemyQueue|GetTotalEnemies))
    (bind _isenemyfound (CallFunction|SearchforRandomEnemy))
    (if _isenemyfound
      ;[0.08333 0.08333 0.08333] Adds the random enemy to queue
      (Utilities|Array|Add (Variables|EnemyQueue|GetEnemyQueue) (Variables|EnemyQueue|GetRandomEnemyClass))
      ;[0.08333 0.08333 0.08333] decrement int on the random EnemyAmount
      (Utilities|Map|Add (Utilities|Struct|BreakS_WaveInfo (Variables|Waves|GetS_CurrentWaveInfo)) _randomenemyclass (- (.Value (Utilities|Map|Find (Utilities|Struct|BreakS_WaveInfo (Variables|Waves|GetS_CurrentWaveInfo)) _randomenemyclass)) 1))
      (Variables|Waves|SetS_CurrentWaveInfo (Utilities|Struct|MakeS_WaveInfo (Utilities|Struct|BreakS_WaveInfo (Variables|Waves|GetS_CurrentWaveInfo))))
      (Development|PrintString (Utilities|String|ToString(Integer) (- (.Value (Utilities|Map|Find (Utilities|Struct|BreakS_WaveInfo (Variables|Waves|GetS_CurrentWaveInfo)) _randomenemyclass)) 1))))))

(fn SpawnPositionHandler
  (bind _allspawnpositions (Variables|SpawnPosition|GetAllSpawnPositions))
  (bind _allspawnpositions_2 (Variables|SpawnPosition|GetAllSpawnPositions))
  ;[0.08333 0.08333 0.08333] Set CurrentSpawnPosition to Random position if array is not empty or not equal to the previous spawn position
  (if (Utilities|Array|IsNotEmpty _allspawnpositions)
    (bind _output_get (Variables|SpawnPosition|SetCurrentSpawnPosition (.OutItem (Utilities|Array|Random _allspawnpositions))))
    ;[0.08333 0.08333 0.08333] if overlapping is true = try finding available spawnpos by iterating through all spawnpositions, else set current spawnposition and return true
    (bind _isoverlapping (SpawnPosition|CheckPOSOverlappingPlayer _output_get))
    (bind (_isoverlapping_2 _currentspawnposition) (SpawnPosition|CheckPOSOverlappingEnemy _output_get))
    (if (or _isoverlapping_2 _isoverlapping)
      ;[0.08333 0.08333 0.08333] tries finding available spawnpos by iterating through all spawnpositions, if all spawn positions are overlapping with enemies, return false
      (bind _index (Utilities|FlowControl|ForLoopwithBreak 0 (- (Utilities|Array|Length _allspawnpositions_2) 1))
        (:LoopBody
          (bind _output_get_2 (Variables|SpawnPosition|SetCurrentSpawnPosition (Utilities|Array|Get(acopy) _allspawnpositions_2 _index)))
          (bind _isoverlapping_3 (SpawnPosition|CheckPOSOverlappingPlayer _output_get_2))
          (bind (_isoverlapping_4 _currentspawnposition_2) (SpawnPosition|CheckPOSOverlappingEnemy _output_get_2))
          (if (not (or _isoverlapping_4 _isoverlapping_3))
            (Variables|SpawnPosition|SetCurrentSpawnPosition _currentspawnposition_2)
            (return true)))
        (:Completed
          (return false)))
      (else
        (Variables|SpawnPosition|SetCurrentSpawnPosition _currentspawnposition)
        (return true)))
    (else
      (Development|PrintString "add spawn locations in the EnemySpawner SpawnPositions array"))))

(fn CheckPOSOverlappingEnemy
  (params (SpawnPosition :type Vector))
  ;[0.08333 0.08333 0.08333] Check if overlapping with an enemy
  (bind _output_get (Variables|SpawnPosition|SetCurrentSpawnPosition SpawnPosition))
  (bind _returnvalue (Collision|SphereOverlapActors (+ (Transformation|GetActorLocation) _output_get) 9e+01 (Utilities|Array|MakeArray "ObjectTypeQuery3") "/Game/Enemies/Blueprints/BP_EnemyBase.BP_EnemyBase_C"))
  (return _returnvalue (+ (Transformation|GetActorLocation) _output_get)))

(fn CheckPOSOverlappingPlayer
  (params (SpawnPosition :type Vector))
  ;[0.08333 0.08333 0.08333] Check if overlapping with an enemy
  (bind _output_get (Variables|SpawnPosition|SetCurrentSpawnPosition SpawnPosition))
  (bind _returnvalue (Collision|SphereOverlapActors (+ (Transformation|GetActorLocation) _output_get) 475.0 (Utilities|Array|MakeArray "ObjectTypeQuery8") "/Game/Player/Blueprints/BP_PlayerCharacter.BP_PlayerCharacter_C"))
  (return _returnvalue (+ (Transformation|GetActorLocation) _output_get)))

(fn SearchforRandomEnemy
  (bind _s_currentwaveinfo (Variables|Waves|GetS_CurrentWaveInfo))
  (bind _enemyamount (Utilities|Struct|BreakS_WaveInfo _s_currentwaveinfo))
  ;[0.08333 0.08333 0.08333] queues random enemy if available
  (bind _keys (Utilities|Map|Keys _enemyamount))
  (bind _output_get (Variables|EnemyQueue|SetRandomEnemyClass (.OutItem (Utilities|Array|Random _keys))))
  (if (.ReturnValue (Utilities|Map|Find _enemyamount _output_get))
    (return true)
    (else
      (Development|PrintString "How is this even possible? " true true "(R=1.000000,G=0.019892,B=0.000000,A=1.000000)" 2e+01))))

(fn DealDamage
  (params (DamageInfo :type S%20Damage%20Info%20Structure))
  (return false))

(fn GetCurrentHealth
  (return 0.0))

(fn GetDamage
  (return 0.0))

(fn GetMaxHealth
  (return 0.0))

(fn Heal
  (params (Amount :type Float%20%28double-precision%29))
  (return 0.0))

(fn IsDead
  (return false))

(fn Respawn
  (return false))