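; Damage component that tracks an actor's health, invincibility, blocking, death and per-damage-type stacks.
; DealDamage gates hits through macros, then fires death or blocked dispatchers, or, for interruptible or forced hits, stack and response dispatchers.
; Stacks cap per type, and a retriggerable delay signals when Bow stacks finish.
; It also has helpers to gather and override skeletal mesh materials, while Heal and health getters are placeholder stubs.
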(event Custom|Stack
  (params (DamageType :type E_DamageType%20Enum :default "NewEnumerator0"))
  ;[0.06771 0.06771 0.06771] Removes stacks after x duration, the timer resets when hit by the same stacktype again
  (switch Utilities|FlowControl|Switch|SwitchonE_DamageType DamageType
    (:NewEnumerator1
      (bind _output_get (Variables|Stacks|SetSavedStackType "NewEnumerator1"))
      (Utilities|FlowControl|RetriggerableDelay 5.0)
      (Default|CallOnStackFinished _output_get))))

(event Custom|SetAllMaterial
  (params (Materials :type Material%20Interface%20Object%20Reference) (OverlayMaterial :type Material%20Interface%20Object%20Reference))
  ;[0.06771 0.06771 0.06771] On-hit set material on actor to chosen material (called when actor takes damage)
  (for _array_element (Variables|OnHit|GetskeletalMeshes)
    (Rendering|Material|SetOverlayMaterial _array_element OverlayMaterial :!class /Script/Engine.MeshComponent)
    (for (_ _array_index) (Variables|OnHit|GetMaterials)
      (Rendering|Material|SetMaterial _array_element _array_index Materials))))

(event EventBeginPlay
  ;[0.06771 0.06771 0.06771] Setup
  (Variables|Default|Sethealth (Variables|Default|GetmaxHealth))
  (EventDispatchers|BindEventtoOnStack (EventDispatchers|CreateEvent :!event Custom|Stack)))

(fn GetAllMaterialsandMeshes
  (params (Actor :type Actor%20Object%20Reference))
  (for _array_element (Actor|GetComponentsByClass Actor "/Script/Engine.SkeletalMeshComponent")
    (Utilities|Array|Add (Variables|OnHit|GetskeletalMeshes) _array_element)
    (for _array_element_2 (Rendering|Material|GetMaterials _array_element)
      (Utilities|Array|Add (Variables|OnHit|GetMaterials) _array_element_2))))

(fn DealDamage
  (params (DamageInfo :type S%20Damage%20Info%20Structure))
  (bind (_damageamount _damagetype _damagesource _damageresponse _stacktype _stunduration _shoulddamageinvincible _canbeblocked _canbeparried _shouldforceinterrupt) (Utilities|Struct|BreakS_DamageInfo DamageInfo))
  (Utilities|CanbeDamagedMacro _shoulddamageinvincible _canbeblocked
    (:DoDamage
      (Utilities|ApplyDamageMacro _damageamount
        (:IsDead
          (Variables|Default|Setis%20Dead true)
          (Default|CallOnDeath)
          (return true))
        (:IsAlive
          (if (or (Variables|Default|GetisInterruptible) _shouldforceinterrupt)
            (Utilities|StacksHandlerMacro _damagetype)
            (Default|CallOnStack _damagetype)
            (Default|CallOnDamageResponse _damageresponse _damagetype)
            (switch Utilities|FlowControl|Switch|SwitchonE_DamageResponse _damageresponse
              (:NewEnumerator0
                (return true))
              (:NewEnumerator1
                (return true))
              (:NewEnumerator4
                (return true))
              (:NewEnumerator3
                (Default|CallOnStunned _stunduration)))))))
    (:BlockDamage
      (Variables|Default|SetDamageAmount 0.0)
      (Default|CallOnBlocked _canbeparried)
      (return false))
    (:NoDamage
      (Variables|Default|SetDamageAmount 0.0)
      (return false))))

(fn GetCurrentHealth
  (return 0.0))

(fn GetDamage
  (return (Variables|Default|GetDamageAmount)))

(fn GetMaxHealth
  (return 0.0))

(fn Heal
  (params (Amount :type Float%20%28double-precision%29))
  (return 0.0))

(fn IsDead
  (return true))