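; BP_LoadNextLevel is a trigger volume that moves the player to another level when they overlap its box.
; It caches the BP_PlayerCharacter on begin play and, on the first overlap by an actor tagged Player, starts that player's black screen transition widget.
; After waiting for the transition's calculated duration plus a short buffer, it opens the level named in LevelNameToLoad.
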(event OnComponentBeginOverlap(Box)
  (params (OverlappedComponent :type Primitive%20Component%20Object%20Reference) (OtherActor :type Actor%20Object%20Reference) (OtherComp :type Primitive%20Component%20Object%20Reference) (OtherBodyIndex :type Integer) (bFromSweep :type Boolean) (SweepResult :type Hit%20Result%20Structure%20%28by%20ref%29))
  (if (Actor|ActorHasTag OtherActor "Player")
    (if (not (Variables|Default|GetOnCooldown))
      (Variables|Default|SetOnCooldown true)
      (Default|StartTransition (Variables|/Game/Player/Blueprints/BP_PlayerCharacter.BP_PlayerCharacter_C|GetWP_BlackScreenTransition (Variables|Default|GetBP_Player)) 1.75 2.0 0.0 false)
      (Utilities|FlowControl|Delay (+ (Variables|/Game/UI/WP_BlackScreenTransition.WP_BlackScreenTransition_C|GetCalculatedDuration (Variables|/Game/Player/Blueprints/BP_PlayerCharacter.BP_PlayerCharacter_C|GetWP_BlackScreenTransition (Variables|Default|GetBP_Player))) 0.5))
      (Game|OpenLevel(byName) (Utilities|String|StringToName (Variables|Default|GetLevelNameToLoad))))))

(event EventBeginPlay
  (bind _returnvalue (Actor|GetActorOfClass "/Game/Player/Blueprints/BP_PlayerCharacter.BP_PlayerCharacter_C"))
  (Variables|Default|SetBP_Player _returnvalue))

(fn ConstructionScript)