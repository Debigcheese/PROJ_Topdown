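; BP_RespawnPosition is a checkpoint trigger that updates where the player character respawns.
; It caches the BP_PlayerCharacter found in the level on BeginPlay.
; When that character overlaps the Box, it passes the RespawnPosition component's world location to the character through CallOnChangeRespawnPosition and prints a debug string.
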(event OnComponentBeginOverlap(Box)
  (params (OverlappedComponent :type Primitive%20Component%20Object%20Reference) (OtherActor :type Actor%20Object%20Reference) (OtherComp :type Primitive%20Component%20Object%20Reference) (OtherBodyIndex :type Integer) (bFromSweep :type Boolean) (SweepResult :type Hit%20Result%20Structure%20%28by%20ref%29))
  (if (== OtherActor (Variables|Default|GetBP_PlayerCharacter))
    (Default|CallOnChangeRespawnPosition (Variables|Default|GetBP_PlayerCharacter) (Transformation|GetWorldLocation (Variables|Default|GetRespawnPosition)))
    (Development|PrintString "ChangeRespawnPosition")))

(event EventBeginPlay
  (bind _returnvalue (Actor|GetActorOfClass "/Game/Player/Blueprints/BP_PlayerCharacter.BP_PlayerCharacter_C"))
  (Variables|Default|SetBP_PlayerCharacter _returnvalue))

(event Collision|EventActorBeginOverlap
  (params (OtherActor :type Actor%20Object%20Reference)))

(event EventTick
  (params (DeltaSeconds :type Float%20%28single-precision%29)))

(fn ConstructionScript)