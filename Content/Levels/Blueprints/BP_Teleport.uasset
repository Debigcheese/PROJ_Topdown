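; BP_Teleport is a level trigger actor that moves the player character to its TeleportTo location on overlap.
; It starts the transition widget held by BP_PlayerCharacter, waits out the widget's duration, then sets the player's location, optionally disabling input during the wait.
; An OnCooldown flag blocks retriggering until a second delay, slightly longer than the transition, ends after the move.
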(event EventBeginPlay
  (bind _returnvalue (Actor|GetActorOfClass "/Game/Player/Blueprints/BP_PlayerCharacter.BP_PlayerCharacter_C"))
  (Variables|Default|SetBP_Player _returnvalue))

(event Collision|EventActorBeginOverlap
  (params (OtherActor :type Actor%20Object%20Reference))
  (if (== OtherActor (Variables|Default|GetBP_Player))
    (if (not (Variables|Default|GetOnCooldown))
      (Variables|Default|SetOnCooldown true)
      (bind _aswp_teleport_transition (Utilities|Casting|CastToWP_TeleportTransition (UserInterface|GetUserWidgetObject (Variables|/Game/Player/Blueprints/BP_PlayerCharacter.BP_PlayerCharacter_C|GetTransition%20%28Widget%29 (Variables|Default|GetBP_Player)))))
      (bind _output_get (Variables|Default|SetWP_TeleportTransition _aswp_teleport_transition))
      (Default|StartTransition _output_get)
      (if (Variables|Default|GetDisableInputOnTp)
        (Input|DisableInput (Variables|Default|GetBP_Player) 0))
      (Utilities|FlowControl|Delay (Variables|/Game/UI/WP_TeleportTransition.WP_TeleportTransition_C|GetDuration (Variables|Default|GetWP_TeleportTransition)))
      (if (Variables|Default|GetDisableInputOnTp)
        (Input|EnableInput (Variables|Default|GetBP_Player) 0))
      (Transformation|SetActorLocation (Variables|Default|GetBP_Player) (Transformation|GetWorldLocation (Variables|Default|GetTeleportTo)) false false)
      ;[0.0625 0.0625 0.0625] Cooldown
      (Utilities|FlowControl|Delay (+ (Variables|/Game/UI/WP_TeleportTransition.WP_TeleportTransition_C|GetDuration (Variables|Default|GetWP_TeleportTransition)) 1.0))
      (Variables|Default|SetOnCooldown false))))

(event EventTick
  (params (DeltaSeconds :type Float%20%28single-precision%29)))

(fn ConstructionScript)