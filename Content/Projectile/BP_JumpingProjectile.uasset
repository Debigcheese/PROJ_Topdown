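; Homing projectile that launches with an upward hop, then steers toward its target and deals damage on impact.
; A looping timer re-aims the ProjectileMovement velocity at the target, scaling only X and Y by Speed.
; UpwardsMomentum boosts Z on the first valid aim and is then zeroed, leaving Z as the unscaled direction component.
; Impact sends the damage message to the hit actor, clears the timer and destroys the projectile.
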(event Custom|RotateToTarget
  (bind _speed (Variables|Default|GetSpeed))
  (bind _returnvalue (Utilities|Time|SetTimerbyEvent (delegate Custom|RotateToTarget) 0.5 true))
  (Variables|Default|SetTimerHandle _returnvalue)
  (bind _target (Variables|Default|GetTarget)
    (:then
      (Variables|/Script/Engine.MovementComponent|SetVelocity (Variables|Default|GetProjectileMovement) (Math|Vector|MakeVector (* (.x (Math|Vector|GetUnitDirection(Vector) (Transformation|GetActorLocation) (Transformation|GetActorLocation _target))) _speed) (* (.y (Math|Vector|GetUnitDirection(Vector) (Transformation|GetActorLocation) (Transformation|GetActorLocation _target))) _speed) (+ (Variables|Default|GetUpwardsMomentum) (.z (Math|Vector|GetUnitDirection(Vector) (Transformation|GetActorLocation) (Transformation|GetActorLocation _target))))))
      (if (!= (Variables|Default|GetUpwardsMomentum) 0.0)
        (Variables|Default|SetUpwardsMomentum 0.0)))
    (:else)))

(event Custom|ProjectileImpact
  (params (Other%20Actor :type Actor%20Object%20Reference) (Hit :type Hit%20Result%20Structure) (SDamageInfo :type S%20Damage%20Info%20Structure))
  (Class|BPIDamagable|DealDamage(Message) Other%20Actor SDamageInfo)
  (Utilities|Time|ClearandInvalidateTimerbyHandle (Variables|Default|GetTimerHandle))
  (Actor|DestroyActor))

(event EventBeginPlay
  (|CallParentFunction)
  (Default|CallOnRotatetoTarget))

(event Collision|EventActorBeginOverlap
  (params (OtherActor :type Actor%20Object%20Reference))
  (|CallParentFunction OtherActor) ; This node is disabled and will not be called.\nDrag off pins to build functionality.
)

(fn ConstructionScript
  (bind _self self)
  (|CallParentFunction)
  (Variables|Default|SetSpeed (Variables|Default|GetSpeed))
  (EventDispatchers|BindEventtoOnRotatetoTarget _self (EventDispatchers|CreateEvent :!event Custom|RotateToTarget))
  (EventDispatchers|BindEventtoOnProjectileImpact _self (EventDispatchers|CreateEvent :!event Custom|ProjectileImpact)))