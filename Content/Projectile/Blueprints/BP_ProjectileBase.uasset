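; Base projectile Blueprint that handles movement setup and collision reporting, with speed and gravity applied in the construction script.
; BeginPlay caches player and combat references and optionally enables homing, briefly disabling WallHit collision.
; ActorCollision overlaps and WallHit blocking hits feed separate collision and hit calls, with overlaps passing damage info.
; Helpers stop movement with wall collision and compute aim direction by intersecting the mouse ray with a horizontal plane.
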(event OnComponentBeginOverlap(ActorCollision)
  (params (OverlappedComponent :type Primitive%20Component%20Object%20Reference) (OtherActor :type Actor%20Object%20Reference) (OtherComp :type Primitive%20Component%20Object%20Reference) (OtherBodyIndex :type Integer) (bFromSweep :type Boolean) (SweepResult :type Hit%20Result%20Structure%20%28by%20ref%29))
  ;[0.07812 0.07812 0.07812] you might be wondering, hmmm what the fuck is the difference between overlap and hit. well i dont even know so keep wondering kid
  (Default|CallOnProjectileCollision OtherActor SweepResult (Variables|ProjectileSettings|GetSDamageInfo))
  (Variables|Default|SetHasCollided true))

(event OnComponentHit(WallHit)
  (params (HitComponent :type Primitive%20Component%20Object%20Reference) (OtherActor :type Actor%20Object%20Reference) (OtherComp :type Primitive%20Component%20Object%20Reference) (NormalImpulse :type Vector :default "0, 0, 0") (Hit :type Hit%20Result%20Structure%20%28by%20ref%29))
  (Default|CallOnProjectileHit Hit))

(event EventBeginPlay
  (bind _wallhit (Variables|Default|GetWallHit))
  (bind _projectilemovement (Variables|Default|GetProjectileMovement))
  (Utilities|GetComponents)
  (if (Variables|Default|GetIsHoming)
    (Variables|/Script/Engine.ProjectileMovementComponent|SetbIsHomingProjectile _projectilemovement true)
    (Variables|/Script/Engine.ProjectileMovementComponent|SetHomingAccelerationMagnitude _projectilemovement (Variables|Default|GetHomingAcceleration))
    (Collision|SetCollisionEnabled _wallhit "NoCollision")
    (Utilities|FlowControl|Delay 0.2)
    (Collision|SetCollisionEnabled _wallhit "QueryAndPhysics")))

(fn ConstructionScript
  (bind _speed (Variables|ProjectileSettings|GetSpeed))
  (bind _projectilemovement (Variables|Default|GetProjectileMovement))
  (Variables|/Script/Engine.ProjectileMovementComponent|SetInitialSpeed _projectilemovement _speed)
  (Variables|/Script/Engine.ProjectileMovementComponent|SetMaxSpeed _projectilemovement _speed)
  (Variables|/Script/Engine.ProjectileMovementComponent|SetProjectileGravityScale _projectilemovement (Variables|ProjectileSettings|GetGravity)))

(fn FindMousePosition
  (params (SceneComponent :type Scene%20Component%20Object%20Reference))
  (bind _returnvalue (Game|GetPlayerController 0))
  (bind _returnvalue_2 (Transformation|GetWorldLocation SceneComponent))
  (bind (_worldlocation _worlddirection) (Game|Player|ConvertMouseLocationToWorldSpace _returnvalue))
  (return (Math|Vector|GetUnitDirection(Vector) _returnvalue_2 (.Intersection (Class|KismetMathLibrary|LinePlaneIntersectionOriginNormal _worldlocation (+ _worldlocation (* _worlddirection 1e+04)) _returnvalue_2 "0.000000,0.000000,1.000000")))))

(fn DisableCollision&Movement
  (bind _projectilemovement (Variables|Default|GetProjectileMovement)
    (:then
      (Game|Components|ProjectileMovement|SetVelocityinLocalSpace _projectilemovement "0, 0, 0"))
    (:else
      _))
  (bind _wallhit (Variables|Default|GetWallHit)
    (:then
      (Collision|SetCollisionEnabled _wallhit "NoCollision"))
    (:else)))