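; Player hook projectile that launches toward the mouse position from the character's hook shoot point and expires shortly if no enemy is caught.
; On collision it sends damage through CalculateStunDuration, whose distance-based stun bonus node is marked unused, then snaps onto the target.
; It reports landing or finishing to the player's hook component, self-destructing after a brief delay on impact.
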(event Custom|ProjectileHit
  (params (Hit :type Hit%20Result%20Structure))
  (Default|HookFinished (Variables|/Game/Player/Blueprints/BPC_PlayerCombatHandler.BPC_PlayerCombatHandler_C|GetBPC_PlayerHook (Variables|Default|GetBPC_PlayerCombat)))
  (Utilities|FlowControl|Delay 0.6)
  (Actor|DestroyActor))

(event Custom|RotateToTarget
  (bind _direction (CallFunction|FindMousePosition (Variables|/Game/Player/Blueprints/BP_PlayerCharacter.BP_PlayerCharacter_C|GetHookShootPoint (Variables|Default|GetBP_PlayerCharacter))))
  (Variables|/Script/Engine.MovementComponent|SetVelocity (Variables|Default|GetProjectileMovement) (* _direction (Variables|Default|GetSpeed))))

(event Custom|ProjectileCollision
  (params (Other%20Actor :type Actor%20Object%20Reference) (Hit :type Hit%20Result%20Structure) (SDamageInfo :type S%20Damage%20Info%20Structure))
  (CallFunction|DisableCollision&Movement)
  (Variables|Default|SetEnemyHooked true)
  (Class|BPIDamagable|DealDamage(Message) Other%20Actor (Utilities|CalculateStunDuration SDamageInfo))
  (Default|HookLanded (Variables|/Game/Player/Blueprints/BPC_PlayerCombatHandler.BPC_PlayerCombatHandler_C|GetBPC_PlayerHook (Variables|Default|GetBPC_PlayerCombat)) Other%20Actor)
  (Transformation|AttachActorToActor Other%20Actor "None" "SnapToTarget" "KeepWorld" "KeepWorld" true)
  (Utilities|FlowControl|Delay 0.6)
  (Actor|DestroyActor))

(event EventBeginPlay
  (|CallParentFunction)
  (Default|CallOnRotatetoTarget)
  (Utilities|FlowControl|Delay 0.43)
  (if (not (Variables|Default|GetEnemyHooked))
    (Default|HookFinished (Variables|/Game/Player/Blueprints/BPC_PlayerCombatHandler.BPC_PlayerCombatHandler_C|GetBPC_PlayerHook (Variables|Default|GetBPC_PlayerCombat)))
    (Actor|DestroyActor)))

(event Collision|EventActorBeginOverlap
  (params (OtherActor :type Actor%20Object%20Reference))
  (|CallParentFunction OtherActor) ; This node is disabled and will not be called.\nDrag off pins to build functionality.
)

(fn ConstructionScript
  (bind _self self)
  (|CallParentFunction)
  (Variables|Default|SetSpeed (Variables|Default|GetSpeed))
  (EventDispatchers|BindEventtoOnRotatetoTarget _self (EventDispatchers|CreateEvent :!event Custom|RotateToTarget))
  (EventDispatchers|BindEventtoOnProjectileCollision _self (EventDispatchers|CreateEvent :!event Custom|ProjectileCollision))
  (EventDispatchers|BindEventtoOnProjectileHit _self (EventDispatchers|CreateEvent :!event Custom|ProjectileHit)))

(fn FindMousePosition
  (params (SceneComponent :type Scene%20Component%20Object%20Reference))
  (bind _direction (|CallParentFunction SceneComponent))
  (return _direction))