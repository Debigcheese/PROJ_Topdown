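; Turret projectile that launches at its target and damages the player.
; The construction script binds handlers to the parent's rotate, impact and overlap dispatchers, and BeginPlay fires the rotate one.
; If the target is valid, velocity is aimed at it, with X and Y scaled by Speed and Z offset by UpwardsMomentum instead.
; Player overlaps deal damage and destroy it, enemies are ignored, and other overlaps or any impact destroy it.
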(event Custom|ProjectileOverlap
  (params (Other%20Actor :type Actor%20Object%20Reference) (Sweep :type Hit%20Result%20Structure) (SDamage%20Info :type S%20Damage%20Info%20Structure))
  (bind _asbp_player_character (Utilities|Casting|CastToBP_PlayerCharacter Other%20Actor)
    (:then
      (Class|BPIDamagable|DealDamage(Message) _asbp_player_character SDamage%20Info))
    (:CastFailed
      (Utilities|Casting|CastToBP_EnemyBase Other%20Actor
        (:CastFailed
          _))))
  (Actor|DestroyActor))

(event Custom|ProjectileImpact
  (params (Other%20Actor :type Actor%20Object%20Reference) (Hit :type Hit%20Result%20Structure) (SDamageInfo :type S%20Damage%20Info%20Structure))
  (Actor|DestroyActor))

(event Custom|RotateToTarget
  (bind _speed (Variables|Default|GetSpeed))
  (bind _target (Variables|Default|GetTarget)
    (:then
      (Variables|/Script/Engine.MovementComponent|SetVelocity (Variables|Default|GetProjectileMovement) (Math|Vector|MakeVector (* (.x (Math|Vector|GetUnitDirection(Vector) (Transformation|GetActorLocation) (Transformation|GetActorLocation _target))) _speed) (* (.y (Math|Vector|GetUnitDirection(Vector) (Transformation|GetActorLocation) (Transformation|GetActorLocation _target))) _speed) (+ (.z (Math|Vector|GetUnitDirection(Vector) (Transformation|GetActorLocation) (Transformation|GetActorLocation _target))) (Variables|Default|GetUpwardsMomentum)))))
    (:else)))

(event EventBeginPlay
  (|CallParentFunction)
  (Default|CallOnRotatetoTarget))

(event Collision|EventActorBeginOverlap
  (params (OtherActor :type Actor%20Object%20Reference))
  (|CallParentFunction OtherActor) ; This node is disabled and will not be called.\nDrag off pins to build functionality.
)

(fn ConstructionScript
  (bind _self self)
  (|CallParentFunction)
  (Variables|Default|SetSpeed (Variables|Default|GetSpeed))
  (EventDispatchers|BindEventtoOnRotatetoTarget _self (EventDispatchers|CreateEvent :!event Custom|RotateToTarget))
  (EventDispatchers|BindEventtoOnProjectileImpact _self (EventDispatchers|CreateEvent :!event Custom|ProjectileImpact))
  (EventDispatchers|BindEventtoOnProjectileOverlap _self (EventDispatchers|CreateEvent :!event Custom|ProjectileOverlap)))