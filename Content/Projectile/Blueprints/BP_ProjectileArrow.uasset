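; Arrow projectile, a child of a base projectile Blueprint, that flies at a target and deals damage on collision.
; The construction script binds its handlers to rotate, collision and hit dispatchers.
; On BeginPlay it triggers rotation, setting velocity once toward the enemy target, or a fallback location if invalid.
; Collisions send a damage message, with piercing arrows lingering before destruction, while hits disable movement and destroy after a short delay.
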(event Custom|ProjectileCollision
  (params (Other%20Actor :type Actor%20Object%20Reference) (Hit :type Hit%20Result%20Structure) (SDamageInfo :type S%20Damage%20Info%20Structure))
  (Utilities|Time|ClearandInvalidateTimerbyHandle (Variables|Default|GetTimerHandle))
  (Utilities|FlowControl|Delay 0.01)
  (Class|BPIDamagable|DealDamage(Message) Other%20Actor SDamageInfo)
  (if (Variables|Default|GetIsPiercing)
    (Utilities|FlowControl|Delay 1.0)
    (Actor|DestroyActor)
    (else
      (Actor|DestroyActor))))

(event Custom|ProjectileHit
  (params (Hit :type Hit%20Result%20Structure))
  (CallFunction|DisableCollision&Movement)
  (Variables|Default|SetHasCollided true)
  (Utilities|FlowControl|Delay 0.6)
  (Actor|DestroyActor))

(event Custom|RotateToTarget
  (bind _enemytarget (Variables|Default|GetEnemyTarget)
    (:then
      (Variables|/Script/Engine.MovementComponent|SetVelocity (Variables|Default|GetProjectileMovement) (* (Math|Vector|GetUnitDirection(Vector) (Transformation|GetActorLocation) (Transformation|GetActorLocation _enemytarget)) (Variables|Default|GetSpeed))))
    (:else
      (Variables|/Script/Engine.MovementComponent|SetVelocity (Variables|Default|GetProjectileMovement) (* (Math|Vector|GetUnitDirection(Vector) (Transformation|GetActorLocation) (Variables|Default|GetRotateLocation)) (Variables|Default|GetSpeed))))))

(event EventBeginPlay
  (|CallParentFunction)
  (Default|CallOnRotatetoTarget))

(event Collision|EventActorBeginOverlap
  (params (OtherActor :type Actor%20Object%20Reference))
  (|CallParentFunction OtherActor) ; This node is disabled and will not be called.\nDrag off pins to build functionality.
)

(fn ConstructionScript
  (bind _self self)
  (|CallParentFunction)
  (EventDispatchers|BindEventtoOnRotatetoTarget _self (EventDispatchers|CreateEvent :!event Custom|RotateToTarget))
  (EventDispatchers|BindEventtoOnProjectileCollision _self (EventDispatchers|CreateEvent :!event Custom|ProjectileCollision))
  (EventDispatchers|BindEventtoOnProjectileHit _self (EventDispatchers|CreateEvent :!event Custom|ProjectileHit)))