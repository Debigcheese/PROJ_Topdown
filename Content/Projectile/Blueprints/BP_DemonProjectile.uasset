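; Demon projectile that acts as a timed area explosion, damaging its Target if it overlaps the actor's collision.
; After a one-second delay, Explosion polls the overlap on a fast looping timer until it deals damage or the short window closes, then the actor destroys itself.
; Rotate, collision and hit handlers are bound in construction but empty, leaving their homing and impact logic disconnected.
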(event Custom|ProjectileHit
  (params (Hit :type Hit%20Result%20Structure)))

(event Custom|Explosion
  (bind _returnvalue (Utilities|Time|SetTimerbyEvent (delegate Custom|Explosion) 0.01 true))
  (Variables|Default|SetTimerHandle _returnvalue)
  (if (Collision|IsOverlappingActor (Variables|Default|GetActorCollision) (Variables|Default|GetTarget) :!class /Script/Engine.PrimitiveComponent)
    (Class|BPIDamagable|DealDamage(Message) (Variables|Default|GetTarget) (Variables|Default|GetSDamageInfo))
    (Utilities|Time|ClearandInvalidateTimerbyHandle (Variables|Default|GetTimerHandle))
    (Development|PrintString (Utilities|String|ToString(Float) (.damageamount (Variables|Default|GetSDamageInfo))))))

(event Custom|RotateToTarget)

(event Custom|ProjectileCollision
  (params (Other%20Actor :type Actor%20Object%20Reference) (Hit :type Hit%20Result%20Structure) (SDamageInfo :type S%20Damage%20Info%20Structure)))

(event EventBeginPlay
  (|CallParentFunction)
  (Default|CallOnRotatetoTarget)
  (Utilities|FlowControl|Delay 1.0)
  (CallFunction|Explosion)
  (Utilities|FlowControl|Delay 0.7)
  (Utilities|Time|ClearandInvalidateTimerbyHandle (Variables|Default|GetTimerHandle))
  (Utilities|FlowControl|Delay 1.0)
  (Actor|DestroyActor))

(event Collision|EventActorBeginOverlap
  (params (OtherActor :type Actor%20Object%20Reference))
  (|CallParentFunction OtherActor) ; This node is disabled and will not be called.\nDrag off pins to build functionality.
)

(fn ConstructionScript
  (bind _self self)
  (|CallParentFunction)
  (EventDispatchers|BindEventtoOnRotatetoTarget _self (EventDispatchers|CreateEvent :!event Custom|RotateToTarget))
  (EventDispatchers|BindEventtoOnProjectileCollision _self (EventDispatchers|CreateEvent :!event Custom|ProjectileCollision))
  (EventDispatchers|BindEventtoOnProjectileHit _self (EventDispatchers|CreateEvent :!event Custom|ProjectileHit)))