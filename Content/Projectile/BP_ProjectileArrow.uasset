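; Homing arrow projectile that steers toward EnemyTarget and deals damage on impact.
; The construction script binds the rotate and impact dispatchers, and BeginPlay fires the rotate one.
; RotateToTarget re-sets its own very short looping timer on every call, pointing ProjectileMovement velocity at a valid target at Speed.
; Impact clears the timer, sends a damage message to the hit actor and destroys the arrow.
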(event Custom|RotateToTarget
  (bind _returnvalue (Utilities|Time|SetTimerbyEvent (delegate Custom|RotateToTarget) 0.001 true))
  (Variables|Default|SetTimerHandle _returnvalue)
  (bind _enemytarget (Variables|Default|GetEnemyTarget)
    (:then
      (Variables|/Script/Engine.MovementComponent|SetVelocity (Variables|Default|GetProjectileMovement) (* (Math|Vector|GetUnitDirection(Vector) (Transformation|GetActorLocation) (Transformation|GetActorLocation _enemytarget)) (Variables|Default|GetSpeed))))
    (:else)))

(event Custom|ProjectileImpact
  (params (Other%20Actor :type Actor%20Object%20Reference) (Hit :type Hit%20Result%20Structure) (SDamageInfo :type S%20Damage%20Info%20Structure))
  (Utilities|Time|ClearandInvalidateTimerbyHandle (Variables|Default|GetTimerHandle))
  (Class|BPIDamagable|DealDamage(Message) Other%20Actor SDamageInfo)
  (Actor|DestroyActor))

(event EventBeginPlay
  (|CallParentFunction)
  (Default|CallOnRotatetoTarget))

(event Collision|EventActorBeginOverlap
  (params (OtherActor :type Actor%20Object%20Reference))
  (|CallParentFunction OtherActor) ; This node is disabled and will not be called.\nDrag off pins to build functionality.
)

(fn ConstructionScript
  (bind _self self)
  (|CallParentFunction)
  (Variables|Default|SetSpeed (Variables|Default|GetSpeed))
  (EventDispatchers|BindEventtoOnRotatetoTarget _self (EventDispatchers|CreateEvent :!event Custom|RotateToTarget))
  (EventDispatchers|BindEventtoOnProjectileImpact _self (EventDispatchers|CreateEvent :!event Custom|ProjectileImpact)))