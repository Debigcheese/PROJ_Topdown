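; Heavy arrow projectile, a child of a parent projectile class, that flies from the player's bow toward the mouse position.
; Construction binds the parent's rotate and impact dispatchers; BeginPlay fires the rotate one, setting velocity from FindMousePosition at the bow shoot point times Speed.
; On impact it damages BP_EnemyBase actors and attaches to them, snapping location but keeping world rotation.
; Any impact destroys the arrow after a short delay.
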(event Custom|RotateToTarget
  (bind _direction (CallFunction|FindMousePosition (Variables|/Game/Player/Blueprints/BP_PlayerCharacter.BP_PlayerCharacter_C|GetBowShootPoint (Variables|Default|GetBP_PlayerCharacter))))
  (Variables|/Script/Engine.MovementComponent|SetVelocity (Variables|Default|GetProjectileMovement) (* _direction (Variables|Default|GetSpeed))))

(event Custom|ProjectileImpact
  (params (Other%20Actor :type Actor%20Object%20Reference) (Hit :type Hit%20Result%20Structure) (SDamageInfo :type S%20Damage%20Info%20Structure))
  (if (Class|GameplayStatics|ObjectIsA Other%20Actor "/Game/Enemies/Blueprints/BP_EnemyBase.BP_EnemyBase_C")
    (Class|BPIDamagable|DealDamage(Message) Other%20Actor SDamageInfo)
    (Transformation|AttachActorToActor Other%20Actor "None" "SnapToTarget" "KeepWorld" "KeepWorld" true))
  (Utilities|FlowControl|Delay 0.6)
  (Actor|DestroyActor))

(event EventBeginPlay
  (|CallParentFunction)
  (Default|CallOnRotatetoTarget))

(event Collision|EventActorBeginOverlap
  (params (OtherActor :type Actor%20Object%20Reference))
  (|CallParentFunction OtherActor) ; This node is disabled and will not be called.\nDrag off pins to build functionality.
)

(fn ConstructionScript
  (bind _self self)
  (|CallParentFunction)
  (Variables|Default|SetSpeed (Variables|Default|GetSpeed))
  (EventDispatchers|BindEventtoOnRotatetoTarget _self (EventDispatchers|CreateEvent :!event Custom|RotateToTarget))
  (EventDispatchers|BindEventtoOnProjectileImpact _self (EventDispatchers|CreateEvent :!event Custom|ProjectileImpact)))

(fn FindMousePosition
  (params (SceneComponent :type Scene%20Component%20Object%20Reference))
  (bind _direction (|CallParentFunction SceneComponent))
  (return _direction))